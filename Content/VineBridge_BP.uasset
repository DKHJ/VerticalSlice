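; A vine bridge actor that fades in or out and switches its collision to become solid or passable.
; Construction creates a dynamic material from Vine_INS, and StartVisible sets its initial Opacity_Control, though collision always starts disabled.
; Activation events run reversed timelines that drive Opacity_Control to zero and enable collision.
; Deactivation calls DoInteract, as ActivateVines activation does, then plays a timeline forward and disables collision when finished.
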(event Custom|ActivateVines
  (params (Activated? :type Boolean))
  (if Activated?
    (CallFunction|DoInteract)
    (bind _time (Timeline|Timeline_0 ReverseFromEnd)
      (:Update
        (Rendering|Material|SetScalarParameterValue (Variables|Default|GetLines) "Opacity_Control" _time :!class /Script/Engine.MaterialInstanceDynamic))
      (:Finished
        (Rendering|Material|SetScalarParameterValue (Variables|Default|GetLines) "Opacity_Control" 0.0 :!class /Script/Engine.MaterialInstanceDynamic)
        (Collision|SetActorEnableCollision true)))
    (else
      (CallFunction|DoInteract)
      (bind _time_2 (Timeline|Timeline_1 PlayFromStart)
        (:Update
          (Rendering|Material|SetScalarParameterValue (Variables|Default|GetLines) "Opacity_Control" _time_2 :!class /Script/Engine.MaterialInstanceDynamic))
        (:Finished
          (Collision|SetActorEnableCollision false))))))

(event EventBeginPlay
  (Collision|SetActorEnableCollision false)
  (if (Variables|Default|GetStartVisible?)
    (Rendering|Material|SetScalarParameterValue (Variables|Default|GetLines) "Opacity_Control" 0.0 :!class /Script/Engine.MaterialInstanceDynamic)
    (else
      (Rendering|Material|SetScalarParameterValue (Variables|Default|GetLines) "Opacity_Control" 1.0 :!class /Script/Engine.MaterialInstanceDynamic))))

(event EventOnActivatedVineBridgeEvent
  (Development|PrintString "BridgeActivated")
  (bind _time (Timeline|Time ReverseFromEnd)
    (:Update
      (Rendering|Material|SetScalarParameterValue (Variables|Default|GetLines) "Opacity_Control" _time :!class /Script/Engine.MaterialInstanceDynamic)
      (Collision|SetActorEnableCollision true))
    (:Finished
      (Rendering|Material|SetScalarParameterValue (Variables|Default|GetLines) "Opacity_Control" 0.0 :!class /Script/Engine.MaterialInstanceDynamic)
      (Collision|SetActorEnableCollision true))))

(fn ConstructionScript
  (bind _returnvalue (Rendering|Material|CreateDynamicMaterialInstance (Variables|Character|GetMesh) 0 "/Game/Assets/Vines/Vine_INS.Vine_INS" "None" :!class /Script/Engine.PrimitiveComponent))
  (Variables|Default|SetLines _returnvalue))

(fn DoInteraction
  (return false))