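; Board actor for a push-tile puzzle that builds and scrambles a square grid of SummerPushPuzzle_BP pieces on BeginPlay.
; CreatePuzzle derives piece size from board and grid size, then spawns and initialises scaled pieces in the XZ plane centred on the actor.
; RandomiseTiles shuffles the cell locations and teleports pieces onto them.
; A location-check macro compares pieces to cells but is not called here, and both its branches set true.
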(event Custom|CreatePuzzle
  (bind _boardsize_const_ (Variables|Default|GetBoardSize%28Const%29))
  (bind _returnvalue (/ _boardsize_const_ 2.0))
  (Variables|Default|SetPuzzlePieceSize (/ (Variables|Default|GetBoardSize%28Const%29) (Math|Conversions|ToFloat(Integer) (Variables|Default|GetGridSize))))
  (Utilities|Array|Clear (Variables|Default|GetLocationsArray))
  (Utilities|Array|Clear (Variables|Default|GetPuzzlePieceArray))
  (for _index (range 0 (|((Size*Size)-2) (Variables|Default|GetGridSize)))
    (Utilities|Array|Add (Variables|Default|GetLocationsArray) (+ (Math|Vector|MakeVector (+ (* (Math|Integer|%(Integer) _index (Variables|Default|GetGridSize)) (Variables|Default|GetPuzzlePieceSize)) (/ (Variables|Default|GetPuzzlePieceSize) 2.0)) 0.0 (- (* (/ _index (Variables|Default|GetGridSize)) (* (Variables|Default|GetPuzzlePieceSize) -1.0)) (/ (Variables|Default|GetPuzzlePieceSize) 2.0))) (Transformation|GetActorLocation) (Math|Vector|MakeVector (* _returnvalue -1.0) 0.0 _returnvalue)))
    (bind _returnvalue_2 (Game|SpawnActorfromClass "/Game/SummerPushPuzzle_BP.SummerPushPuzzle_BP_C" (Math|Transform|MakeTransform (+ (Math|Vector|MakeVector (+ (* (Math|Integer|%(Integer) _index (Variables|Default|GetGridSize)) (Variables|Default|GetPuzzlePieceSize)) (/ (Variables|Default|GetPuzzlePieceSize) 2.0)) 0.0 (- (* (/ _index (Variables|Default|GetGridSize)) (* (Variables|Default|GetPuzzlePieceSize) -1.0)) (/ (Variables|Default|GetPuzzlePieceSize) 2.0))) (Transformation|GetActorLocation) (Math|Vector|MakeVector (* _returnvalue -1.0) 0.0 _returnvalue)) "0, 0, 0" (Math|Conversions|ToVector(Float) (/ (Variables|Default|GetPuzzlePieceSize) 1e+02))) "AlwaysSpawn" 0 0))
    (Utilities|Array|Add (Variables|Default|GetPuzzlePieceArray) _returnvalue_2)
    (Variables|/Game/SummerPushPuzzle_BP.SummerPushPuzzle_BP_C|SetPuzzlePieceSize _returnvalue_2 (Variables|Default|GetPuzzlePieceSize))
    (Default|InitPuzzlePiece _returnvalue_2 _index (Variables|Default|GetGridSize)))
  (CallFunction|RandomiseTiles (Variables|Default|GetLocationsArray) (Variables|Default|GetPuzzlePieceArray)))

(event Collision|EventActorBeginOverlap
  (params (OtherActor :type Actor%20Object%20Reference)))

(event EventTick
  (params (DeltaSeconds :type Float%20%28single-precision%29)))

(event EventBeginPlay
  (CallFunction|CreatePuzzle))

(fn ConstructionScript)

(fn RandomiseTiles
  (params (Locations :type Array%20of%20Vectors) (PuzzlePieces :type Array%20of%20Summer%20Push%20Puzzle%20BP%20Object%20References))
  (bind _output_get (Variables|Default|SetLocationsArray Locations))
  (Utilities|Array|Shuffle _output_get)
  (for (_array_element _array_index) PuzzlePieces
    (Transformation|SetActorLocation _array_element (Utilities|Array|Get(acopy) (Variables|Default|GetLocationsArray) _array_index) false false)))