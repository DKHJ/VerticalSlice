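; A portal actor that shows a live view from its linked OtherPortal on its Plane.
; BeginPlay creates a viewport-sized render target, feeds it to a dynamic material on the Plane and assigns it to OtherPortal's scene capture.
; Each tick moves that capture to mirror the player camera's world-space offset from this Plane and copies its rotation, ignoring relative portal orientation.
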(event EventBeginPlay
  (bind _returnvalue (Viewport|GetViewportSize))
  (bind _returnvalue_2 (Rendering|Material|CreateDynamicMaterialInstance (Variables|Default|GetPortalMaterial) "None" :!class /Script/Engine.KismetMaterialLibrary))
  (bind _output_get (Variables|Default|SetMaterialInstance _returnvalue_2))
  (Rendering|Material|SetMaterial (Variables|Default|GetPlane) 0 _output_get)
  (bind _returnvalue_3 (Rendering|CreateRenderTarget2D (Math|Float|Truncate (.x _returnvalue)) (Math|Float|Truncate (.y _returnvalue)) "RTF_RGBA16f" "(R=1.000000,G=0.000000,B=0.049067,A=1.000000)"))
  (bind _output_get_2 (Variables|Default|SetRenderTarget _returnvalue_3))
  (Rendering|Material|SetTextureParameterValue (Variables|Default|GetMaterialInstance) "Texture" _output_get_2)
  (bind _otherportal (Variables|Default|GetOtherPortal)
    (:then
      (Variables|/Script/Engine.SceneCaptureComponent2D|SetTextureTarget (Variables|NewPortal_BP_C|GetSceneCaptureComponent2D _otherportal) (Variables|Default|GetRenderTarget)))
    (:else)))

(event Collision|EventActorBeginOverlap
  (params (OtherActor :type Actor%20Object%20Reference)))

(event EventTick
  (params (DeltaSeconds :type Float%20%28single-precision%29))
  (bind _otherportal (Variables|Default|GetOtherPortal)
    (:then
      (Transformation|SetWorldRotation (Variables|NewPortal_BP_C|GetSceneCaptureComponent2D _otherportal) (Camera|GetCameraRotation (Variables|/Script/Engine.PlayerController|GetPlayerCameraManager (Game|GetPlayerController 0))) false false)
      (Transformation|SetWorldLocation (Variables|NewPortal_BP_C|GetSceneCaptureComponent2D (Variables|Default|GetOtherPortal)) (- (Transformation|GetWorldLocation (Variables|NewPortal_BP_C|GetPlane (Variables|Default|GetOtherPortal))) (- (Transformation|GetWorldLocation (Variables|Default|GetPlane)) (Camera|GetCameraLocation (Variables|/Script/Engine.PlayerController|GetPlayerCameraManager (Game|GetPlayerController 0))))) false false))
    (:else)))

(fn ConstructionScript)