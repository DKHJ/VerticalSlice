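; Spring hub world portal Blueprint that supplies the portal's cinematic playback.
; GotoCinematicMode calls PlayCinematic, which puts player controller 0 into cinematic mode affecting movement and turning, then creates and plays a level sequence player for SequenceToPlay.
; Nothing in this graph triggers GotoCinematicMode or exits cinematic mode, and the default BeginPlay, overlap and Tick events are disabled.
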(event Custom|PlayCinematic
  (Class|PlayerController|SetCinematicMode (Game|GetPlayerController 0) true true true true true)
  (bind _outactor (Sequencer|Player|CreateLevelSequencePlayer (Variables|Default|GetSequenceToPlay)))
  (Sequencer|Player|Play (Variables|/Script/LevelSequence.LevelSequenceActor|GetSequencePlayer _outactor) :!class /Script/MovieScene.MovieSceneSequencePlayer))

(event EventBeginPlay
  (|CallParentFunction) ; This node is disabled and will not be called.\nDrag off pins to build functionality.
)

(event Collision|EventActorBeginOverlap
  (params (OtherActor :type Actor%20Object%20Reference)))

(event EventTick
  (params (DeltaSeconds :type Float%20%28single-precision%29))
  (|CallParentFunction DeltaSeconds) ; This node is disabled and will not be called.\nDrag off pins to build functionality.
)

(event EventGotoCinematicMode
  (CallFunction|PlayCinematic))

(fn ConstructionScript
  (|CallParentFunction))