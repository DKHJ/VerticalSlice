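; Winter portal actor for the hub world that records where the player respawns on returning to the hub.
; When BP_BigCharacter overlaps its collision, it writes a fixed HubWorldSpawnNumber into NetworkGameInstance_BP.
; A separate GotoCinematicMode event calls PlayCinematic, which locks player 0's movement and turning in cinematic mode and plays the assigned level sequence.
; Nothing in this graph triggers the cinematic or performs level travel.
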(event OnComponentBeginOverlap(Collision)
  (params (OverlappedComponent :type Primitive%20Component%20Object%20Reference) (OtherActor :type Actor%20Object%20Reference) (OtherComp :type Primitive%20Component%20Object%20Reference) (OtherBodyIndex :type Integer) (bFromSweep :type Boolean) (SweepResult :type Hit%20Result%20Structure%20%28by%20ref%29))
  ;[1 1 1] Here we are setting the world spawn number so when we return to the hub world we know where to spawn
  (Utilities|Casting|CastToBP_BigCharacter OtherActor)
  (bind _asnetwork_game_instance_bp (Utilities|Casting|CastToNetworkGameInstance_BP (Game|GetGameInstance)))
  (Variables|/Game/Blueprints/GameLogic/NetworkGameInstance_BP.NetworkGameInstance_BP_C|SetHubWorldSpawnNumber _asnetwork_game_instance_bp 4))

(event Custom|PlayCinematic
  (Class|PlayerController|SetCinematicMode (Game|GetPlayerController 0) true true true true true)
  (bind _outactor (Sequencer|Player|CreateLevelSequencePlayer (Variables|Default|GetSequenceToPlay)))
  (Sequencer|Player|Play (Variables|/Script/LevelSequence.LevelSequenceActor|GetSequencePlayer _outactor) :!class /Script/MovieScene.MovieSceneSequencePlayer))

(event EventBeginPlay
  (|CallParentFunction) ; This node is disabled and will not be called.\nDrag off pins to build functionality.
)

(event Collision|EventActorBeginOverlap
  (params (OtherActor :type Actor%20Object%20Reference)))

(event EventTick
  (params (DeltaSeconds :type Float%20%28single-precision%29))
  (|CallParentFunction DeltaSeconds) ; This node is disabled and will not be called.\nDrag off pins to build functionality.
)

(event EventGotoCinematicMode
  (CallFunction|PlayCinematic))

(fn ConstructionScript
  (|CallParentFunction))