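; Portal in the Winter level that returns players to the HubWorld map once both characters stand in it.
; Collision overlap events track presence of actors tagged BigCharacter and SmallCharacter in two flags.
; When both flags are set and NetworkGameInstance reports Winter completed, it issues a ServerTravel console command through the first player controller.
; Completion is only checked on overlap begin.
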(event OnComponentBeginOverlap(Collision)
  (params (OverlappedComponent :type Primitive%20Component%20Object%20Reference) (OtherActor :type Actor%20Object%20Reference) (OtherComp :type Primitive%20Component%20Object%20Reference) (OtherBodyIndex :type Integer) (bFromSweep :type Boolean) (SweepResult :type Hit%20Result%20Structure%20%28by%20ref%29))
  (if (Actor|ActorHasTag OtherActor "BigCharacter")
    (bind _output_get (Variables|Default|SetBigCharacterPresent_0 true))
    (if (Math|Boolean|Equal(Boolean) _output_get (stale _output_get_2)) :!label _label
      (bind _asnetwork_game_instance (Utilities|Casting|CastToNetworkGameInstance (Game|GetGameInstance)))
      (if (Variables|/Script/VerticalSlice.NetworkGameInstance|GetbIsWinterCompleted _asnetwork_game_instance)
        (CallFunction|BacktoHubWorld)))
    (elif (Actor|ActorHasTag OtherActor "SmallCharacter")
      (bind _output_get_2 (Variables|Default|SetSmallCharacterPresent_0 true))
      (goto _label))))

(event OnComponentEndOverlap(Collision)
  (params (OverlappedComponent :type Primitive%20Component%20Object%20Reference) (OtherActor :type Actor%20Object%20Reference) (OtherComp :type Primitive%20Component%20Object%20Reference) (OtherBodyIndex :type Integer))
  (if (Actor|ActorHasTag OtherActor "BigCharacter")
    (Variables|Default|SetBigCharacterPresent_0 false)
    (elif (Actor|ActorHasTag OtherActor "SmallCharacter")
      (Variables|Default|SetSmallCharacterPresent_0 false))))

(event Custom|BackToHubWorld
  (Development|ExecuteConsoleCommand "ServerTravel/Game/Levels/HubWorld" (Game|GetPlayerController 0)))

(event EventBeginPlay
  (|CallParentFunction) ; This node is disabled and will not be called.\nDrag off pins to build functionality.
)

(event Collision|EventActorBeginOverlap
  (params (OtherActor :type Actor%20Object%20Reference)))

(event EventTick
  (params (DeltaSeconds :type Float%20%28single-precision%29))
  (|CallParentFunction DeltaSeconds) ; This node is disabled and will not be called.\nDrag off pins to build functionality.
)

(fn ConstructionScript
  (|CallParentFunction))