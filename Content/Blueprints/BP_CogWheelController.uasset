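; BP_CogWheelController is a cog puzzle controller that activates placed cog wheels to match how many cogs have been picked up.
; When BP_BigCharacter overlaps its box, the server reads the pickup count from NetworkGameInstance_BP and loops over that many CogWheels references.
; Each non-visible cog gets its material swapped, is flagged activated and plays a sound.
; CogsInPlace becomes true once the activated count equals the number needed.
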(event OnComponentBeginOverlap(Box)
  (params (OverlappedComponent :type Primitive%20Component%20Object%20Reference) (OtherActor :type Actor%20Object%20Reference) (OtherComp :type Primitive%20Component%20Object%20Reference) (OtherBodyIndex :type Integer) (bFromSweep :type Boolean) (SweepResult :type Hit%20Result%20Structure%20%28by%20ref%29))
  (Utilities|Casting|CastToBP_BigCharacter OtherActor)
  (Networking|SwitchHasAuthority
    (:Authority
      (Development|PrintString "[SERVER] Checking Cog Progress..." true true "(R=1.000000,G=0.675707,B=0.449984,A=1.000000)")
      (CallFunction|CheckCogWheels))))

(event Custom|CheckCogWheels
  ;[1 1 1] First we get the number of cogs picked up
  (bind _asnetwork_game_instance_bp (Utilities|Casting|CastToNetworkGameInstance_BP (Game|GetGameInstance)))
  (for _index (range 1 (Variables|/Game/Blueprints/GameLogic/NetworkGameInstance_BP.NetworkGameInstance_BP_C|GetCogsPickedUp _asnetwork_game_instance_bp))
    ;[1 1 1] Check through our references based on the cog number
    (if (not (Variables|/Game/Blueprints/Interactables/Wheels+Cogs/BP_CogWheel.BP_CogWheel_C|GetVisible (Utilities|Array|Get(acopy) (Variables|Default|GetCogWheels) _index)))
      (Rendering|Material|SetMaterial (Variables|/Game/Blueprints/Interactables/Wheels+Cogs/BP_CogWheel.BP_CogWheel_C|GetStaticMesh (Utilities|Array|Get(acopy) (Variables|Default|GetCogWheels) _index)) 0 "/Game/Assets/WheelAndGear/WheelAndGears.WheelAndGears")
      (Variables|/Game/Blueprints/Interactables/Wheels+Cogs/BP_CogWheel.BP_CogWheel_C|SetActivated (Utilities|Array|Get(acopy) (Variables|Default|GetCogWheels) _index) true)
      (Math|Integer|IncrementInt (Variables|Default|GetCogsActivated)
        (:%20%20
          (Audio|PlaySound2D "/Game/Audio/ftus_industrial_lever_metal_pull_old_rusty_002_677__online-audio-converter_com_.ftus_industrial_lever_metal_pull_old_rusty_002_677__online-audio-converter_com_" 1.0 1.0 0.0 0 0)
          (Development|PrintString "Cog Activated & Visible")))))
  (Development|PrintString (Utilities|String|Append "Cogs Picked up: " (Utilities|String|ToString(Integer) (Variables|/Game/Blueprints/GameLogic/NetworkGameInstance_BP.NetworkGameInstance_BP_C|GetCogsPickedUp _asnetwork_game_instance_bp))))
  (if (== (Variables|Default|GetNumOfCogsNeeded) (Variables|Default|GetCogsActivated))
    (Variables|Default|SetCogsInPlace true)))

(fn ConstructionScript)