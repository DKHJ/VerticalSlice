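; BP_WinterPillar is an interactable pillar that toggles an ice effect and its collision.
; The construction script puts a dynamic IceFade_INS material on the mesh's second material slot, and BeginPlay zeroes its scalar parameter.
; DoInteract flips the Activated state and plays or reverses a timeline that drives that parameter.
; When the timeline finishes, the mesh gets query and physics collision if activated, or none otherwise.
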(event EventDoInteract
  (if (Variables|Default|GetActivated)
    (Variables|Default|SetActivated false)
    (bind _time (Timeline|Timeline_0 ReverseFromEnd)
      (:Update
        (Rendering|Material|SetScalarParameterValue (Variables|Default|GetIceMaterial) "Param" _time :!class /Script/Engine.MaterialInstanceDynamic))
      (:Finished
        (if (Variables|Default|GetActivated)
          (Collision|SetCollisionEnabled (Variables|Character|GetMesh) "QueryAndPhysics")
          (else
            (Collision|SetCollisionEnabled (Variables|Character|GetMesh) "NoCollision")))))
    (else
      (Variables|Default|SetActivated true)
      (Timeline|Timeline_0 PlayFromStart))))

(event EventBeginPlay
  (Rendering|Material|SetScalarParameterValue (Variables|Default|GetIceMaterial) "Param" 0.0 :!class /Script/Engine.MaterialInstanceDynamic))

(fn ConstructionScript
  (bind _returnvalue (Rendering|Material|CreateDynamicMaterialInstance (Variables|Character|GetMesh) 1 "/Game/Assets/IceMaterial/IceFade_INS.IceFade_INS" "None" :!class /Script/Engine.PrimitiveComponent))
  (Variables|Default|SetIceMaterial _returnvalue))