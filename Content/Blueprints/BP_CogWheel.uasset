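; BP_CogWheel is a cog wheel actor whose static mesh can be shown or hidden and spun by a RotatingMovement component.
; On BeginPlay, flags set mesh visibility, optionally override the rotation rate for reverse spin, and optionally activate the movement.
; ActivateCogs and DeactivateCogs events start and stop the rotation, while SetVisible toggles the mesh independently of the movement.
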(event Custom|ActivateCogs
  (Components|Activation|Activate (Variables|Default|GetRotatingMovement) false))

(event Custom|DeactivateCogs
  (Components|Activation|Deactivate (Variables|Default|GetRotatingMovement)))

(event EventBeginPlay
  (if (Variables|Default|GetReverseDirection)
    (Variables|/Script/Engine.RotatingMovementComponent|SetRotationRate (Variables|Default|GetRotatingMovement) "-180.000000, 0, 0"))
  (if (Variables|Default|GetVisible)
    (Rendering|SetVisibility (Variables|Default|GetStaticMesh) true false)
    (else
      (Rendering|SetVisibility (Variables|Default|GetStaticMesh) false false)))
  (if (Variables|Default|GetStartActivated)
    (Components|Activation|Activate (Variables|Default|GetRotatingMovement) false)))

(fn ConstructionScript)

(fn SetVisible
  (params (Visible :type Boolean))
  (if Visible
    (Rendering|SetVisibility (Variables|Default|GetStaticMesh) true false)
    (else
      (Rendering|SetVisibility (Variables|Default|GetStaticMesh) false false)))
  (return))