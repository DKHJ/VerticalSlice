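; Big playable character that carries and throws the small character or boxes, with interaction and static-camera switching.
; Holding AimThrow opens a Tick gate that swaps material, matches control yaw and ping-pongs launch velocity via timelines.
; Each update previews the arc with debug line traces along sampled ballistic segments.
; Action throws on authority by spawning projectiles at that velocity, destroying the small character when it is the one thrown.
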(event Custom|ResetTimeLine
  (bind _returnvalue (Game|GetPlayerController 0))
  (bind _returnvalue_2 (Pawn|GetControlRotation _returnvalue :!class /Script/Engine.Controller))
  (bind _newtrack_6 (Timeline|Timeline_1 SetNewTime)
    (:Update
      (bind _output_get (Variables|Default|SetBoxInitialLocalVelocity (Math|Vector|Lerp(Vector) "0, 0, 0" "1000.000000,0.000000,850.000000" _newtrack_6)))
      (CallFunction|DrawThrowTrajectory _output_get)
      (Variables|Default|SetOldRotation (Transformation|GetActorRotation))
      (Transformation|SetActorRotation (Math|Rotator|MakeRotator (.roll _returnvalue_2) (Math|Float|ClampAngle (.pitch _returnvalue_2) 0.0 0.0) (.yaw _returnvalue_2))))
    (:Finished
      (if (Variables|Default|GetCanRetractLine)
        (Variables|Default|SetCanRetractLine false)
        (else
          (Variables|Default|SetCanRetractLine true))))))

(event Custom|Action%20Server
  (if (Variables|Default|GetSmallCharacterPickedUp)
    (CallFunction|ThrowCharacter)
    (Variables|Default|SetSmallCharacterPickedUp false)
    (Variables|/Game/Animations/Big/Big_AnimBP.Big_AnimBP_C|SetbThrowLittle (Variables|Default|GetBigAnimBP) true)
    (elif (or (Variables|Default|GetPickedUpBigBox) (Variables|Default|GetPickedUpBox))
      (CallFunction|ThrowBox)
      (Variables|Default|SetPickedUpBox false)
      (Variables|Default|SetPickedUpBigBox false))))

(event Custom|ChangeMat
  (Rendering|Material|SetMaterial (Variables|Character|GetMesh) 0 "/Game/Animations/Big/BigGuyOpaque.BigGuyOpaque"))

(event Custom|ChangeMatBack
  (Rendering|Material|SetMaterial (Variables|Character|GetMesh) 0 "/Game/Assets/Characters/BigGuy_MAT_Diffuse_Mat.BigGuy_MAT_Diffuse_Mat"))

(event EventTick
  (params (DeltaSeconds :type Float%20%28single-precision%29))
  (bind _returnvalue (Game|GetPlayerController 0))
  (bind _returnvalue_2 (Game|GetPlayerController 0))
  (bind _returnvalue_3 (Pawn|GetControlRotation _returnvalue :!class /Script/Engine.Controller))
  (bind _returnvalue_4 (Pawn|GetControlRotation _returnvalue_2 :!class /Script/Engine.Controller))
  (if (Math|Boolean|ORBoolean (Variables|Default|GetSmallCharacterPickedUp) (Variables|Default|GetPickedUpBox) (Variables|Default|GetPickedUpBigBox))
    (Utilities|FlowControl|Sequence
      (:then_0
        (Utilities|FlowControl|Gate true
          (:Exit
            (CallFunction|ChangeMat)
            (if (Variables|Default|GetSmallCharacterPickedUp)
              (if (Variables|Default|GetCanRetractLine)
                (bind _newtrack_6 (Timeline|Timeline_0 Reverse)
                  (:Update
                    (bind _output_get (Variables|Default|SetPlayerInitialVelocity (Math|Vector|Lerp(Vector) "0, 0, 0" "700.000000,0.000000,700.000000" _newtrack_6)))
                    (CallFunction|DrawThrowTrajectory _output_get)
                    (Variables|Default|SetOldRotation (Transformation|GetActorRotation))
                    (Transformation|SetActorRotation (Math|Rotator|MakeRotator (.roll _returnvalue_4) (Math|Float|ClampAngle (.pitch _returnvalue_4) 0.0 0.0) (.yaw _returnvalue_4))))
                  (:Finished
                    (if (Variables|Default|GetCanRetractLine)
                      (Variables|Default|SetCanRetractLine false)
                      (else
                        (Variables|Default|SetCanRetractLine true)))))
                (else
                  (Timeline|Timeline_0 Play)))
              (elif (Variables|Default|GetCanRetractLine)
                (bind _newtrack_6_2 (Timeline|Timeline_1 Reverse)
                  (:Update
                    (bind _output_get_2 (Variables|Default|SetBoxInitialLocalVelocity (Math|Vector|Lerp(Vector) "0, 0, 0" "1000.000000,0.000000,850.000000" _newtrack_6_2)))
                    (CallFunction|DrawThrowTrajectory _output_get_2)
                    (Variables|Default|SetOldRotation (Transformation|GetActorRotation))
                    (Transformation|SetActorRotation (Math|Rotator|MakeRotator (.roll _returnvalue_3) (Math|Float|ClampAngle (.pitch _returnvalue_3) 0.0 0.0) (.yaw _returnvalue_3))))
                  (:Finished
                    (if (Variables|Default|GetCanRetractLine)
                      (Variables|Default|SetCanRetractLine false)
                      (else
                        (Variables|Default|SetCanRetractLine true)))))
                (else
                  (Timeline|Timeline_1 Play))))))))))

(event EventBeginPlay
  ;[1 1 1] Event Begin Play
  (Utilities|FlowControl|Delay 1.0)
  ;;[1 0 0.1577] Get a reference to the small character
  (bind _outactors (Actor|GetAllActorsOfClass "/Game/Blueprints/Characters/BP_SmallCharacter.BP_SmallCharacter_C"))
  (Variables|Default|SetSmallCharacterRef (Utilities|Array|Get(acopy) _outactors))
  (bind _outactors_2 (Actor|GetAllActorsOfClass "/Game/Blueprints/Cameras/StaticCamera.StaticCamera_C"))
  (for _array_element _outactors_2
    (switch int (Variables|/Game/Blueprints/Cameras/StaticCamera.StaticCamera_C|GetCameraNumber _array_element)
      (:1
        (Variables|Default|SetStaticCamera1 _array_element))
      (:2
        (Variables|Default|SetStaticCamera2 _array_element))
      (:3
        (Variables|Default|SetStaticCamera3 _array_element))))
  (bind _asbig_anim_bp (Utilities|Casting|CastToBig_AnimBP (Components|SkeletalMesh|GetAnimInstance (Variables|Character|GetMesh))))
  (Variables|Default|SetBigAnimBP _asbig_anim_bp))

(event Input|ActionEvents|InputActionAction
  (params (Key :type Key%20Structure :default "None"))
  (:Pressed
    (Networking|SwitchHasAuthority
      (:Authority
        (Development|PrintString "[SERVER] Big Character Action")
        (CallFunction|ActionServer)))))

(event Input|ActionEvents|InputActionInteract
  (params (Key :type Key%20Structure :default "None"))
  (bind _interactactorreference (Variables|Default|GetInteractActorReference))
  (:Pressed
    (Development|PrintString "[BC] Interact Pressed" true true "(R=1.000000,G=0.810099,B=0.522876,A=1.000000)")
    ;[1 1 1] Check if we're allowed to interact, Double check if the actor is valid
    (if (Variables|Default|GetCanInteract)
      (Utilities|IsValid _interactactorreference
        (:Is%20Valid
          ;[1 1 1] Send the Interact Message to the actor
          (Development|PrintString (Utilities|String|Append "[BC] Initiating Interact with: " (Utilities|GetDisplayName _interactactorreference)) true true "(R=1.000000,G=0.810099,B=0.522876,A=1.000000)")
          (Class|InteractInterface|DoInteract(Message) _interactactorreference))))))

(event Input|ActionEvents|InputActionAimThrow
  (params (Key :type Key%20Structure :default "None"))
  (bind _returnvalue (Game|GetPlayerController 0))
  (bind _returnvalue_2 (Game|GetPlayerController 0))
  (bind _returnvalue_3 (Pawn|GetControlRotation _returnvalue :!class /Script/Engine.Controller))
  (bind _returnvalue_4 (Pawn|GetControlRotation _returnvalue_2 :!class /Script/Engine.Controller))
  (:Pressed
    (Variables|Default|SetLMBPressed true)
    (Utilities|FlowControl|Delay 0.5)
    (if (Variables|Default|GetLMBPressed) :!label _label
      (Utilities|FlowControl|Gate true) ; enters at Open
      (else
        (CallFunction|ChangeMatBack)
        (Utilities|FlowControl|Gate true) ; enters at Close
      )))
  (:Released
    (Variables|Default|SetLMBPressed false)
    (goto _label)))

(event Input|KeyboardEvents|1
  (params (Key :type Key%20Structure :default "None"))
  ;[1 1 1] Swap the controller to small character
)

(event Input|MouseEvents|MouseWheelDown
  (params (Key :type Key%20Structure :default "None"))
  (bind _cameraboom (Variables|Default|GetCameraBoom))
  ;[0 0.7385 1] Scroll the camera out
  (:Pressed
    (Variables|/Script/Engine.SpringArmComponent|SetTargetArmLength _cameraboom (+ (Variables|/Script/Engine.SpringArmComponent|GetTargetArmLength _cameraboom) 1e+01))))

(event Input|MouseEvents|MouseWheelUp
  (params (Key :type Key%20Structure :default "None"))
  (bind _cameraboom (Variables|Default|GetCameraBoom))
  ;[0 0.7385 1] Scroll the camera out
  (:Pressed
    (Variables|/Script/Engine.SpringArmComponent|SetTargetArmLength _cameraboom (- (Variables|/Script/Engine.SpringArmComponent|GetTargetArmLength _cameraboom) 1e+01))))

(fn ConstructionScript)

(fn UpdateInteract
  (params (InteractActorReference :type Actor%20Object%20Reference) (CanInteract :type Boolean))
  (bind _output_get (Variables|Default|SetInteractActorReference InteractActorReference))
  (bind _output_get_2 (Variables|Default|SetCanInteract CanInteract))
  (Development|PrintString (Utilities|String|Append (Utilities|String|ToString(Boolean) _output_get_2) " interact with: " (Utilities|GetDisplayName _output_get))))

(fn EnablePlayerInput
  (Input|EnableInput (Game|GetPlayerController 0))
  (return))

(fn PickUpPlayer)

(fn DisablePlayerInput
  (Input|DisableInput (Game|GetPlayerController 0))
  (return))

(fn ThrowCharacter
  (bind _returnvalue (Pawn|GetControlRotation :!class /Script/Engine.Pawn))
  (Networking|SwitchHasAuthority
    (:Authority
      (bind _outactors (Actor|GetAllActorsOfClass "/Game/Blueprints/Characters/BP_SmallCharacter.BP_SmallCharacter_C"))
      (Actor|DestroyActor _outactors)
      (bind _returnvalue_2 (Game|SpawnActorfromClass "/Game/BP_ThrowPlayerProjectile.BP_ThrowPlayerProjectile_C" (select false "" (Math|Transform|MakeTransform (+ (Transformation|GetWorldLocation (Variables|Default|GetSphere)) (Math|Vector|RotateVector "0, 0, 0" _returnvalue)) _returnvalue)) "AlwaysSpawn" 0 0)) ; Spawn projectile
      (Game|Components|ProjectileMovement|SetVelocityinLocalSpace (Variables|/Game/BP_ThrowPlayerProjectile.BP_ThrowPlayerProjectile_C|GetProjectile _returnvalue_2) (Variables|Default|GetPlayerInitialVelocity)))
    (:Remote
      (Game|Player|SetViewTargetwithBlend (Game|GetPlayerController 1) 0 0.0 "VTBlend_Linear" 0.0 false)))
  (return))

(fn GetSegmentatTime
  (params (StartLocation :type Vector) (InitialVelocity :type Vector) (Gravity :type Vector) (Time1 :type Float%20%28single-precision%29) (Time2 :type Float%20%28single-precision%29))
  (return (+ StartLocation (* InitialVelocity Time1) (* Gravity (* Time1 Time1 0.5))) (+ StartLocation (* InitialVelocity Time2) (* Gravity (* Time2 Time2 0.5)))))

(fn DrawThrowTrajectory
  (params (VectorType :type Vector))
  (bind _returnvalue (Pawn|GetController))
  (bind _returnvalue_2 (Pawn|GetControlRotation :!class /Script/Engine.Pawn))
  (bind _sphere (Variables|Default|GetSphere))
  (bind _returnvalue_3 (Transformation|GetWorldLocation _sphere))
  (bind _returnvalue_4 (Math|Vector|RotateVector "0, 0, 0" _returnvalue_2))
  (bind _returnvalue_5 (Pawn|GetControlRotation _returnvalue :!class /Script/Engine.Controller))
  (bind _returnvalue_6 (+ _returnvalue_3 _returnvalue_4))
  (Variables|Default|SetStartLocation _returnvalue_6)
  (Variables|Default|SetInitialVelocity (Math|Transform|TransformDirection (Math|Transform|MakeTransform _returnvalue_6 _returnvalue_2) VectorType))
  (bind _index (Utilities|FlowControl|ForLoopwithBreak 0 (Math|Float|Floor (/ (Variables|Default|GetPathLifeTime) (Variables|Default|GetTimeInterval))))
    (:LoopBody
      (bind (_point1 _point2) (CallFunction|GetSegmentatTime (Variables|Default|GetStartLocation) (Variables|Default|GetInitialVelocity) "0, 0,-980.000000" (* _index (Variables|Default|GetTimeInterval)) (* (+ _index 1) (Variables|Default|GetTimeInterval))))
      (bind _returnvalue_7 (Collision|LineTraceByChannel _point1 _point2 "TraceTypeQuery1" true 0 "ForOneFrame"))
      (if _returnvalue_7
        (Pawn|SetControlRotation _returnvalue (Math|Rotator|MakeRotator (.roll _returnvalue_5) (Math|Float|ClampAngle (.pitch _returnvalue_5) -45.0 45.0) (.yaw _returnvalue_5)))
        (return)))))

(fn ChangeCameraView
  (params (CameraNumber :type Integer))
  (switch int CameraNumber
    (:0
      (Game|Player|SetViewTargetwithBlend (Game|GetPlayerController 0) self 1.0 "VTBlend_Linear" 0.0 false))
    (:1
      (Game|Player|SetViewTargetwithBlend (Game|GetPlayerController 0) (Variables|Default|GetStaticCamera1) 1.0 "VTBlend_Linear" 0.0 false))
    (:2
      (Game|Player|SetViewTargetwithBlend (Game|GetPlayerController 0) (Variables|Default|GetStaticCamera2) 1.0 "VTBlend_Linear" 0.0 false))
    (:3
      (Game|Player|SetViewTargetwithBlend (Game|GetPlayerController 0) (Variables|Default|GetStaticCamera3) 1.0 "VTBlend_Linear" 0.0 false))))

(fn ThrowBox
  (bind _returnvalue (Pawn|GetControlRotation :!class /Script/Engine.Pawn))
  (bind _returnvalue_2 (Pawn|GetControlRotation :!class /Script/Engine.Pawn))
  (Networking|SwitchHasAuthority
    (:Authority
      (Animation|PlayAnimMontage "/Game/Animations/Big/Big_ThrowAnim_Montage.Big_ThrowAnim_Montage" 1.0 "None")
      (if (Variables|Default|GetPickedUpBox)
        (bind _returnvalue_3 (Game|SpawnActorfromClass "/Game/Blueprints/Interactables/BigCharacterInteractable/BP_ThrowableBox.BP_ThrowableBox_C" (select false "" (Math|Transform|MakeTransform (+ (Transformation|GetWorldLocation (Variables|Default|GetSphere)) (Math|Vector|RotateVector "0, 0, 0" _returnvalue_2)) _returnvalue_2)) "AlwaysSpawn" 0 0)) ; Spawn projectile
        (Game|Components|ProjectileMovement|SetVelocityinLocalSpace (Variables|/Game/Blueprints/Interactables/BigCharacterInteractable/BP_ThrowableBox.BP_ThrowableBox_C|GetProjectileMovement _returnvalue_3) (Variables|Default|GetBoxInitialLocalVelocity))
        (return)
        (elif (Variables|Default|GetPickedUpBigBox)
          (bind _returnvalue_4 (Game|SpawnActorfromClass "/Game/Blueprints/Interactables/BigCharacterInteractable/BP_BigThrowableBox.BP_BigThrowableBox_C" (select false "" (Math|Transform|MakeTransform (+ (Transformation|GetWorldLocation (Variables|Default|GetSphere)) (Math|Vector|RotateVector "0, 0, 0" _returnvalue)) _returnvalue)) "AlwaysSpawn" 0 0)) ; Spawn projectile
          (Game|Components|ProjectileMovement|SetVelocityinLocalSpace (Variables|/Game/Blueprints/Interactables/BigCharacterInteractable/BP_BigThrowableBox.BP_BigThrowableBox_C|GetProjectileMovement _returnvalue_4) (Variables|Default|GetBoxInitialLocalVelocity))
          (return))))))

(fn ChangeCameraActor
  (params (ActorReference :type Actor%20Object%20Reference) (BlendTime :type Float%20%28single-precision%29))
  (Game|Player|SetViewTargetwithBlend (Game|GetPlayerController 0) ActorReference BlendTime "VTBlend_Linear" 0.0 false))

(fn NewFunction0)

(fn DoTouchAnimation
  (Animation|PlayAnimMontage "/Game/Animations/Big/Big_TouchAnim_Montage.Big_TouchAnim_Montage" 1.0 "None"))

(fn DetermineLMBHeldTime
  (if (Variables|Default|GetLMBPressed)
    (bind _output_get (Variables|Default|SetLMBHeldTime (Class|PlayerController|GetInputKeyTimeDown (Game|GetPlayerController 0) "LeftMouseButton")))
    (Development|PrintString (Utilities|String|ToString(Float) _output_get))))