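; Small playable character in a two-player setup that BP_BigCharacter can pick up and that can interact with other actors.
; Its outer sphere registers it as the big character's interactable, while its own Interact input messages the actor stored by UpdateInteract.
; DoInteract disables its input, blends player 1's camera to the big character, plays paired montages and socket-attaches it.
; Key 2 swaps controller possession between both characters for testing.
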(event OnComponentBeginOverlap(OuterCollisionSphere)
  (params (OverlappedComponent :type Primitive%20Component%20Object%20Reference) (OtherActor :type Actor%20Object%20Reference) (OtherComp :type Primitive%20Component%20Object%20Reference) (OtherBodyIndex :type Integer) (bFromSweep :type Boolean) (SweepResult :type Hit%20Result%20Structure%20%28by%20ref%29))
  (bind _asbp_big_character (Utilities|Casting|CastToBP_BigCharacter OtherActor))
  (Default|UpdateInteract _asbp_big_character self true))

(event OnComponentEndOverlap(OuterCollisionSphere)
  (params (OverlappedComponent :type Primitive%20Component%20Object%20Reference) (OtherActor :type Actor%20Object%20Reference) (OtherComp :type Primitive%20Component%20Object%20Reference) (OtherBodyIndex :type Integer))
  (bind _asbp_big_character (Utilities|Casting|CastToBP_BigCharacter OtherActor))
  (Default|UpdateInteract _asbp_big_character self false))

(event EventDoInteract
  (bind _bigcharacterreference (Variables|Default|GetBigCharacterReference))
  ;[1 1 1] Check if we've been picked up, if not then set this to true on both characters.
  (if (not (Variables|Default|GetIsCharacterPickedUp))
    (Variables|/Game/Blueprints/Characters/BP_BigCharacter.BP_BigCharacter_C|SetSmallCharacterPickedUp (Variables|Default|GetBigCharacterReference) true)
    (Variables|Default|SetIsCharacterPickedUp true)
    (CallFunction|DisablePlayerInput)
    (Game|Player|SetViewTargetwithBlend (Game|GetPlayerController 1) _bigcharacterreference 1.0 "VTBlend_EaseIn" 1.0 false)
    (Animation|PlayAnimMontage "/Game/Animations/Little/Little_PuPrepAnim_Montage.Little_PuPrepAnim_Montage" 1.0 "None")
    (Animation|PlayAnimMontage _bigcharacterreference "/Game/Animations/Big/Big_PickupAnim_Montage.Big_PickupAnim_Montage" 1.0 "None")
    (Transformation|SetActorLocation (Transformation|GetSocketLocation (Variables|/Script/Engine.Character|GetMesh (Variables|Default|GetBigCharacterReference)) "ApeRUpperArmDigit12") false false)
    (Transformation|SetActorRotation (Transformation|GetActorRotation (Variables|Default|GetBigCharacterReference)))
    (Transformation|AttachActorToActor self (Variables|Default|GetBigCharacterReference) "ApeRUpperArmDigit12" "KeepWorld" "KeepWorld" "KeepRelative" true)
    (Utilities|FlowControl|Delay 3.0)
    (Input|EnableInput (Variables|Default|GetBigCharacterReference) (Class|GameplayStatics|GetPlayerControllerfromID))))

(event EventBeginPlay
  (bind _outactors (Actor|GetAllActorsOfClass "/Game/Blueprints/Characters/BP_BigCharacter.BP_BigCharacter_C"))
  (Variables|Default|SetBigCharacterReference (Utilities|Array|Get(acopy) _outactors)))

(event Input|ActionEvents|InputActionInteract
  (params (Key :type Key%20Structure :default "None"))
  (bind _interactactorreference (Variables|Default|GetInteractActorReference))
  (:Pressed
    (Development|PrintString "[SC] Interact Pressed" true true "(R=1.000000,G=0.810099,B=0.522876,A=1.000000)")
    ;[1 1 1] Check if we're allowed to interact, Double check if the actor is valid
    (if (Variables|Default|GetCanInteract)
      (Utilities|IsValid _interactactorreference
        (:Is%20Valid
          ;[1 1 1] Send the Interact Message to the actor
          (Development|PrintString (Utilities|String|Append "[SC] Initiating Interact with: " (Utilities|GetDisplayName _interactactorreference)) true true "(R=1.000000,G=0.810099,B=0.522876,A=1.000000)")
          (Class|InteractInterface|DoInteract(Message) _interactactorreference))))))

(event Input|KeyboardEvents|2
  (params (Key :type Key%20Structure :default "None"))
  ;[1 1 1] Swap the controller to Big character
  (:Pressed
    (Development|PrintString "[SC] Controllers Swapped!" true true "(R=0.966663,G=1.000000,B=0.417691,A=1.000000)")
    (bind _outactors (Actor|GetAllActorsOfClass "/Game/Blueprints/Characters/BP_BigCharacter.BP_BigCharacter_C"))
    (Pawn|Possess (Game|GetPlayerController 0) (Utilities|Array|Get(acopy) _outactors))
    (Pawn|Possess (Game|GetPlayerController 1) self)))

(fn ConstructionScript)

(fn DisablePlayerInput
  (Input|DisableInput self (Class|GameplayStatics|GetPlayerControllerfromID 1))
  (return))

(fn EnablePlayerInput
  (Input|EnableInput self (Class|GameplayStatics|GetPlayerControllerfromID 1))
  (return))

(fn UpdateInteract
  (params (InteractActorReference :type Actor%20Object%20Reference) (CanInteract :type Boolean))
  (bind _output_get (Variables|Default|SetInteractActorReference InteractActorReference))
  (bind _output_get_2 (Variables|Default|SetCanInteract CanInteract))
  (Development|PrintString (Utilities|String|Append (Utilities|String|ToString(Boolean) _output_get_2) " interact with: " (Utilities|GetDisplayName _output_get))))