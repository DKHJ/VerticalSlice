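; Projectile that stands in for a thrown player and turns back into a playable small character on impact.
; ChangeCamera points player controller 0's view at the projectile, prints its name and stores its starting rotation.
; On an authority-side hit, ServerHit spawns BP_SmallCharacter at the sphere's location with the stored roll and yaw, has player controller 1 possess it, then destroys the projectile.
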(event Custom|Server%20Hit
  (bind _startrotation (Variables|Default|GetStartRotation))
  (bind _returnvalue (Game|SpawnActorfromClass "/Game/Blueprints/Characters/BP_SmallCharacter.BP_SmallCharacter_C" (Math|Transform|MakeTransform (Transformation|GetWorldLocation (Variables|Default|GetSphere1)) (Math|Rotator|MakeRotator (.roll _startrotation) 0.0 (.yaw _startrotation))) "AdjustIfPossibleButAlwaysSpawn" 0 0))
  (Pawn|Possess (Game|GetPlayerController 1) _returnvalue)
  (Actor|DestroyActor) ; Then destroy this projectile
)

(event Custom|ChangeCamera
  (bind _asnetwork_player_controller_bp (Utilities|Casting|CastToNetworkPlayerController_BP (Game|GetPlayerController 0)))
  (Game|Player|SetViewTargetwithBlend _asnetwork_player_controller_bp self 0.0 "VTBlend_Linear" 0.0 false)
  (Development|PrintString (Utilities|GetDisplayName 0) true true "(R=1.000000,G=0.651208,B=0.000000,A=1.000000)" 5.0)
  (Variables|Default|SetStartRotation (Transformation|GetActorRotation self)))

(event EventBeginPlay)

(event Collision|EventHit
  (params (MyComp :type Primitive%20Component%20Object%20Reference) (Other :type Actor%20Object%20Reference) (OtherComp :type Primitive%20Component%20Object%20Reference) (bSelfMoved :type Boolean) (HitLocation :type Vector :default "0, 0, 0") (HitNormal :type Vector :default "0, 0, 0") (NormalImpulse :type Vector :default "0, 0, 0") (Hit :type Hit%20Result%20Structure%20%28by%20ref%29))
  (Networking|SwitchHasAuthority
    (:Authority
      (CallFunction|ServerHit))))

(fn ConstructionScript)

(fn NewFunction0)