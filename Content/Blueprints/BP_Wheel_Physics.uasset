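; Physics wheel that the small character spins from inside to open linked vines.
; Overlapping the collision enables physics and activates the wheel; on tick, horizontal movement input adds angular velocity and a debug text shows the speed.
; Exceeding the goal speed opens the vines and dropping below closes them, with paired DoOnce nodes resetting each other to fire once per crossing.
; Leaving stops simulation and closes the vines if the goal was reached.
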(event OnComponentBeginOverlap(Collision)
  (params (OverlappedComponent :type Primitive%20Component%20Object%20Reference) (OtherActor :type Actor%20Object%20Reference) (OtherComp :type Primitive%20Component%20Object%20Reference) (OtherBodyIndex :type Integer) (bFromSweep :type Boolean) (SweepResult :type Hit%20Result%20Structure%20%28by%20ref%29))
  ;[0.3846 1 0.4252] Collision Handling, get a reference to the small player and set the wheel to active.
  (bind _asbp_small_character (Utilities|Casting|CastToBP_SmallCharacter OtherActor))
  (Variables|Default|SetSmallCharacterReference _asbp_small_character)
  (Variables|Default|SetbIsActive? true)
  (Physics|SetSimulatePhysics (Variables|Default|GetMesh) true))

(event OnComponentEndOverlap(Collision)
  (params (OverlappedComponent :type Primitive%20Component%20Object%20Reference) (OtherActor :type Actor%20Object%20Reference) (OtherComp :type Primitive%20Component%20Object%20Reference) (OtherBodyIndex :type Integer))
  ;[1 0.4995 0.5997] Collision Handling, player has left the wheel, deactivate.
  (Utilities|Casting|CastToBP_SmallCharacter OtherActor)
  (Variables|Default|SetbIsActive? false)
  (if (Variables|Default|GetGoalSpeedReached)
    (Default|Activated (Variables|Default|GetVinesReference) true))
  (Physics|SetSimulatePhysics (Variables|Default|GetMesh) false))

(event EventTick
  (params (DeltaSeconds :type Float%20%28single-precision%29))
  (bind _mesh (Variables|Default|GetMesh))
  (bind _returnvalue (Physics|GetPhysicsAngularVelocityinDegrees _mesh "None"))
  (bind _returnvalue_2 (Math|Float|Absolute(Float) (.y _returnvalue)))
  ;[1 1 1] We only want to tick if a player is in the wheel
  (if (Variables|Default|GetbIsActive?)
    ;[1 1 1] Get the players movement input ( 1 or -1 ) and add it to the physics wheels rotation velocity
    (Class|PrimitiveComponent|SetPhysicsAngularVelocityinDegrees (Variables|Default|GetMesh) (Math|Vector|MakeVector 0.0 (* 20 (.x (Pawn|Components|PawnMovement|GetLastInputVector (Variables|/Script/Engine.Character|GetCharacterMovement (Variables|Default|GetSmallCharacterReference))))) 0.0) true "None")
    ;[1 1 1] DEBUG: Show the speed
    (Rendering|Components|TextRender|SetText (Variables|Default|GetTextRender) (Utilities|Text|ToText(Float) _returnvalue_2 "HalfToEven"))
    ;[1 1 1] Check if the wheel is spinning faster than the goal speed
    (if (> _returnvalue_2 (Variables|Default|GetGoalThresholdSpeed))
      (Variables|Default|SetGoalSpeedReached true)
      (Utilities|FlowControl|DoOnce false :!label _label
        (:Completed
          (Default|Activated (Variables|Default|GetVinesReference) false)
          (Development|PrintString "Vine should open")
          (goto _label_2 Reset)))
      (elif (Variables|Default|GetGoalSpeedReached)
        (Variables|Default|SetGoalSpeedReached false)
        (Utilities|FlowControl|DoOnce false :!label _label_2
          (:Completed
            (Default|Activated (Variables|Default|GetVinesReference) true)
            (Development|PrintString "Vine should close")
            (goto _label Reset)))))))

(fn ConstructionScript)