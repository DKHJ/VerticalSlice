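; MapBoundary is an out-of-bounds volume that sends the big character, small character and throwable boxes to their own designated locations.
; On overlap with its collision component, it checks the actor's tag and teleports it to the matching location actor with zeroed rotation.
; Both characters get a fruit-drop sound and a short delay before teleporting, longer for the big one, while boxes move immediately and silently.
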(event OnComponentBeginOverlap(CollisionComponent)
  (params (OverlappedComponent :type Primitive%20Component%20Object%20Reference) (OtherActor :type Actor%20Object%20Reference) (OtherComp :type Primitive%20Component%20Object%20Reference) (OtherBodyIndex :type Integer) (bFromSweep :type Boolean) (SweepResult :type Hit%20Result%20Structure%20%28by%20ref%29))
  (if (Actor|ActorHasTag OtherActor "BigCharacter")
    (Audio|PlaySound2D "/Game/Audio/Props/Fruit_Drop/as_pr_Fruit_Drop_01.as_pr_Fruit_Drop_01" 1.0 1.0 0.0 0 0)
    (Utilities|FlowControl|Delay 1.0)
    (Transformation|Teleport OtherActor (Transformation|GetActorLocation (Variables|Default|GetBigCharTeleportLocation)) "0, 0, 0")
    (elif (Actor|ActorHasTag OtherActor "SmallCharacter")
      (Audio|PlaySound2D "/Game/Audio/Props/Fruit_Drop/as_pr_Fruit_Drop_01.as_pr_Fruit_Drop_01" 1.0 1.0 0.0 0 0)
      (Utilities|FlowControl|Delay 0.5)
      (Transformation|Teleport OtherActor (Transformation|GetActorLocation (Variables|Default|GetSmallCharTeleportLocation)) "0, 0, 0")
      (elif (Actor|ActorHasTag OtherActor "ThrowableBox")
        (Transformation|Teleport OtherActor (Transformation|GetActorLocation (Variables|Default|GetBoxTeleportLocation)) "0, 0, 0")))))

(event OnComponentEndOverlap(CollisionComponent)
  (params (OverlappedComponent :type Primitive%20Component%20Object%20Reference) (OtherActor :type Actor%20Object%20Reference) (OtherComp :type Primitive%20Component%20Object%20Reference) (OtherBodyIndex :type Integer)))

(fn ConstructionScript)