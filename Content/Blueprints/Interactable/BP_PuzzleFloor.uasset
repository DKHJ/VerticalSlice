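; BP_PuzzleFloor is an indexed, interactable puzzle floor piece whose mesh slides along a spline when activated.
; Interacting deactivates every active piece in the level, itself included, then toggles its own state, so the interacted piece always ends up activated.
; A timeline plays forward or reverses to move the mesh by spline distance.
; TryMove functions report whether each of four linked neighbour pieces is inactive.
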(event Custom|Activate
  (if (Variables|Default|GetIsActivated?)
    (bind _distance (Timeline|Timeline_0 Play)
      (:Update
        (Transformation|SetWorldLocation (Variables|Default|GetPuzzleMesh) (Spline|GetLocationatDistanceAlongSpline (Variables|Default|GetSpline) (* _distance (Spline|GetSplineLength (Variables|Default|GetSpline))) "World") false false)))
    (else
      (Timeline|Timeline_0 Reverse))))

(event Custom|DoInteract_1
  (CallFunction|ResetAllOtherPieces)
  (if (Variables|Default|GetIsActivated?)
    (Variables|Default|SetIsActivated? false)
    (else
      (Variables|Default|SetIsActivated? true)))
  (CallFunction|Activate))

(event EventBeginPlay
  (CallFunction|PostInitialise))

(fn ConstructionScript)

(fn PostInitialise
  (Rendering|Components|TextRender|SetText (Variables|Default|GetTextRender) (Utilities|Text|ToText(Integer) (Variables|Default|GetIndex)))
  (bind _outactors (Actor|GetAllActorsOfClass "BP_PuzzleFloor_C"))
  (Variables|Default|SetAllPieces _outactors))

(fn TryMoveLeft
  (bind _newparam (CallFunction|GetNextLeftNode))
  (if (Variables|BP_PuzzleFloor_C|GetIsActivated? _newparam)
    (return false)
    (else
      (return true))))

(fn GetNextLeftNode
  (return (Variables|NodeInfo|GetNextLeftNode)))

(fn GetNextRightNode
  (return (Variables|NodeInfo|GetNextRightNode)))

(fn TryMoveRight
  (bind _nextrightnode (CallFunction|GetNextRightNode))
  (if (Variables|BP_PuzzleFloor_C|GetIsActivated? _nextrightnode)
    (return false)
    (else
      (return true))))

(fn TryMoveUp
  (bind _nextupnode (CallFunction|GetNextUpNode))
  (if (Variables|BP_PuzzleFloor_C|GetIsActivated? _nextupnode)
    (return false)
    (else
      (return true))))

(fn TryMoveDown
  (bind _nextdownnode (CallFunction|GetNextDownNode))
  (if (Variables|BP_PuzzleFloor_C|GetIsActivated? _nextdownnode)
    (return false)
    (else
      (return true))))

(fn GetNextUpNode
  (return (Variables|NodeInfo|GetNextUpNode)))

(fn GetNextDownNode
  (return (Variables|NodeInfo|GetNextDownNode)))

(fn ResetAllOtherPieces
  (for _array_element (Variables|Default|GetAllPieces)
    (if (Variables|BP_PuzzleFloor_C|GetIsActivated? _array_element)
      (Variables|BP_PuzzleFloor_C|SetIsActivated? _array_element false)
      (CallFunction|Activate _array_element))))