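; BP_ColumnGridNode is one node in a Summer interactable column grid, tracking whether it is occupied and linking to up, down, left and right neighbours.
; Four check functions report whether the neighbour is free, the node to move to, and whether the grid ends.
; Unlike the others, the right check never flags a last node, and only the up check returns an occupied neighbour.
; Tick swaps the cube's material every frame to show occupancy.
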(event EventTick
  (params (DeltaSeconds :type Float%20%28single-precision%29))
  (if (Variables|Default|GetbIsOccupied?)
    (Rendering|Material|SetMaterial (Variables|Default|GetCube) 0 "/Game/Blueprints/Interactables/Crystals/Crystal_Spring_Inst.Crystal_Spring_Inst")
    (else
      (Rendering|Material|SetMaterial (Variables|Default|GetCube) 0 "/Game/Assets/BeanStalk/Beanstalk_MAT.Beanstalk_MAT"))))

(fn ConstructionScript)

(fn CheckMoveUp
  (bind _nextupnode (Variables|Default|GetNextUpNode))
  (Utilities|IsValid (Variables|Default|GetNextUpNode)
    (:Is%20Valid
      (if (Variables|BP_ColumnGridNode_C|GetbIsOccupied? _nextupnode)
        (return false _nextupnode false)
        (else
          (return true _nextupnode false))))
    (:Is%20Not%20Valid
      (return false 0 true))))

(fn CheckMoveDown
  (bind _nextdownnode (Variables|Default|GetNextDownNode))
  (Utilities|IsValid (Variables|Default|GetNextDownNode)
    (:Is%20Valid
      (if (Variables|BP_ColumnGridNode_C|GetbIsOccupied? _nextdownnode)
        (return false 0 false)
        (else
          (return true _nextdownnode false))))
    (:Is%20Not%20Valid
      (return false 0 true))))

(fn CheckMoveLeft
  (bind _nextleftnode (Variables|Default|GetNextLeftNode))
  (Utilities|IsValid (Variables|Default|GetNextLeftNode)
    (:Is%20Valid
      (if (Variables|BP_ColumnGridNode_C|GetbIsOccupied? _nextleftnode)
        (return false 0 false)
        (else
          (return true _nextleftnode false))))
    (:Is%20Not%20Valid
      (return false 0 true))))

(fn CheckMoveRight
  (bind _nextrightnode (Variables|Default|GetNextRightNode))
  (Utilities|IsValid (Variables|Default|GetNextRightNode)
    (:Is%20Valid
      (if (Variables|BP_ColumnGridNode_C|GetbIsOccupied? _nextrightnode)
        (return false 0 false)
        (else
          (return true _nextrightnode false))))
    (:Is%20Not%20Valid
      (return false 0 false))))