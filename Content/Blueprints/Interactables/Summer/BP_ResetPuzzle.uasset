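; Interactable that resets the column puzzle when triggered, playing a rune sound.
; Shortly after BeginPlay it caches every BP_Column and BP_ColumnGridNode in the level.
; Its collision overlap registers it as the interact target for BP_SmallCharacter and disables interaction on exit.
; DoInteract proceeds only with authority, calling ServerInteract to clear every grid node's occupancy and reset every column.
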(event OnComponentBeginOverlap(Collision)
  (params (OverlappedComponent :type Primitive%20Component%20Object%20Reference) (OtherActor :type Actor%20Object%20Reference) (OtherComp :type Primitive%20Component%20Object%20Reference) (OtherBodyIndex :type Integer) (bFromSweep :type Boolean) (SweepResult :type Hit%20Result%20Structure%20%28by%20ref%29))
  ;[1 0.3646 0.3646] Collision Handling
  (bind _asbp_small_character (Utilities|Casting|CastToBP_SmallCharacter OtherActor))
  (bind _output_get (Variables|Default|SetSmallCharReference _asbp_small_character))
  (Default|UpdateInteract _output_get self true))

(event OnComponentEndOverlap(Collision)
  (params (OverlappedComponent :type Primitive%20Component%20Object%20Reference) (OtherActor :type Actor%20Object%20Reference) (OtherComp :type Primitive%20Component%20Object%20Reference) (OtherBodyIndex :type Integer))
  ;[1 0.3646 0.3646] Collision Handling
  (bind _asbp_small_character (Utilities|Casting|CastToBP_SmallCharacter OtherActor))
  (Default|UpdateInteract _asbp_small_character 0 false))

(event Custom|Server%20Interact
  (CallFunction|ResetPuzzle))

(event Custom|ResetPuzzle
  (Audio|PlaySound2D "/Game/Audio/RuneInteractSound.RuneInteractSound" 1.0 1.0 0.0 0 0)
  (Development|PrintString "Here we want to reset the puzzle")
  (for _array_element (Variables|Default|GetAllColumnGrids)
    (Default|ClearOccupy _array_element))
  (for _array_element_2 (Variables|Default|GetAllColumnsReference)
    (Default|ResetSelf _array_element_2)))

(event EventBeginPlay
  (Utilities|FlowControl|Delay 0.2)
  (bind _outactors (Actor|GetAllActorsOfClass "/Game/Blueprints/Interactables/Summer/BP_Column.BP_Column_C"))
  (Variables|Default|SetAllColumnsReference _outactors)
  (bind _outactors_2 (Actor|GetAllActorsOfClass "/Game/Blueprints/Interactables/Summer/BP_ColumnGridNode.BP_ColumnGridNode_C"))
  (Variables|Default|SetAllColumnGrids _outactors_2))

(event EventDoInteract
  (Networking|SwitchHasAuthority
    (:Authority
      (CallFunction|ServerInteract))))

(fn ConstructionScript)