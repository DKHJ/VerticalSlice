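; Pushable column for a grid puzzle, kicked from any of four sides by BP_BigCharacter.
; Side overlaps set the push direction; on authority, interacting snaps the character into place and plays a kick montage.
; After a delay, it gathers the adjacent column chain through linked grid nodes and moves it last-to-first with timeline lerps.
; When all columns occupy their goal nodes, it calls Activated on the Waterfall-tagged BP_Vines.
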(event OnComponentBeginOverlap(DownCollision)
  (params (OverlappedComponent :type Primitive%20Component%20Object%20Reference) (OtherActor :type Actor%20Object%20Reference) (OtherComp :type Primitive%20Component%20Object%20Reference) (OtherBodyIndex :type Integer) (bFromSweep :type Boolean) (SweepResult :type Hit%20Result%20Structure%20%28by%20ref%29))
  ;[1 0.1864 0.2262] OVERLAP Handling
  (bind _asbp_big_character (Utilities|Casting|CastToBP_BigCharacter OtherActor))
  (Default|UpdateInteract _asbp_big_character self true)
  (Variables|Default|SetMoveDirection "NewEnumerator0")
  (Variables|Default|SetBigCharReference _asbp_big_character))

(event OnComponentEndOverlap(DownCollision)
  (params (OverlappedComponent :type Primitive%20Component%20Object%20Reference) (OtherActor :type Actor%20Object%20Reference) (OtherComp :type Primitive%20Component%20Object%20Reference) (OtherBodyIndex :type Integer))
  ;[1 0.1864 0.2262] OVERLAP Handling
  (bind _asbp_big_character (Utilities|Casting|CastToBP_BigCharacter OtherActor))
  (Default|UpdateInteract _asbp_big_character 0 false))

(event OnComponentBeginOverlap(UpCollision)
  (params (OverlappedComponent :type Primitive%20Component%20Object%20Reference) (OtherActor :type Actor%20Object%20Reference) (OtherComp :type Primitive%20Component%20Object%20Reference) (OtherBodyIndex :type Integer) (bFromSweep :type Boolean) (SweepResult :type Hit%20Result%20Structure%20%28by%20ref%29))
  ;[1 0.1864 0.2262] OVERLAP Handling
  (bind _asbp_big_character (Utilities|Casting|CastToBP_BigCharacter OtherActor))
  (Default|UpdateInteract _asbp_big_character self true)
  (Variables|Default|SetMoveDirection "NewEnumerator1")
  (Variables|Default|SetBigCharReference _asbp_big_character))

(event OnComponentEndOverlap(UpCollision)
  (params (OverlappedComponent :type Primitive%20Component%20Object%20Reference) (OtherActor :type Actor%20Object%20Reference) (OtherComp :type Primitive%20Component%20Object%20Reference) (OtherBodyIndex :type Integer))
  ;[1 0.1864 0.2262] OVERLAP Handling
  (bind _asbp_big_character (Utilities|Casting|CastToBP_BigCharacter OtherActor))
  (Default|UpdateInteract _asbp_big_character 0 false))

(event OnComponentBeginOverlap(LeftCollision)
  (params (OverlappedComponent :type Primitive%20Component%20Object%20Reference) (OtherActor :type Actor%20Object%20Reference) (OtherComp :type Primitive%20Component%20Object%20Reference) (OtherBodyIndex :type Integer) (bFromSweep :type Boolean) (SweepResult :type Hit%20Result%20Structure%20%28by%20ref%29))
  ;[1 0.1864 0.2262] OVERLAP Handling
  (bind _asbp_big_character (Utilities|Casting|CastToBP_BigCharacter OtherActor))
  (Default|UpdateInteract _asbp_big_character self true)
  (Variables|Default|SetMoveDirection "NewEnumerator3")
  (Variables|Default|SetBigCharReference _asbp_big_character))

(event OnComponentEndOverlap(LeftCollision)
  (params (OverlappedComponent :type Primitive%20Component%20Object%20Reference) (OtherActor :type Actor%20Object%20Reference) (OtherComp :type Primitive%20Component%20Object%20Reference) (OtherBodyIndex :type Integer))
  ;[1 0.1864 0.2262] OVERLAP Handling
  (bind _asbp_big_character (Utilities|Casting|CastToBP_BigCharacter OtherActor))
  (Default|UpdateInteract _asbp_big_character 0 false))

(event OnComponentBeginOverlap(RightCollision)
  (params (OverlappedComponent :type Primitive%20Component%20Object%20Reference) (OtherActor :type Actor%20Object%20Reference) (OtherComp :type Primitive%20Component%20Object%20Reference) (OtherBodyIndex :type Integer) (bFromSweep :type Boolean) (SweepResult :type Hit%20Result%20Structure%20%28by%20ref%29))
  ;[1 0.1864 0.2262] OVERLAP Handling
  (bind _asbp_big_character (Utilities|Casting|CastToBP_BigCharacter OtherActor))
  (Default|UpdateInteract _asbp_big_character self true)
  (Variables|Default|SetMoveDirection "NewEnumerator2")
  (Variables|Default|SetBigCharReference _asbp_big_character))

(event OnComponentEndOverlap(RightCollision)
  (params (OverlappedComponent :type Primitive%20Component%20Object%20Reference) (OtherActor :type Actor%20Object%20Reference) (OtherComp :type Primitive%20Component%20Object%20Reference) (OtherBodyIndex :type Integer))
  ;[1 0.1864 0.2262] OVERLAP Handling
  (bind _asbp_big_character (Utilities|Casting|CastToBP_BigCharacter OtherActor))
  (Default|UpdateInteract _asbp_big_character 0 false))

(event Custom|MoveUp
  ;[0.2235 0.9103 1] Interact Direction Handling
  (CallFunction|AnimateBigCharacter)
  (Utilities|FlowControl|Delay 1.6)
  ;;[1 1 1] Get an array of columns that we need to move in this direction
  (CallFunction|GetConnectedColumns)
  ;;[1 1 1] Loop through each connected column starting from the end, check if we can move, then move it
  (bind _arrayelement (Utilities|Array|ReverseforEachLoop (Variables|Default|GetColumnsToMove))
    (:LoopBody
      (bind (_canmove _nodetomoveto _islastnode) (Default|CheckMoveUp (Variables|BP_Column_C|GetCurrentGridNode _arrayelement)))
      (if _islastnode
        (Development|PrintString "Cannot Move Last Node " true true "(R=1.000000,G=0.036018,B=0.000000,A=1.000000)")
        (elif _canmove
          (Variables|BP_Column_C|SetMoveToNode (Variables|/Game/Blueprints/Interactables/Summer/BP_ColumnGridNode.BP_ColumnGridNode_C|GetOccupyingColumn (Variables|BP_Column_C|GetCurrentGridNode _arrayelement)) _nodetomoveto)
          (CallFunction|DoMovement (Variables|/Game/Blueprints/Interactables/Summer/BP_ColumnGridNode.BP_ColumnGridNode_C|GetOccupyingColumn (Variables|BP_Column_C|GetCurrentGridNode _arrayelement))))))
    (:Completed
      (Utilities|Array|Clear (Variables|Default|GetColumnsToMove))
      (bind _puzzlecomplete_ (CallFunction|CheckPuzzleComplete))
      (if _puzzlecomplete_
        (CallFunction|CompletePuzzle)))))

(event Custom|DoMovement
  (params (ColumnToMove :type BP%20Column%20Object%20Reference))
  (bind _movetonode (Variables|Default|GetMoveToNode))
  ;[1 0.8542 0.3886] Movement Event
  (Variables|/Game/Blueprints/Interactables/Summer/BP_ColumnGridNode.BP_ColumnGridNode_C|SetbIsOccupied? (Variables|PuzzleProperties|GetCurrentGridNode) false)
  (Variables|/Game/Blueprints/Interactables/Summer/BP_ColumnGridNode.BP_ColumnGridNode_C|SetOccupyingColumn (Variables|PuzzleProperties|GetCurrentGridNode) 0)
  (bind _output_get (Variables|Default|SetInitialLocation (Transformation|GetWorldLocation (Variables|Default|GetStaticMesh))))
  (Variables|/Game/Blueprints/Interactables/Summer/BP_ColumnGridNode.BP_ColumnGridNode_C|SetbIsOccupied? _movetonode true)
  (Variables|/Game/Blueprints/Interactables/Summer/BP_ColumnGridNode.BP_ColumnGridNode_C|SetOccupyingColumn _movetonode self)
  (Variables|PuzzleProperties|SetCurrentGridNode _movetonode)
  (bind _newtrack_0 (Timeline|Timeline_0 PlayFromStart)
    (:Update
      (Transformation|SetActorLocation (Math|Vector|Lerp(Vector) _output_get (Transformation|GetActorLocation (Variables|Default|GetMoveToNode)) _newtrack_0) false false))))

(event Custom|MoveDown
  ;[0.2235 0.9103 1] Interact Direction Handling
  (CallFunction|AnimateBigCharacter)
  (Utilities|FlowControl|Delay 1.6)
  ;;[1 1 1] Get an array of columns that we need to move in this direction
  (CallFunction|GetConnectedColumns)
  ;;[1 1 1] ^
  (bind _arrayelement (Utilities|Array|ReverseforEachLoop (Variables|Default|GetColumnsToMove))
    (:LoopBody
      (bind (_canmove _nodetomoveto _islastnode) (Default|CheckMoveDown (Variables|BP_Column_C|GetCurrentGridNode _arrayelement)))
      (if _islastnode
        (Development|PrintString "Cannot Move Last Node " true true "(R=1.000000,G=0.036018,B=0.000000,A=1.000000)")
        (elif _canmove
          (Variables|BP_Column_C|SetMoveToNode (Variables|/Game/Blueprints/Interactables/Summer/BP_ColumnGridNode.BP_ColumnGridNode_C|GetOccupyingColumn (Variables|BP_Column_C|GetCurrentGridNode _arrayelement)) _nodetomoveto)
          (CallFunction|DoMovement (Variables|/Game/Blueprints/Interactables/Summer/BP_ColumnGridNode.BP_ColumnGridNode_C|GetOccupyingColumn (Variables|BP_Column_C|GetCurrentGridNode _arrayelement))))))
    (:Completed
      (Utilities|Array|Clear (Variables|Default|GetColumnsToMove))
      (bind _puzzlecomplete_ (CallFunction|CheckPuzzleComplete))
      (if _puzzlecomplete_
        (CallFunction|CompletePuzzle)))))

(event Custom|CompletePuzzle
  (bind _vinereference (Variables|Default|GetVineReference))
  ;[0.4015 1 0.4162] COMPLETE Event
  (Development|PrintString "Puzzle Complete!" true true "(R=0.099998,G=1.000000,B=0.205036,A=1.000000)")
  (if (Utilities|IsValid _vinereference)
    (Default|Activated _vinereference false)))

(event Custom|ServerInteract
  ;[1 0.8542 0.3886] Interact Handling
  (Audio|PlaySound2D "/Game/Audio/Woosh-B8-www_fesliyanstudios_com.Woosh-B8-www_fesliyanstudios_com" 1.0 1.0 0.0 0 0)
  (switch Utilities|FlowControl|Switch|SwitchonEnum_Direction (Variables|Default|GetMoveDirection)
    (:NewEnumerator0
      (CallFunction|MoveUp))
    (:NewEnumerator1
      (CallFunction|MoveDown))
    (:NewEnumerator2
      (CallFunction|MoveLeft))
    (:NewEnumerator3
      (CallFunction|MoveRight))))

(event Custom|AnimateBigCharacter
  (bind _bigcharreference (Variables|Default|GetBigCharReference))
  (bind _bigcharreference_2 (Variables|Default|GetBigCharReference))
  (bind _bigcharreference_3 (Variables|Default|GetBigCharReference))
  (bind _bigcharreference_4 (Variables|Default|GetBigCharReference))
  (switch Utilities|FlowControl|Switch|SwitchonEnum_Direction (Variables|Default|GetMoveDirection)
    (:NewEnumerator0
      (Transformation|SetActorLocation (Variables|Default|GetBigCharReference) (Transformation|GetWorldLocation (Variables|Default|GetTeleportLocationUp)) false false)
      (Transformation|SetActorRotation _bigcharreference_2)
      (Animation|Montage|PlayMontage (Variables|/Script/Engine.Character|GetMesh _bigcharreference_2) "/Game/Animations/Big/Big_KickAnim_Montage.Big_KickAnim_Montage"))
    (:NewEnumerator1
      (Transformation|SetActorLocation (Variables|Default|GetBigCharReference) (Transformation|GetWorldLocation (Variables|Default|GetTeleportLocationDown)) false false)
      (Transformation|SetActorRotation _bigcharreference_4 "0,180.000000, 0")
      (Animation|Montage|PlayMontage (Variables|/Script/Engine.Character|GetMesh _bigcharreference_4) "/Game/Animations/Big/Big_KickAnim_Montage.Big_KickAnim_Montage"))
    (:NewEnumerator2
      (Transformation|SetActorLocation (Variables|Default|GetBigCharReference) (Transformation|GetWorldLocation (Variables|Default|GetTeleportLocationLeft)) false false)
      (Transformation|SetActorRotation _bigcharreference_3 "0.000000,-90.000000,0.000000")
      (Animation|Montage|PlayMontage (Variables|/Script/Engine.Character|GetMesh _bigcharreference_3) "/Game/Animations/Big/Big_KickAnim_Montage.Big_KickAnim_Montage"))
    (:NewEnumerator3
      (Transformation|SetActorLocation (Variables|Default|GetBigCharReference) (Transformation|GetWorldLocation (Variables|Default|GetTeleportLocationRight)) false false)
      (Transformation|SetActorRotation _bigcharreference "0.000000,90.000000,0.000000")
      (Animation|Montage|PlayMontage (Variables|/Script/Engine.Character|GetMesh _bigcharreference) "/Game/Animations/Big/Big_KickAnim_Montage.Big_KickAnim_Montage"))))

(event Custom|MoveLeft
  ;[0.2235 0.9103 1] Interact Direction Handling
  (CallFunction|AnimateBigCharacter)
  (Utilities|FlowControl|Delay 1.6)
  ;;[1 1 1] Get an array of columns that we need to move in this direction
  (CallFunction|GetConnectedColumns)
  ;;[1 1 1] ^
  (bind _arrayelement (Utilities|Array|ReverseforEachLoop (Variables|Default|GetColumnsToMove))
    (:LoopBody
      (bind (_canmove _nodetomoveto _islastnode) (Default|CheckMoveLeft (Variables|BP_Column_C|GetCurrentGridNode _arrayelement)))
      (if _islastnode
        (Development|PrintString "Cannot Move Last Node " true true "(R=1.000000,G=0.036018,B=0.000000,A=1.000000)")
        (elif _canmove
          (Variables|BP_Column_C|SetMoveToNode (Variables|/Game/Blueprints/Interactables/Summer/BP_ColumnGridNode.BP_ColumnGridNode_C|GetOccupyingColumn (Variables|BP_Column_C|GetCurrentGridNode _arrayelement)) _nodetomoveto)
          (CallFunction|DoMovement (Variables|/Game/Blueprints/Interactables/Summer/BP_ColumnGridNode.BP_ColumnGridNode_C|GetOccupyingColumn (Variables|BP_Column_C|GetCurrentGridNode _arrayelement))))))
    (:Completed
      (Utilities|Array|Clear (Variables|Default|GetColumnsToMove))
      (bind _puzzlecomplete_ (CallFunction|CheckPuzzleComplete))
      (if _puzzlecomplete_
        (CallFunction|CompletePuzzle)))))

(event Custom|MoveRight
  ;[0.2235 0.9103 1] Interact Direction Handling
  (CallFunction|AnimateBigCharacter)
  (Utilities|FlowControl|Delay 1.6)
  ;;[1 1 1] Get an array of columns that we need to move in this direction
  (CallFunction|GetConnectedColumns)
  ;;[1 1 1] ^
  (bind _arrayelement (Utilities|Array|ReverseforEachLoop (Variables|Default|GetColumnsToMove))
    (:LoopBody
      (bind (_canmove _nodetomoveto _islastnode) (Default|CheckMoveRight (Variables|BP_Column_C|GetCurrentGridNode _arrayelement)))
      (if _islastnode
        (Development|PrintString "Cannot Move Last Node " true true "(R=1.000000,G=0.036018,B=0.000000,A=1.000000)")
        (elif _canmove
          (Variables|BP_Column_C|SetMoveToNode (Variables|/Game/Blueprints/Interactables/Summer/BP_ColumnGridNode.BP_ColumnGridNode_C|GetOccupyingColumn (Variables|BP_Column_C|GetCurrentGridNode _arrayelement)) _nodetomoveto)
          (CallFunction|DoMovement (Variables|/Game/Blueprints/Interactables/Summer/BP_ColumnGridNode.BP_ColumnGridNode_C|GetOccupyingColumn (Variables|BP_Column_C|GetCurrentGridNode _arrayelement))))))
    (:Completed
      (Utilities|Array|Clear (Variables|Default|GetColumnsToMove))
      (bind _puzzlecomplete_ (CallFunction|CheckPuzzleComplete))
      (if _puzzlecomplete_
        (CallFunction|CompletePuzzle)))))

(event EventBeginPlay
  ;[1 1 1] BEGINPLAY event; Set ourselves a current grid reference, move there and set the spot to be occupied
  (Utilities|FlowControl|Delay 0.2)
  (if (Utilities|IsValid (Variables|PuzzleProperties|GetStartingGridNode))
    (Variables|PuzzleProperties|SetCurrentGridNode (Variables|PuzzleProperties|GetStartingGridNode))
    (Transformation|SetActorLocation (Transformation|GetActorLocation (Variables|PuzzleProperties|GetCurrentGridNode)) false false)
    (Variables|/Game/Blueprints/Interactables/Summer/BP_ColumnGridNode.BP_ColumnGridNode_C|SetbIsOccupied? (Variables|PuzzleProperties|GetCurrentGridNode) true)
    (Variables|/Game/Blueprints/Interactables/Summer/BP_ColumnGridNode.BP_ColumnGridNode_C|SetOccupyingColumn (Variables|PuzzleProperties|GetCurrentGridNode) self)
    ;[1 1 1] We want all the columns that exist
    (bind _outactors (Actor|GetAllActorsOfClass "BP_Column_C"))
    (bind _output_get (Variables|Default|SetAllColumns _outactors))
    (Variables|Default|SetTotalNumberOfColumns (Utilities|Array|Length _output_get))))

(event EventDoInteract
  ;[1 0.8542 0.3886] Interact Handling
  (Networking|SwitchHasAuthority
    (:Authority
      (CallFunction|ServerInteract))))

(fn ConstructionScript
  (bind _outactors (Actor|GetAllActorsOfClasswithTag "/Game/Blueprints/Interactables/Vines/BP_Vines.BP_Vines_C" "Waterfall"))
  (Variables|Default|SetVineReference (Utilities|Array|Get(acopy) _outactors)))

(fn GetConnectedColumns
  (Variables|Default|SetSearchingForColumns true)
  (Variables|Default|SetNodeToSearch (Variables|PuzzleProperties|GetCurrentGridNode))
  (while (Variables|Default|GetSearchingForColumns)
    (switch Utilities|FlowControl|Switch|SwitchonEnum_Direction (Variables|Default|GetMoveDirection)
      (:NewEnumerator0
        (if (Utilities|IsValid (Variables|/Game/Blueprints/Interactables/Summer/BP_ColumnGridNode.BP_ColumnGridNode_C|GetNextUpNode (Variables|Default|GetNodeToSearch)))
          (if (Variables|/Game/Blueprints/Interactables/Summer/BP_ColumnGridNode.BP_ColumnGridNode_C|GetbIsOccupied? (Variables|/Game/Blueprints/Interactables/Summer/BP_ColumnGridNode.BP_ColumnGridNode_C|GetNextUpNode (Variables|Default|GetNodeToSearch)))
            (Utilities|Array|AddUnique (Variables|Default|GetColumnsToMove) (Variables|/Game/Blueprints/Interactables/Summer/BP_ColumnGridNode.BP_ColumnGridNode_C|GetOccupyingColumn (Variables|Default|GetNodeToSearch)))
            (Variables|Default|SetNodeToSearch (Variables|/Game/Blueprints/Interactables/Summer/BP_ColumnGridNode.BP_ColumnGridNode_C|GetNextUpNode (Variables|Default|GetNodeToSearch)))
            (else
              (Utilities|Array|AddUnique (Variables|Default|GetColumnsToMove) (Variables|/Game/Blueprints/Interactables/Summer/BP_ColumnGridNode.BP_ColumnGridNode_C|GetOccupyingColumn (Variables|Default|GetNodeToSearch)))
              (Variables|Default|SetSearchingForLastNode false)
              (return)))
          (else
            (Variables|Default|SetSearchingForLastNode false)
            (return))))
      (:NewEnumerator1
        (if (Utilities|IsValid (Variables|/Game/Blueprints/Interactables/Summer/BP_ColumnGridNode.BP_ColumnGridNode_C|GetNextDownNode (Variables|Default|GetNodeToSearch)))
          (if (Variables|/Game/Blueprints/Interactables/Summer/BP_ColumnGridNode.BP_ColumnGridNode_C|GetbIsOccupied? (Variables|/Game/Blueprints/Interactables/Summer/BP_ColumnGridNode.BP_ColumnGridNode_C|GetNextDownNode (Variables|Default|GetNodeToSearch)))
            (Utilities|Array|AddUnique (Variables|Default|GetColumnsToMove) (Variables|/Game/Blueprints/Interactables/Summer/BP_ColumnGridNode.BP_ColumnGridNode_C|GetOccupyingColumn (Variables|Default|GetNodeToSearch)))
            (Variables|Default|SetNodeToSearch (Variables|/Game/Blueprints/Interactables/Summer/BP_ColumnGridNode.BP_ColumnGridNode_C|GetNextDownNode (Variables|Default|GetNodeToSearch)))
            (else
              (Utilities|Array|AddUnique (Variables|Default|GetColumnsToMove) (Variables|/Game/Blueprints/Interactables/Summer/BP_ColumnGridNode.BP_ColumnGridNode_C|GetOccupyingColumn (Variables|Default|GetNodeToSearch)))
              (Variables|Default|SetSearchingForLastNode false)
              (return)))
          (else
            (Variables|Default|SetSearchingForLastNode false)
            (return))))
      (:NewEnumerator2
        (if (Utilities|IsValid (Variables|/Game/Blueprints/Interactables/Summer/BP_ColumnGridNode.BP_ColumnGridNode_C|GetNextLeftNode (Variables|Default|GetNodeToSearch)))
          (if (Variables|/Game/Blueprints/Interactables/Summer/BP_ColumnGridNode.BP_ColumnGridNode_C|GetbIsOccupied? (Variables|/Game/Blueprints/Interactables/Summer/BP_ColumnGridNode.BP_ColumnGridNode_C|GetNextLeftNode (Variables|Default|GetNodeToSearch)))
            (Utilities|Array|AddUnique (Variables|Default|GetColumnsToMove) (Variables|/Game/Blueprints/Interactables/Summer/BP_ColumnGridNode.BP_ColumnGridNode_C|GetOccupyingColumn (Variables|Default|GetNodeToSearch)))
            (Variables|Default|SetNodeToSearch (Variables|/Game/Blueprints/Interactables/Summer/BP_ColumnGridNode.BP_ColumnGridNode_C|GetNextLeftNode (Variables|Default|GetNodeToSearch)))
            (else
              (Utilities|Array|Add (Variables|Default|GetColumnsToMove) (Variables|/Game/Blueprints/Interactables/Summer/BP_ColumnGridNode.BP_ColumnGridNode_C|GetOccupyingColumn (Variables|Default|GetNodeToSearch)))
              (Variables|Default|SetSearchingForLastNode false)
              (return)))
          (else
            (Variables|Default|SetSearchingForLastNode false)
            (return))))
      (:NewEnumerator3
        (if (Utilities|IsValid (Variables|/Game/Blueprints/Interactables/Summer/BP_ColumnGridNode.BP_ColumnGridNode_C|GetNextRightNode (Variables|Default|GetNodeToSearch)))
          (if (Variables|/Game/Blueprints/Interactables/Summer/BP_ColumnGridNode.BP_ColumnGridNode_C|GetbIsOccupied? (Variables|/Game/Blueprints/Interactables/Summer/BP_ColumnGridNode.BP_ColumnGridNode_C|GetNextRightNode (Variables|Default|GetNodeToSearch)))
            (Utilities|Array|AddUnique (Variables|Default|GetColumnsToMove) (Variables|/Game/Blueprints/Interactables/Summer/BP_ColumnGridNode.BP_ColumnGridNode_C|GetOccupyingColumn (Variables|Default|GetNodeToSearch)))
            (Variables|Default|SetNodeToSearch (Variables|/Game/Blueprints/Interactables/Summer/BP_ColumnGridNode.BP_ColumnGridNode_C|GetNextRightNode (Variables|Default|GetNodeToSearch)))
            (else
              (Utilities|Array|AddUnique (Variables|Default|GetColumnsToMove) (Variables|/Game/Blueprints/Interactables/Summer/BP_ColumnGridNode.BP_ColumnGridNode_C|GetOccupyingColumn (Variables|Default|GetNodeToSearch)))
              (Variables|Default|SetSearchingForLastNode false)
              (return)))
          (else
            (Variables|Default|SetSearchingForLastNode false)
            (return))))))
  (return))

(fn CheckPuzzleComplete
  (Variables|Default|SetCorrectNumberOfColumns 0)
  (for _array_element (Variables|Default|GetAllColumns)
    (if (== (Variables|BP_Column_C|GetCurrentGridNode _array_element) (Variables|BP_Column_C|GetGoalGridNode _array_element))
      (Math|Integer|IncrementInt (Variables|Default|GetCorrectNumberOfColumns))))
  (if (== (Variables|Default|GetCorrectNumberOfColumns) (Variables|Default|GetTotalNumberOfColumns))
    (return true)))

(fn ResetSelf
  (bind _startinggridnode (Variables|PuzzleProperties|GetStartingGridNode))
  (Variables|PuzzleProperties|SetCurrentGridNode _startinggridnode)
  (Variables|/Game/Blueprints/Interactables/Summer/BP_ColumnGridNode.BP_ColumnGridNode_C|SetbIsOccupied? _startinggridnode true)
  (Variables|/Game/Blueprints/Interactables/Summer/BP_ColumnGridNode.BP_ColumnGridNode_C|SetOccupyingColumn (Variables|PuzzleProperties|GetCurrentGridNode) self)
  (Transformation|SetWorldLocation (Variables|Default|GetScene) (Transformation|GetActorLocation (Variables|PuzzleProperties|GetCurrentGridNode)) false false))

(fn ClearOccupy
  (Variables|/Game/Blueprints/Interactables/Summer/BP_ColumnGridNode.BP_ColumnGridNode_C|SetbIsOccupied? (Variables|PuzzleProperties|GetCurrentGridNode) false)
  (return))