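; Interactable wheel that the small character runs in to drive linked cog wheels and control vines.
; Box overlap registers it for interaction and shows an outline; interacting toggles it and teleports the character onto the wheel.
; While active, Tick spins it and enabled cogs only during positive X velocity.
; The game instance's picked-up cog count unlocks a further cog and lets turning disable vine collision, restored on deactivation.
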(event OnComponentBeginOverlap(Box)
  (params (OverlappedComponent :type Primitive%20Component%20Object%20Reference) (OtherActor :type Actor%20Object%20Reference) (OtherComp :type Primitive%20Component%20Object%20Reference) (OtherBodyIndex :type Integer) (bFromSweep :type Boolean) (SweepResult :type Hit%20Result%20Structure%20%28by%20ref%29))
  (bind _asbp_small_character (Utilities|Casting|CastToBP_SmallCharacter OtherActor))
  (Variables|/Game/Blueprints/Characters/BP_SmallCharacter.BP_SmallCharacter_C|SetInteractActorReference _asbp_small_character self)
  (Variables|/Game/Blueprints/Characters/BP_SmallCharacter.BP_SmallCharacter_C|SetCanInteract _asbp_small_character true)
  (Variables|Default|SetSmallCharacterReference _asbp_small_character)
  (if (Variables|Default|GetActivated?)
    (Rendering|SetRenderCustomDepth (Variables|Default|GetStaticMesh) false)
    (else
      (Rendering|SetRenderCustomDepth (Variables|Default|GetStaticMesh) true))))

(event OnComponentEndOverlap(Box)
  (params (OverlappedComponent :type Primitive%20Component%20Object%20Reference) (OtherActor :type Actor%20Object%20Reference) (OtherComp :type Primitive%20Component%20Object%20Reference) (OtherBodyIndex :type Integer))
  (bind _asbp_small_character (Utilities|Casting|CastToBP_SmallCharacter OtherActor))
  (Variables|/Game/Blueprints/Characters/BP_SmallCharacter.BP_SmallCharacter_C|SetInteractActorReference _asbp_small_character 0)
  (Variables|/Game/Blueprints/Characters/BP_SmallCharacter.BP_SmallCharacter_C|SetCanInteract _asbp_small_character false)
  (Rendering|SetRenderCustomDepth (Variables|Default|GetStaticMesh) false)
  (Variables|Default|SetActivated? false)
  (CallFunction|Activate))

(event Custom|Activate
  (bind _vinesreference (Variables|Default|GetVinesReference))
  (if (Variables|Default|GetActivated?)
    (Components|Activation|Activate (Variables|Default|GetRotatingMovement) false)
    (Transformation|Teleport (Variables|Default|GetSmallCharacterReference) (Transformation|GetWorldLocation (Variables|Default|GetSphere)) "0, 0, 0")
    (else
      (Components|Activation|Deactivate (Variables|Default|GetRotatingMovement))
      (for _array_element (Variables|Default|GetCogWheels)
        (Default|DeactivateCogs _array_element)
        (bind _asnetwork_game_instance_bp (Utilities|Casting|CastToNetworkGameInstance_BP (Game|GetGameInstance)))
        (if (== (Variables|/Game/Blueprints/GameLogic/NetworkGameInstance_BP.NetworkGameInstance_BP_C|GetCogsPickedUp _asnetwork_game_instance_bp) 3)
          (Default|Activated _vinesreference true)
          (Collision|SetCollisionEnabled (Variables|/Game/Blueprints/Interactables/Vines/BP_Vines.BP_Vines_C|GetStaticMesh _vinesreference) "QueryAndPhysics")
          (Pawn|Components|CharacterMovement|SetMovementMode (Variables|/Script/Engine.Character|GetCharacterMovement (Variables|Default|GetSmallCharacterReference)) "MOVE_Walking" 0))))))

(event EventDoInteract
  (if (Variables|Default|GetActivated?)
    (Variables|Default|SetActivated? false)
    (else
      (Variables|Default|SetActivated? true)
      (Rendering|SetRenderCustomDepth (Variables|Default|GetStaticMesh) false) ; Renders the outlines
    ))
  (CallFunction|Activate))

(event EventTick
  (params (DeltaSeconds :type Float%20%28single-precision%29))
  (bind _vinesreference (Variables|Default|GetVinesReference))
  (if (Variables|Default|GetActivated?)
    (if (> (.x (Transformation|GetVelocity (Variables|Default|GetSmallCharacterReference))) 0.0)
      (Components|Activation|Activate (Variables|Default|GetRotatingMovement) false)
      (for _array_element (Variables|Default|GetCogWheels)
        (if (Variables|/Game/Blueprints/Interactables/Wheels+Cogs/BP_CogWheel.BP_CogWheel_C|GetActivated _array_element)
          (Default|ActivateCogs _array_element)
          (bind _asnetwork_game_instance_bp (Utilities|Casting|CastToNetworkGameInstance_BP (Game|GetGameInstance)))
          (if (== (Variables|/Game/Blueprints/GameLogic/NetworkGameInstance_BP.NetworkGameInstance_BP_C|GetCogsPickedUp _asnetwork_game_instance_bp) 2)
            (Variables|/Game/Blueprints/Interactables/Wheels+Cogs/BP_CogWheel.BP_CogWheel_C|SetActivated (Utilities|Array|Get(acopy) (Variables|Default|GetCogWheels) 4) true))))
      (bind _asnetwork_game_instance_bp_2 (Utilities|Casting|CastToNetworkGameInstance_BP (Game|GetGameInstance)))
      (if (== (Variables|/Game/Blueprints/GameLogic/NetworkGameInstance_BP.NetworkGameInstance_BP_C|GetCogsPickedUp _asnetwork_game_instance_bp_2) 3)
        (Default|Activated _vinesreference false)
        (Collision|SetCollisionEnabled (Variables|/Game/Blueprints/Interactables/Vines/BP_Vines.BP_Vines_C|GetStaticMesh _vinesreference) "NoCollision"))
      (else
        (Components|Activation|Deactivate (Variables|Default|GetRotatingMovement))
        (for _array_element_2 (Variables|Default|GetCogWheels)
          (Default|DeactivateCogs _array_element_2))))))

(fn ConstructionScript)