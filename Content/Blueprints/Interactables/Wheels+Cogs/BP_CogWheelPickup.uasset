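; Collectible cog wheel pickup that either the big or small character collects by walking into its box.
; On overlap it plays a 2D sound for any actor, then for those characters increments CogsPickedUp on the network game instance, prints the total and destroys itself.
; Despite the "[SERVER]" print label there is no authority check, and the owner-only visibility and cog widget nodes are left unconnected.
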(event OnComponentBeginOverlap(Box)
  (params (OverlappedComponent :type Primitive%20Component%20Object%20Reference) (OtherActor :type Actor%20Object%20Reference) (OtherComp :type Primitive%20Component%20Object%20Reference) (OtherBodyIndex :type Integer) (bFromSweep :type Boolean) (SweepResult :type Hit%20Result%20Structure%20%28by%20ref%29))
  (Audio|PlaySound2D "/Game/Audio/magic-idea-02-sound-effect-29898072__online-audio-converter_com_.magic-idea-02-sound-effect-29898072__online-audio-converter_com_" 1.0 1.0 0.0 0 0)
  (Utilities|FlowControl|Sequence
    (:then_0
      (Utilities|Casting|CastToBP_BigCharacter OtherActor))
    (:then_1
      (Utilities|Casting|CastToBP_SmallCharacter OtherActor)))
  (bind _asnetwork_game_instance_bp (Utilities|Casting|CastToNetworkGameInstance_BP (Game|GetGameInstance)))
  (bind _result (Math|Integer|IncrementInt (Variables|/Game/Blueprints/GameLogic/NetworkGameInstance_BP.NetworkGameInstance_BP_C|GetCogsPickedUp _asnetwork_game_instance_bp))
    (:%20%20
      (Development|PrintString (Utilities|String|Append "[SERVER] Cogs Collected: " (Utilities|String|ToString(Integer) _result)))
      (Actor|DestroyActor))))

(event EventBeginPlay)

(fn ConstructionScript)