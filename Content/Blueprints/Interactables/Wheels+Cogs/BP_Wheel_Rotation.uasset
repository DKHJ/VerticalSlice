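; Interactable wheel that the small character spins to drive cogwheels and clear vines in a networked game.
; Overlap makes the player the wheel's owner, so the client's Tick can send movement input to the server to set rotation rate.
; Passing the threshold speed with cogs in place runs activated cogs and, once all are collected, disables vine collision.
; Slowing down or leaving deactivates the cogs and, if the goal was reached, re-triggers the vines.
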(event OnComponentBeginOverlap(Collision)
  (params (OverlappedComponent :type Primitive%20Component%20Object%20Reference) (OtherActor :type Actor%20Object%20Reference) (OtherComp :type Primitive%20Component%20Object%20Reference) (OtherBodyIndex :type Integer) (bFromSweep :type Boolean) (SweepResult :type Hit%20Result%20Structure%20%28by%20ref%29))
  ;[0.3846 1 0.4252] Collision Handling, get a reference to the small player and set the wheel to active.
  (bind _asbp_small_character (Utilities|Casting|CastToBP_SmallCharacter OtherActor))
  (bind _output_get (Variables|Default|SetSmallCharacterReference _asbp_small_character))
  (Variables|Default|SetbIsActive? true)
  (Actor|SetOwner _output_get)
  (Components|Activation|Activate (Variables|Default|GetRotatingMovement) false)
  (Components|Activation|Deactivate (Variables|Default|GetHoverParticleSystem)))

(event OnComponentEndOverlap(Collision)
  (params (OverlappedComponent :type Primitive%20Component%20Object%20Reference) (OtherActor :type Actor%20Object%20Reference) (OtherComp :type Primitive%20Component%20Object%20Reference) (OtherBodyIndex :type Integer))
  ;[1 0.4995 0.5997] Collision Handling, player has left the wheel, deactivate.
  (Utilities|Casting|CastToBP_SmallCharacter OtherActor)
  (Variables|Default|SetbIsActive? false)
  (if (Variables|Default|GetGoalSpeedReached)
    (Default|Activated (Variables|Default|GetVinesReference) true))
  (Components|Activation|Deactivate (Variables|Default|GetRotatingMovement))
  (for _array_element (Variables|Default|GetCogWheels)
    (Default|DeactivateCogs _array_element)
    (Components|Activation|SetActive (Variables|Default|GetHoverParticleSystem) true false)))

(event Custom|CogLogic
  (bind _vinesreference (Variables|Default|GetVinesReference))
  (bind _numberofcogs (Variables|Default|GetNumberOfCogs))
  (for _array_element (Variables|Default|GetCogWheels)
    (if (Variables|/Game/Blueprints/Interactables/Wheels+Cogs/BP_CogWheel.BP_CogWheel_C|GetActivated _array_element)
      (Default|ActivateCogs _array_element)
      (bind _asnetwork_game_instance_bp (Utilities|Casting|CastToNetworkGameInstance_BP (Game|GetGameInstance)))
      (if (== (Variables|/Game/Blueprints/GameLogic/NetworkGameInstance_BP.NetworkGameInstance_BP_C|GetCogsPickedUp _asnetwork_game_instance_bp) _numberofcogs)
        (Variables|/Game/Blueprints/Interactables/Wheels+Cogs/BP_CogWheel.BP_CogWheel_C|SetActivated (Utilities|Array|Get(acopy) (Variables|Default|GetCogWheels) _numberofcogs) true))))
  (bind _asnetwork_game_instance_bp_2 (Utilities|Casting|CastToNetworkGameInstance_BP (Game|GetGameInstance)))
  (if (== (Variables|/Game/Blueprints/GameLogic/NetworkGameInstance_BP.NetworkGameInstance_BP_C|GetCogsPickedUp _asnetwork_game_instance_bp_2) (Variables|Default|GetNumberOfCogs))
    (Default|Activated _vinesreference false)
    (Collision|SetCollisionEnabled (Variables|/Game/Blueprints/Interactables/Vines/BP_Vines.BP_Vines_C|GetStaticMesh _vinesreference) "NoCollision")))

(event Custom|MoveWheelServer
  (params (LastInput_X :type Float%20%28single-precision%29))
  ;[1 1 1] Feed the Last input into our rotation of the wheel
  (bind _result (Math|Float|NegateFloat (* LastInput_X (Variables|Default|GetWheelRotationSpeed)))
    (:%20%20
      (Variables|/Script/Engine.RotatingMovementComponent|SetRotationRate (Variables|Default|GetRotatingMovement) (Math|Rotator|MakeRotator 0.0 _result 0.0))
      ;[1 1 1] Check if the wheel is spinning faster than the goal speed
      (if (> (Math|Float|Absolute(Float) (.pitch (Variables|/Script/Engine.RotatingMovementComponent|GetRotationRate (Variables|Default|GetRotatingMovement)))) (Variables|Default|GetGoalThresholdSpeed))
        (if (Variables|/Game/Blueprints/BP_CogWheelController.BP_CogWheelController_C|GetCogsInPlace (Variables|Default|GetCogWheelController))
          ;[0.6225 1 0.6817] We have reached the goal, do our goal logic.
          (Variables|Default|SetGoalSpeedReached true)
          (Utilities|FlowControl|DoOnce false :!label _label
            (:Completed
              (Components|Activation|Activate (Variables|Default|GetRotatingMovement) false)
              (CallFunction|CogLogic))))
        (elif (Variables|/Game/Blueprints/BP_CogWheelController.BP_CogWheelController_C|GetCogsInPlace (Variables|Default|GetCogWheelController))
          (for _array_element (Variables|Default|GetCogWheels)
            (Default|DeactivateCogs _array_element)
            ;[1 0.5098 0.4999] We have NOT reached our goal, do some handling to see if we were previously activated
            (if (Variables|Default|GetGoalSpeedReached)
              (Variables|Default|SetGoalSpeedReached false)
              (Components|Activation|Deactivate (Variables|Default|GetRotatingMovement))
              (Default|Activated (Variables|Default|GetVinesReference) true)
              (goto _label Reset)
              (else
                (goto _label Reset)))))))))

(event EventTick
  (params (DeltaSeconds :type Float%20%28single-precision%29))
  ;[1 1 1] We only want to tick if a player is in the wheel
  (if (Variables|Default|GetbIsActive?)
    ;[1 1 1] Check if we're running this on the client, pass the server our Last Input Vector on the X direction
    (Networking|SwitchHasAuthority
      (:Remote
        (CallFunction|MoveWheelServer (.x (Pawn|Components|PawnMovement|GetLastInputVector (Variables|/Script/Engine.Character|GetCharacterMovement (Variables|Default|GetSmallCharacterReference)))))))))

(fn ConstructionScript)