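; BP_WinterWheel is an interactable wheel that the small character toggles to drive the winter state of a referenced vines actor.
; Box overlap registers it as the interact target and controls outline highlighting; leaving clears the active flag.
; Activating starts rotation, teleports the character to the sphere and disables movement; deactivating reverses rotation, vines and movement lock.
; While active, Tick re-activates rotation on positive X velocity and switches camera on remote instances.
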(event OnComponentBeginOverlap(Box)
  (params (OverlappedComponent :type Primitive%20Component%20Object%20Reference) (OtherActor :type Actor%20Object%20Reference) (OtherComp :type Primitive%20Component%20Object%20Reference) (OtherBodyIndex :type Integer) (bFromSweep :type Boolean) (SweepResult :type Hit%20Result%20Structure%20%28by%20ref%29))
  (bind _asbp_small_character (Utilities|Casting|CastToBP_SmallCharacter OtherActor))
  (Variables|/Game/Blueprints/Characters/BP_SmallCharacter.BP_SmallCharacter_C|SetInteractActorReference _asbp_small_character self)
  (Variables|/Game/Blueprints/Characters/BP_SmallCharacter.BP_SmallCharacter_C|SetCanInteract _asbp_small_character true)
  (Variables|Default|SetSmallCharacterReference _asbp_small_character)
  (if (Variables|Default|GetActivated?)
    (Rendering|SetRenderCustomDepth (Variables|Default|GetStaticMesh) false)
    (else
      (Rendering|SetRenderCustomDepth (Variables|Default|GetStaticMesh) true))))

(event OnComponentEndOverlap(Box)
  (params (OverlappedComponent :type Primitive%20Component%20Object%20Reference) (OtherActor :type Actor%20Object%20Reference) (OtherComp :type Primitive%20Component%20Object%20Reference) (OtherBodyIndex :type Integer))
  (bind _asbp_small_character (Utilities|Casting|CastToBP_SmallCharacter OtherActor))
  (Variables|/Game/Blueprints/Characters/BP_SmallCharacter.BP_SmallCharacter_C|SetInteractActorReference _asbp_small_character self)
  (Variables|/Game/Blueprints/Characters/BP_SmallCharacter.BP_SmallCharacter_C|SetCanInteract _asbp_small_character false)
  (Rendering|SetRenderCustomDepth (Variables|Default|GetStaticMesh) false)
  (Variables|Default|SetActivated? false))

(event Custom|Activate
  (if (Variables|Default|GetActivated?)
    (Variables|/Game/Blueprints/Interactables/Vines/BP_WinterVines.BP_WinterVines_C|SetWinterVinesActivated (Variables|Default|GetVinesReference) true)
    (Components|Activation|Activate (Variables|Default|GetRotatingMovement) false)
    (Transformation|Teleport (Variables|Default|GetSmallCharacterReference) (Transformation|GetWorldLocation (Variables|Default|GetSphere)) "0, 0, 0")
    (Pawn|Components|CharacterMovement|DisableMovement (Variables|/Script/Engine.Character|GetCharacterMovement (Variables|Default|GetSmallCharacterReference)))
    (Default|Activated (Variables|Default|GetVinesReference) false)
    (else
      (Components|Activation|Deactivate (Variables|Default|GetRotatingMovement))
      (Default|Activated (Variables|Default|GetVinesReference) true)
      (Pawn|Components|CharacterMovement|SetMovementMode (Variables|/Script/Engine.Character|GetCharacterMovement (Variables|Default|GetSmallCharacterReference)) "MOVE_Walking" 0)
      (Variables|/Game/Blueprints/Interactables/Vines/BP_WinterVines.BP_WinterVines_C|SetWinterVinesActivated (Variables|Default|GetVinesReference) false))))

(event EventDoInteract
  (if (Variables|Default|GetActivated?)
    (Variables|Default|SetActivated? false)
    (else
      (Variables|Default|SetActivated? true)
      (Rendering|SetRenderCustomDepth (Variables|Default|GetStaticMesh) false)))
  (CallFunction|Activate))

(event EventTick
  (params (DeltaSeconds :type Float%20%28single-precision%29))
  (bind _rotatingmovement (Variables|Default|GetRotatingMovement))
  (if (Variables|Default|GetActivated?)
    (if (> (.x (Transformation|GetVelocity (Variables|Default|GetSmallCharacterReference))) 0.0)
      (Class|ActorComponent|SetIsReplicated _rotatingmovement true)
      (Components|Activation|Activate _rotatingmovement false)
      (Networking|SwitchHasAuthority
        (:Remote
          (Default|ChangeCamera (Variables|Default|GetSmallCharacterReference)))))))

(fn ConstructionScript)