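; Cog wheel interactable that spins a static mesh through a RotatingMovement component.
; On BeginPlay it can reverse the spin, start it immediately, and pick either the gear material or an indicator material based on its Visible flag.
; ActivateCogs and DeactivateCogs events start and stop the rotation, while a separate SetVisible function shows or hides the mesh.
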(event Custom|ActivateCogs
  (Components|Activation|Activate (Variables|Default|GetRotatingMovement) false))

(event Custom|DeactivateCogs
  (Components|Activation|Deactivate (Variables|Default|GetRotatingMovement)))

(event Custom|ConfigureCog
  (if (Variables|Default|GetReverseDirection)
    (Variables|/Script/Engine.RotatingMovementComponent|SetRotationRate (Variables|Default|GetRotatingMovement) "-180.000000, 0, 0"))
  (if (Variables|Default|GetVisible)
    (Rendering|Material|SetMaterial (Variables|Default|GetStaticMesh) 0 "/Game/Assets/WheelAndGear/WheelAndGears.WheelAndGears")
    (else
      (Rendering|Material|SetMaterial (Variables|Default|GetStaticMesh) 0 "/Game/Assets/WheelAndGear/GearIndicator_INS.GearIndicator_INS")))
  (if (Variables|Default|GetStartActivated)
    (Components|Activation|Activate (Variables|Default|GetRotatingMovement) false)))

(event EventBeginPlay
  (CallFunction|ConfigureCog))

(fn ConstructionScript)

(fn SetVisible
  (params (Visible :type Boolean))
  (if Visible
    (Rendering|SetVisibility (Variables|Default|GetStaticMesh) true false)
    (else
      (Rendering|SetVisibility (Variables|Default|GetStaticMesh) false false)))
  (return))