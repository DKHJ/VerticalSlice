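; Interactable wheel that the small character runs in to rotate it and switch a linked vines actor.
; Box overlap registers it as the character's interact target and shows a custom-depth outline; leaving deactivates it.
; Interacting toggles activation, teleporting the character to the sphere when turned on.
; Tick rotates it and disables vine collision only while activated with positive X velocity, otherwise stopping it and restoring vines per CogWheels entry.
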(event OnComponentBeginOverlap(Box)
  (params (OverlappedComponent :type Primitive%20Component%20Object%20Reference) (OtherActor :type Actor%20Object%20Reference) (OtherComp :type Primitive%20Component%20Object%20Reference) (OtherBodyIndex :type Integer) (bFromSweep :type Boolean) (SweepResult :type Hit%20Result%20Structure%20%28by%20ref%29))
  (bind _asbp_small_character (Utilities|Casting|CastToBP_SmallCharacter OtherActor))
  (Variables|/Game/Blueprints/Characters/BP_SmallCharacter.BP_SmallCharacter_C|SetInteractActorReference _asbp_small_character self)
  (Variables|/Game/Blueprints/Characters/BP_SmallCharacter.BP_SmallCharacter_C|SetCanInteract _asbp_small_character true)
  (Variables|Default|SetSmallCharacterReference _asbp_small_character)
  (if (Variables|Default|GetActivated?)
    (Rendering|SetRenderCustomDepth (Variables|Default|GetStaticMesh) false)
    (else
      (Rendering|SetRenderCustomDepth (Variables|Default|GetStaticMesh) true))))

(event OnComponentEndOverlap(Box)
  (params (OverlappedComponent :type Primitive%20Component%20Object%20Reference) (OtherActor :type Actor%20Object%20Reference) (OtherComp :type Primitive%20Component%20Object%20Reference) (OtherBodyIndex :type Integer))
  (bind _asbp_small_character (Utilities|Casting|CastToBP_SmallCharacter OtherActor))
  (Variables|/Game/Blueprints/Characters/BP_SmallCharacter.BP_SmallCharacter_C|SetInteractActorReference _asbp_small_character 0)
  (Variables|/Game/Blueprints/Characters/BP_SmallCharacter.BP_SmallCharacter_C|SetCanInteract _asbp_small_character false)
  (Rendering|SetRenderCustomDepth (Variables|Default|GetStaticMesh) false)
  (Variables|Default|SetActivated? false)
  (CallFunction|Activate))

(event Custom|Activate
  (bind _vinesreference (Variables|Default|GetVinesReference))
  (if (Variables|Default|GetActivated?)
    (Components|Activation|Activate (Variables|Default|GetRotatingMovement) false)
    (Transformation|Teleport (Variables|Default|GetSmallCharacterReference) (Transformation|GetWorldLocation (Variables|Default|GetSphere)) "0, 0, 0")
    (Default|Activated (Variables|Default|GetVinesReference) false)
    (else
      (Components|Activation|Deactivate (Variables|Default|GetRotatingMovement))
      (Default|Activated _vinesreference true)
      (Collision|SetCollisionEnabled (Variables|/Game/Blueprints/Interactables/Vines/BP_Vines.BP_Vines_C|GetStaticMesh _vinesreference) "QueryAndPhysics")
      (Pawn|Components|CharacterMovement|SetMovementMode (Variables|/Script/Engine.Character|GetCharacterMovement (Variables|Default|GetSmallCharacterReference)) "MOVE_Walking" 0))))

(event EventDoInteract
  (if (Variables|Default|GetActivated?)
    (Variables|Default|SetActivated? false)
    (else
      (Variables|Default|SetActivated? true)
      (Rendering|SetRenderCustomDepth (Variables|Default|GetStaticMesh) false) ; Renders the outlines
    ))
  (CallFunction|Activate))

(event EventTick
  (params (DeltaSeconds :type Float%20%28single-precision%29))
  (bind _vinesreference (Variables|Default|GetVinesReference))
  (bind _vinesreference_2 (Variables|Default|GetVinesReference))
  (if (Variables|Default|GetActivated?)
    (if (> (.x (Transformation|GetVelocity (Variables|Default|GetSmallCharacterReference))) 0.0)
      (Components|Activation|Activate (Variables|Default|GetRotatingMovement) false)
      (Default|Activated _vinesreference_2 false)
      (Collision|SetCollisionEnabled (Variables|/Game/Blueprints/Interactables/Vines/BP_Vines.BP_Vines_C|GetStaticMesh _vinesreference_2) "NoCollision")
      (else
        (Components|Activation|Deactivate (Variables|Default|GetRotatingMovement) :!label _label)
        (for _array_element (Variables|Default|GetCogWheels)
          (Default|Activated _vinesreference true)
          (Collision|SetCollisionEnabled (Variables|/Game/Blueprints/Interactables/Vines/BP_Vines.BP_Vines_C|GetStaticMesh _vinesreference) "QueryAndPhysics"))))
    (else
      (goto _label))))

(fn ConstructionScript)