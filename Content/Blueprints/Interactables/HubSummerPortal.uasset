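; Hub portal that sends the game to the SummerRevised level once both the big and small characters stand in its box.
; Box begin overlap identifies each character by actor tag, sets its presence flag and fires GoToSummerLevel when both match.
; Travel runs through a ServerTravel console command on player controller 0.
; End overlap tests the portal's own tags instead of the leaving actor's when clearing flags.
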(event OnComponentBeginOverlap(Box)
  (params (OverlappedComponent :type Primitive%20Component%20Object%20Reference) (OtherActor :type Actor%20Object%20Reference) (OtherComp :type Primitive%20Component%20Object%20Reference) (OtherBodyIndex :type Integer) (bFromSweep :type Boolean) (SweepResult :type Hit%20Result%20Structure%20%28by%20ref%29))
  (if (Actor|ActorHasTag OtherActor "BigCharacter")
    (bind _output_get (Variables|Default|SetBigCharacterPresent true))
    (if (Math|Boolean|Equal(Boolean) _output_get (stale _output_get_2)) :!label _label
      (CallFunction|GotoSummerLevel))
    (elif (Actor|ActorHasTag OtherActor "SmallCharacter")
      (bind _output_get_2 (Variables|Default|SetSmallCharacterPresent true))
      (goto _label))))

(event OnComponentEndOverlap(Box)
  (params (OverlappedComponent :type Primitive%20Component%20Object%20Reference) (OtherActor :type Actor%20Object%20Reference) (OtherComp :type Primitive%20Component%20Object%20Reference) (OtherBodyIndex :type Integer))
  (if (Actor|ActorHasTag "BigCharacter")
    (Variables|Default|SetBigCharacterPresent false)
    (elif (Actor|ActorHasTag "SmallCharacter")
      (Variables|Default|SetSmallCharacterPresent false))))

(event Custom|GoToSummerLevel
  (Development|ExecuteConsoleCommand "ServerTravel/Game/Levels/SummerRevised" (Game|GetPlayerController 0)))

(event EventBeginPlay)

(event Collision|EventActorBeginOverlap
  (params (OtherActor :type Actor%20Object%20Reference)))

(event EventTick
  (params (DeltaSeconds :type Float%20%28single-precision%29)))

(fn ConstructionScript)