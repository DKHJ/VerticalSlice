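; BP_SpringSmallPressurePlatform is a pressure platform that switches a linked vine bridge on and off when a throwable box is placed on or removed from it.
; Box overlap events run on the server only, filter for BP_ThrowableBox, and call ActivateVines on VineBridgeRef with true on entry and false on exit.
; Entry also stores the box reference.
; A separate Activated event forwards to DoInteract.
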(event OnComponentBeginOverlap(Box)
  (params (OverlappedComponent :type Primitive%20Component%20Object%20Reference) (OtherActor :type Actor%20Object%20Reference) (OtherComp :type Primitive%20Component%20Object%20Reference) (OtherBodyIndex :type Integer) (bFromSweep :type Boolean) (SweepResult :type Hit%20Result%20Structure%20%28by%20ref%29))
  ;[0.5748 1 0.5817] BEGIN overlap
  (Networking|SwitchHasAuthority
    (:Authority
      (bind _asbp_throwable_box (Utilities|Casting|CastToBP_ThrowableBox OtherActor))
      (Variables|Default|SetThrowBoxRef _asbp_throwable_box)
      (Default|ActivateVines (Variables|Default|GetVineBridgeRef) true))))

(event OnComponentEndOverlap(Box)
  (params (OverlappedComponent :type Primitive%20Component%20Object%20Reference) (OtherActor :type Actor%20Object%20Reference) (OtherComp :type Primitive%20Component%20Object%20Reference) (OtherBodyIndex :type Integer))
  ;[1 0.5208 0.5208] END overlap
  (Networking|SwitchHasAuthority
    (:Authority
      (Utilities|Casting|CastToBP_ThrowableBox OtherActor)
      (Default|ActivateVines (Variables|Default|GetVineBridgeRef) false))))

(event Custom|Activated
  (CallFunction|DoInteract))

(fn ConstructionScript)