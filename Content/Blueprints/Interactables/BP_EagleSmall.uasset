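; BP_EagleSmall is an interactable trigger volume that gives the small character a dedicated eagle camera view while inside its box.
; On begin overlap it calls the character's ChangeCamera with EagleCamera and snaps the controller to a fixed yaw.
; On end overlap it calls ChangeCamera again with the default camera index.
; Both changes run only on the non-authority (Remote) branch, so the server skips them.
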(event OnComponentBeginOverlap(Box)
  (params (OverlappedComponent :type Primitive%20Component%20Object%20Reference) (OtherActor :type Actor%20Object%20Reference) (OtherComp :type Primitive%20Component%20Object%20Reference) (OtherBodyIndex :type Integer) (bFromSweep :type Boolean) (SweepResult :type Hit%20Result%20Structure%20%28by%20ref%29))
  (bind _asbp_small_character (Utilities|Casting|CastToBP_SmallCharacter OtherActor))
  (bind _output_get (Variables|Default|SetSmallCharRef _asbp_small_character))
  (Networking|SwitchHasAuthority
    (:Remote
      (Default|ChangeCamera _output_get 9 (Variables|Default|GetEagleCamera))
      (Pawn|SetControlRotation (Pawn|GetController _output_get) (Math|Rotator|MakeRotator 0.0 0.0 4e+01)))))

(event OnComponentEndOverlap(Box)
  (params (OverlappedComponent :type Primitive%20Component%20Object%20Reference) (OtherActor :type Actor%20Object%20Reference) (OtherComp :type Primitive%20Component%20Object%20Reference) (OtherBodyIndex :type Integer))
  (bind _asbp_small_character (Utilities|Casting|CastToBP_SmallCharacter OtherActor))
  (Networking|SwitchHasAuthority
    (:Remote
      (Default|ChangeCamera _asbp_small_character 0 (Variables|Default|GetEagleCamera)))))

(fn ConstructionScript)