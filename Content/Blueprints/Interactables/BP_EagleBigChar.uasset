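; BP_EagleBigChar is a trigger volume that switches the big character's view to an eagle camera while that character is inside it.
; On box overlap begin, the server blends BP_BigCharacter's camera to EagleCamera and zeroes its controller rotation.
; On overlap end, the server blends the camera back to the character itself.
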(event OnComponentBeginOverlap(Box)
  (params (OverlappedComponent :type Primitive%20Component%20Object%20Reference) (OtherActor :type Actor%20Object%20Reference) (OtherComp :type Primitive%20Component%20Object%20Reference) (OtherBodyIndex :type Integer) (bFromSweep :type Boolean) (SweepResult :type Hit%20Result%20Structure%20%28by%20ref%29))
  (bind _asbp_big_character (Utilities|Casting|CastToBP_BigCharacter OtherActor))
  (bind _output_get (Variables|Default|SetBigCharRef _asbp_big_character))
  (Networking|SwitchHasAuthority
    (:Authority
      (Default|ChangeCameraActor _output_get (Variables|Default|GetEagleCamera) 0.5)
      (Pawn|SetControlRotation (Pawn|GetController _output_get) (Math|Rotator|MakeRotator 0.0 0.0 0.0)))))

(event OnComponentEndOverlap(Box)
  (params (OverlappedComponent :type Primitive%20Component%20Object%20Reference) (OtherActor :type Actor%20Object%20Reference) (OtherComp :type Primitive%20Component%20Object%20Reference) (OtherBodyIndex :type Integer))
  (bind _asbp_big_character (Utilities|Casting|CastToBP_BigCharacter OtherActor))
  (Networking|SwitchHasAuthority
    (:Authority
      (Default|ChangeCameraActor _asbp_big_character _asbp_big_character 0.5))))

(fn ConstructionScript)