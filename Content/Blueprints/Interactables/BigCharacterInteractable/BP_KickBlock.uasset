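; Kickable puzzle block that the Big Character kicks to slide across a linked node grid until the path ends.
; Four side collisions register it as the character's interactable and set the kick direction.
; On interact, it plays the kick montage and walks neighbour nodes to the last valid, non-activated one.
; A timeline lerps the mesh there in XY at fixed height, then updates the current node.
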(event OnComponentBeginOverlap(MoveUpCollision)
  (params (OverlappedComponent :type Primitive%20Component%20Object%20Reference) (OtherActor :type Actor%20Object%20Reference) (OtherComp :type Primitive%20Component%20Object%20Reference) (OtherBodyIndex :type Integer) (bFromSweep :type Boolean) (SweepResult :type Hit%20Result%20Structure%20%28by%20ref%29))
  ;[0 1 0.9925] Collision Entries
  (bind _asbp_big_character (Utilities|Casting|CastToBP_BigCharacter OtherActor))
  (Default|UpdateInteract _asbp_big_character self true)
  (Variables|Default|SetDirection "UP")
  (Variables|Default|SetBigCharacterReference _asbp_big_character))

(event OnComponentEndOverlap(MoveUpCollision)
  (params (OverlappedComponent :type Primitive%20Component%20Object%20Reference) (OtherActor :type Actor%20Object%20Reference) (OtherComp :type Primitive%20Component%20Object%20Reference) (OtherBodyIndex :type Integer))
  ;[0 1 0.9925] Collision Entries
  (bind _asbp_big_character (Utilities|Casting|CastToBP_BigCharacter OtherActor))
  (Default|UpdateInteract _asbp_big_character 0 false)
  (Variables|Default|SetDirection "NONE"))

(event OnComponentBeginOverlap(MoveDownCollision)
  (params (OverlappedComponent :type Primitive%20Component%20Object%20Reference) (OtherActor :type Actor%20Object%20Reference) (OtherComp :type Primitive%20Component%20Object%20Reference) (OtherBodyIndex :type Integer) (bFromSweep :type Boolean) (SweepResult :type Hit%20Result%20Structure%20%28by%20ref%29))
  ;[0 1 0.9925] Collision Entries
  (bind _asbp_big_character (Utilities|Casting|CastToBP_BigCharacter OtherActor))
  (Default|UpdateInteract _asbp_big_character self true)
  (Variables|Default|SetDirection "DOWN")
  (Variables|Default|SetBigCharacterReference _asbp_big_character))

(event OnComponentEndOverlap(MoveDownCollision)
  (params (OverlappedComponent :type Primitive%20Component%20Object%20Reference) (OtherActor :type Actor%20Object%20Reference) (OtherComp :type Primitive%20Component%20Object%20Reference) (OtherBodyIndex :type Integer))
  ;[0 1 0.9925] Collision Entries
  (bind _asbp_big_character (Utilities|Casting|CastToBP_BigCharacter OtherActor))
  (Default|UpdateInteract _asbp_big_character 0 false)
  (Variables|Default|SetDirection "NONE"))

(event OnComponentBeginOverlap(MoveLeftCollision)
  (params (OverlappedComponent :type Primitive%20Component%20Object%20Reference) (OtherActor :type Actor%20Object%20Reference) (OtherComp :type Primitive%20Component%20Object%20Reference) (OtherBodyIndex :type Integer) (bFromSweep :type Boolean) (SweepResult :type Hit%20Result%20Structure%20%28by%20ref%29))
  ;[0 1 0.9925] Collision Entries
  (bind _asbp_big_character (Utilities|Casting|CastToBP_BigCharacter OtherActor))
  (Default|UpdateInteract _asbp_big_character self true)
  (Variables|Default|SetDirection "LEFT")
  (Variables|Default|SetBigCharacterReference _asbp_big_character))

(event OnComponentEndOverlap(MoveLeftCollision)
  (params (OverlappedComponent :type Primitive%20Component%20Object%20Reference) (OtherActor :type Actor%20Object%20Reference) (OtherComp :type Primitive%20Component%20Object%20Reference) (OtherBodyIndex :type Integer))
  ;[0 1 0.9925] Collision Entries
  (bind _asbp_big_character (Utilities|Casting|CastToBP_BigCharacter OtherActor))
  (Default|UpdateInteract _asbp_big_character 0 false)
  (Variables|Default|SetDirection "NONE"))

(event OnComponentBeginOverlap(MoveRightCollision)
  (params (OverlappedComponent :type Primitive%20Component%20Object%20Reference) (OtherActor :type Actor%20Object%20Reference) (OtherComp :type Primitive%20Component%20Object%20Reference) (OtherBodyIndex :type Integer) (bFromSweep :type Boolean) (SweepResult :type Hit%20Result%20Structure%20%28by%20ref%29))
  ;[0 1 0.9925] Collision Entries
  (bind _asbp_big_character (Utilities|Casting|CastToBP_BigCharacter OtherActor))
  (Default|UpdateInteract _asbp_big_character self true)
  (Variables|Default|SetDirection "RIGHT")
  (Variables|Default|SetBigCharacterReference _asbp_big_character))

(event OnComponentEndOverlap(MoveRightCollision)
  (params (OverlappedComponent :type Primitive%20Component%20Object%20Reference) (OtherActor :type Actor%20Object%20Reference) (OtherComp :type Primitive%20Component%20Object%20Reference) (OtherBodyIndex :type Integer))
  ;[0 1 0.9925] Collision Entries
  (bind _asbp_big_character (Utilities|Casting|CastToBP_BigCharacter OtherActor))
  (Default|UpdateInteract _asbp_big_character 0 false)
  (Variables|Default|SetDirection "NONE"))

(event Custom|MoveUp
  (bind _upnode (Default|GetUpNode (Variables|Default|GetCurrent%20Node)))
  (if (and (not (Variables|/Game/Blueprints/Interactables/Winter/BP_GridNode.BP_GridNode_C|GetActivated? _upnode)) (Utilities|IsValid _upnode))
    (Variables|Default|SetNextNode _upnode)
    (Variables|Default|SetSearchingForLastNode true)
    (while (Variables|Default|GetSearchingForLastNode)
      (bind _upnode_2 (Default|GetUpNode (Variables|Default|GetNextNode)))
      (if (and (not (Variables|/Game/Blueprints/Interactables/Winter/BP_GridNode.BP_GridNode_C|GetActivated? _upnode_2)) (Utilities|IsValid _upnode_2))
        (Variables|Default|SetNextNode _upnode_2)
        (else
          (Variables|Default|SetLastNode (Variables|Default|GetNextNode))
          (Variables|Default|SetSearchingForLastNode false))))
    (CallFunction|DoMovement)))

(event Custom|MoveRight
  (bind _getrightnode (Default|GetRightNode (Variables|Default|GetCurrent%20Node)))
  (if (and (not (Variables|/Game/Blueprints/Interactables/Winter/BP_GridNode.BP_GridNode_C|GetActivated? _getrightnode)) (Utilities|IsValid _getrightnode))
    (Variables|Default|SetNextNode _getrightnode)
    (Variables|Default|SetSearchingForLastNode true)
    (while (Variables|Default|GetSearchingForLastNode)
      (bind _getrightnode_2 (Default|GetRightNode (Variables|Default|GetNextNode)))
      (if (and (not (Variables|/Game/Blueprints/Interactables/Winter/BP_GridNode.BP_GridNode_C|GetActivated? _getrightnode_2)) (Utilities|IsValid _getrightnode_2))
        (Variables|Default|SetNextNode _getrightnode_2)
        (else
          (Variables|Default|SetLastNode (Variables|Default|GetNextNode))
          (Variables|Default|SetSearchingForLastNode false))))
    (CallFunction|DoMovement)))

(event Custom|MoveDown
  (bind _upnode (Default|GetDownNode (Variables|Default|GetCurrent%20Node)))
  (if (and (not (Variables|/Game/Blueprints/Interactables/Winter/BP_GridNode.BP_GridNode_C|GetActivated? _upnode)) (Utilities|IsValid _upnode))
    (Variables|Default|SetNextNode _upnode)
    (Variables|Default|SetSearchingForLastNode true)
    (while (Variables|Default|GetSearchingForLastNode)
      (bind _upnode_2 (Default|GetDownNode (Variables|Default|GetNextNode)))
      (if (and (not (Variables|/Game/Blueprints/Interactables/Winter/BP_GridNode.BP_GridNode_C|GetActivated? _upnode_2)) (Utilities|IsValid _upnode_2))
        (Variables|Default|SetNextNode _upnode_2)
        (else
          (Variables|Default|SetLastNode (Variables|Default|GetNextNode))
          (Variables|Default|SetSearchingForLastNode false))))
    (CallFunction|DoMovement)))

(event Custom|MoveLeft
  (bind _upnode (Default|GetLeftNode (Variables|Default|GetCurrent%20Node)))
  (if (and (not (Variables|/Game/Blueprints/Interactables/Winter/BP_GridNode.BP_GridNode_C|GetActivated? _upnode)) (Utilities|IsValid _upnode))
    (Variables|Default|SetNextNode _upnode)
    (Variables|Default|SetSearchingForLastNode true)
    (while (Variables|Default|GetSearchingForLastNode)
      (bind _upnode_2 (Default|GetLeftNode (Variables|Default|GetNextNode)))
      (if (and (not (Variables|/Game/Blueprints/Interactables/Winter/BP_GridNode.BP_GridNode_C|GetActivated? _upnode_2)) (Utilities|IsValid _upnode_2))
        (Variables|Default|SetNextNode _upnode_2)
        (else
          (Variables|Default|SetLastNode (Variables|Default|GetNextNode))
          (Variables|Default|SetSearchingForLastNode false))))
    (CallFunction|DoMovement)))

(event Custom|DoMovement
  (bind _lastnode (Variables|Default|GetLastNode))
  (bind _returnvalue (Transformation|GetActorLocation _lastnode))
  (bind _time (Timeline|Timeline_0 PlayFromStart)
    (:Update
      (Transformation|SetWorldLocation (Variables|Default|GetStaticMesh) (Math|Vector|MakeVector (Math|Float|Lerp (.x (Transformation|GetActorLocation (Variables|Default|GetCurrent%20Node))) (.x _returnvalue) _time) (Math|Float|Lerp (.y (Transformation|GetActorLocation (Variables|Default|GetCurrent%20Node))) (.y _returnvalue) _time) -25.0) false false))
    (:Finished
      (Variables|Default|SetCurrent%20Node (Variables|Default|GetLastNode)))))

(event EventDoInteract
  (Animation|PlayAnimMontage (Variables|Default|GetBigCharacterReference) "/Game/Animations/Big/Big_KickAnim_Montage.Big_KickAnim_Montage" 3.0 "None")
  (switch string (Variables|Default|GetDirection)
    (:UP
      (CallFunction|MoveUp))
    (:DOWN
      (CallFunction|MoveDown))
    (:LEFT
      (CallFunction|MoveLeft))
    (:RIGHT
      (CallFunction|MoveRight))))

(fn ConstructionScript)