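; BP_WinterResetButton is an interactable button for BP_BigCharacter that resets its referenced kick block.
; Box overlap registers it as the character's interact target and toggles a custom-depth highlight on the mesh.
; DoInteract locks input, teleports the character into place for a touch montage, then after a short delay fires particles, resets the block and restores input.
; It also caches all runes for ResetAllOtherRunes, which is never called here; camera-switch nodes are unwired.
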(event OnComponentBeginOverlap(Box)
  (params (OverlappedComponent :type Primitive%20Component%20Object%20Reference) (OtherActor :type Actor%20Object%20Reference) (OtherComp :type Primitive%20Component%20Object%20Reference) (OtherBodyIndex :type Integer) (bFromSweep :type Boolean) (SweepResult :type Hit%20Result%20Structure%20%28by%20ref%29))
  (bind _asbp_big_character (Utilities|Casting|CastToBP_BigCharacter OtherActor))
  (Variables|/Game/Blueprints/Characters/BP_BigCharacter.BP_BigCharacter_C|SetInteractActorReference _asbp_big_character self)
  (Variables|/Game/Blueprints/Characters/BP_BigCharacter.BP_BigCharacter_C|SetbCanInteract _asbp_big_character true)
  (Variables|Default|SetBigCharRef _asbp_big_character)
  (Rendering|SetRenderCustomDepth (Variables|Default|GetStaticMesh) true))

(event OnComponentEndOverlap(Box)
  (params (OverlappedComponent :type Primitive%20Component%20Object%20Reference) (OtherActor :type Actor%20Object%20Reference) (OtherComp :type Primitive%20Component%20Object%20Reference) (OtherBodyIndex :type Integer))
  (bind _asbp_big_character (Utilities|Casting|CastToBP_BigCharacter OtherActor))
  (Variables|/Game/Blueprints/Characters/BP_BigCharacter.BP_BigCharacter_C|SetInteractActorReference _asbp_big_character 0)
  (Variables|/Game/Blueprints/Characters/BP_BigCharacter.BP_BigCharacter_C|SetbCanInteract _asbp_big_character false)
  (Rendering|SetRenderCustomDepth (Variables|Default|GetStaticMesh) false))

(event EventBeginPlay
  (bind _outactors (Actor|GetAllActorsOfClass "/Game/Blueprints/Interactables/BigCharacterInteractable/BP_Rune.BP_Rune_C"))
  (Variables|Default|SetAllRuneActors _outactors))

(event EventDoInteract
  (bind _bigcharref (Variables|Default|GetBigCharRef))
  (Audio|PlaySound2D "/Game/Audio/220171__gameaudio__flourish-spacey-1.220171__gameaudio__flourish-spacey-1" 1.0 1.0 0.0 0 0)
  (Default|DisablePlayerInput _bigcharref)
  (Transformation|Teleport _bigcharref (Transformation|GetWorldLocation (Variables|Default|GetAnimationLocation)) "0,180.000000, 0")
  (Animation|PlayAnimMontage (Variables|Default|GetBigCharRef) "/Game/Animations/Big/Big_TouchAnim_Montage.Big_TouchAnim_Montage" 1.0 "None")
  (Utilities|FlowControl|Delay 0.5)
  (Components|Activation|Activate (Variables|Default|GetTouchParticle_PAR) false)
  (Default|ResetBox (Variables|Default|GetKickBlockReference))
  (Default|EnablePlayerInput (Variables|Default|GetBigCharRef)))

(fn ConstructionScript)

(fn ResetAllOtherRunes
  (params (CurrentRune :type BP%20Rune%20Object%20Reference))
  (for _array_element (Variables|Default|GetAllRuneActors)
    (if (not (== _array_element CurrentRune))
      (if (Variables|/Game/Blueprints/Interactables/BigCharacterInteractable/BP_Rune.BP_Rune_C|GetActivated _array_element)
        (Variables|/Game/Blueprints/Interactables/BigCharacterInteractable/BP_Rune.BP_Rune_C|SetActivated _array_element false)
        (Default|DoInteract (Variables|/Game/Blueprints/Interactables/BigCharacterInteractable/BP_Rune.BP_Rune_C|GetMagicPlatformReference _array_element))))))