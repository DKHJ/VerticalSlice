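; BP_SummerImagePuzzleRune is an interactable puzzle rune that the big character touches to cycle its symbol toward a goal.
; Box overlap enables interaction and custom-depth highlighting; interacting plays a camera-blended touch sequence, then advances the number, text and decal.
; Each rune caches all runes in the level and, on reaching its goal, scans them with a running count of activated ones.
; At four, it turns their text green and switches both characters' cameras while vines activate on the bridge.
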(event OnComponentBeginOverlap(Box)
  (params (OverlappedComponent :type Primitive%20Component%20Object%20Reference) (OtherActor :type Actor%20Object%20Reference) (OtherComp :type Primitive%20Component%20Object%20Reference) (OtherBodyIndex :type Integer) (bFromSweep :type Boolean) (SweepResult :type Hit%20Result%20Structure%20%28by%20ref%29))
  (bind _asbp_big_character (Utilities|Casting|CastToBP_BigCharacter OtherActor))
  (Variables|/Game/Blueprints/Characters/BP_BigCharacter.BP_BigCharacter_C|SetbCanInteract _asbp_big_character true)
  (Default|UpdateInteract _asbp_big_character self true)
  (Variables|Default|SetBigCharRef _asbp_big_character)
  (Rendering|SetRenderCustomDepth (Variables|Default|GetStaticMesh) true))

(event OnComponentEndOverlap(Box)
  (params (OverlappedComponent :type Primitive%20Component%20Object%20Reference) (OtherActor :type Actor%20Object%20Reference) (OtherComp :type Primitive%20Component%20Object%20Reference) (OtherBodyIndex :type Integer))
  (bind _asbp_big_character (Utilities|Casting|CastToBP_BigCharacter OtherActor))
  (Variables|/Game/Blueprints/Characters/BP_BigCharacter.BP_BigCharacter_C|SetbCanInteract _asbp_big_character false)
  (Default|UpdateInteract _asbp_big_character 0 false)
  (Rendering|SetRenderCustomDepth (Variables|Default|GetStaticMesh) false))

(event Custom|CheckRunes
  (for _array_element (Variables|Default|GetAllRunes)
    (if (Variables|BP_SummerImagePuzzleRune_C|GetRuneActivated _array_element)
      (bind _result (Math|Integer|IncrementInt (Variables|Default|GetCompleteCount))
        (:%20%20
          (Development|PrintString (Utilities|String|ToString(Integer) _result))
          (if (== _result 4)
            (Development|PrintString "Puzzle Completed")
            (for _array_element_2 (Variables|Default|GetAllRunes)
              (Rendering|Components|TextRender|SetTextRenderColor (Variables|BP_SummerImagePuzzleRune_C|GetImage _array_element_2) (Variables|Default|GetColorGreen)))
            (CallFunction|ServerCompletePuzzle))))
      (else
        (Development|PrintString "puzzle incomplete")
        (Variables|Default|SetCompleteCount 0)))))

(event Custom|Server%20Complete%20Puzzle
  (Default|ChangeCameraView (Variables|Default|GetBigCharRef) 1)
  (bind _outactors (Actor|GetAllActorsOfClass "/Game/Blueprints/Characters/BP_SmallCharacter.BP_SmallCharacter_C"))
  (Default|ChangeCamera (Utilities|Array|Get(acopy) _outactors) 1)
  (Utilities|FlowControl|Delay 1.5)
  (Default|ActivateVines (Variables|Default|GetVinesBridgeReference) true)
  (Utilities|FlowControl|Delay 2.0)
  (Default|ChangeCameraView (Variables|Default|GetBigCharRef))
  (Default|ChangeCamera (Utilities|Array|Get(acopy) _outactors)))

(event EventBeginPlay
  (Rendering|Components|TextRender|SetText (Variables|Default|GetImage) (Utilities|Text|ToText(Integer) (Variables|Default|GetRuneNumber)))
  (bind _outactors (Actor|GetAllActorsOfClass "BP_SummerImagePuzzleRune_C"))
  (bind _output_get (Variables|Default|SetAllRunes _outactors))
  (CallFunction|ConfigureMesh _output_get))

(event EventDoInteract
  (bind _bigcharref (Variables|Default|GetBigCharRef))
  (bind _animationlocation (Variables|Default|GetAnimationLocation))
  (Default|ChangeCameraActor (Variables|Default|GetBigCharRef) self 0.5)
  (Default|DisablePlayerInput (Variables|Default|GetBigCharRef))
  (Transformation|Teleport (Variables|Default|GetBigCharRef) (Transformation|GetWorldLocation _animationlocation) (Transformation|GetWorldRotation _animationlocation))
  (Utilities|FlowControl|Delay 0.5)
  (Default|DoTouchAnimation (Variables|Default|GetBigCharRef))
  (Utilities|FlowControl|Delay 0.5)
  (CallFunction|IterateNumber)
  (CallFunction|ConfigureMesh)
  (Components|Activation|Activate (Variables|Default|GetParticleSystem) false)
  (Utilities|FlowControl|Delay 0.7)
  (Input|EnableInput _bigcharref 0)
  (Default|ChangeCameraActor _bigcharref _bigcharref 0.5)
  (if (== (Variables|Default|GetRuneNumber) (Variables|Default|GetGoalNumber))
    (Variables|Default|SetRuneActivated true)
    (Development|PrintString "rune activated")
    (CallFunction|CheckRunes)
    (Audio|PlaySound2D "/Game/Audio/RuneInteractSound.RuneInteractSound" 1.0 1.0 0.0 0 0)
    (else
      (Variables|Default|SetRuneActivated false))))

(fn ConstructionScript)

(fn ConfigureMesh
  (switch int (Variables|Default|GetRuneNumber)
    (:0
      (Rendering|Components|Decal|SetDecalMaterial (Variables|Default|GetDecal) "/Game/Assets/RunesAndPlatforms/NewRunesAndPillars/RuneMaterials/Rune_05_INS.Rune_05_INS"))
    (:1
      (Rendering|Components|Decal|SetDecalMaterial (Variables|Default|GetDecal) "/Game/Assets/RunesAndPlatforms/NewRunesAndPillars/RuneMaterials/Rune_06_INS.Rune_06_INS"))
    (:2
      (Rendering|Components|Decal|SetDecalMaterial (Variables|Default|GetDecal) "/Game/Assets/RunesAndPlatforms/NewRunesAndPillars/RuneMaterials/Rune_07_INS.Rune_07_INS"))
    (:3
      (Rendering|Components|Decal|SetDecalMaterial (Variables|Default|GetDecal) "/Game/Assets/RunesAndPlatforms/NewRunesAndPillars/RuneMaterials/Rune_08_INS.Rune_08_INS"))))

(fn IterateNumber
  (if (>= (Variables|Default|GetRuneNumber) 3)
    (bind _output_get (Variables|Default|SetRuneNumber 0))
    (else
      (bind _result (Math|Integer|IncrementInt (Variables|Default|GetRuneNumber))
        (:%20%20
          _))))
  (Rendering|Components|TextRender|SetText (Variables|Default|GetImage) (Utilities|Text|ToText(Integer) _output_get))
  (return))