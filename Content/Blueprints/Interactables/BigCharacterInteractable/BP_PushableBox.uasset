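; Pushable box interactable that the big character can shove and the small character cannot.
; Two trigger volumes, XBox and YBox, run identical logic: a big character entering turns on the Cube's physics simulation and sets IsPushing on its animation Blueprint.
; The big character leaving either volume clears both, while a small character entering either one turns physics off.
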(event OnComponentBeginOverlap(YBox)
  (params (OverlappedComponent :type Primitive%20Component%20Object%20Reference) (OtherActor :type Actor%20Object%20Reference) (OtherComp :type Primitive%20Component%20Object%20Reference) (OtherBodyIndex :type Integer) (bFromSweep :type Boolean) (SweepResult :type Hit%20Result%20Structure%20%28by%20ref%29))
  (Utilities|FlowControl|Sequence
    (:then_0
      (bind _asbp_big_character (Utilities|Casting|CastToBP_BigCharacter OtherActor))
      (Variables|/Game/Animations/Big/Big_AnimBP.Big_AnimBP_C|SetbIsPushing (Variables|/Game/Blueprints/Characters/BP_BigCharacter.BP_BigCharacter_C|GetBigAnimBP _asbp_big_character) true)
      (Physics|SetSimulatePhysics (Variables|Default|GetCube) true))
    (:then_1
      (Utilities|Casting|CastToBP_SmallCharacter OtherActor)
      (Physics|SetSimulatePhysics (Variables|Default|GetCube) false))))

(event OnComponentEndOverlap(YBox)
  (params (OverlappedComponent :type Primitive%20Component%20Object%20Reference) (OtherActor :type Actor%20Object%20Reference) (OtherComp :type Primitive%20Component%20Object%20Reference) (OtherBodyIndex :type Integer))
  (bind _asbp_big_character (Utilities|Casting|CastToBP_BigCharacter OtherActor))
  (Variables|/Game/Animations/Big/Big_AnimBP.Big_AnimBP_C|SetbIsPushing (Variables|/Game/Blueprints/Characters/BP_BigCharacter.BP_BigCharacter_C|GetBigAnimBP _asbp_big_character) false)
  (Physics|SetSimulatePhysics (Variables|Default|GetCube) false))

(event OnComponentBeginOverlap(XBox)
  (params (OverlappedComponent :type Primitive%20Component%20Object%20Reference) (OtherActor :type Actor%20Object%20Reference) (OtherComp :type Primitive%20Component%20Object%20Reference) (OtherBodyIndex :type Integer) (bFromSweep :type Boolean) (SweepResult :type Hit%20Result%20Structure%20%28by%20ref%29))
  (Utilities|FlowControl|Sequence
    (:then_0
      (bind _asbp_big_character (Utilities|Casting|CastToBP_BigCharacter OtherActor))
      (Variables|/Game/Animations/Big/Big_AnimBP.Big_AnimBP_C|SetbIsPushing (Variables|/Game/Blueprints/Characters/BP_BigCharacter.BP_BigCharacter_C|GetBigAnimBP _asbp_big_character) true)
      (Physics|SetSimulatePhysics (Variables|Default|GetCube) true))
    (:then_1
      (Utilities|Casting|CastToBP_SmallCharacter OtherActor)
      (Physics|SetSimulatePhysics (Variables|Default|GetCube) false))))

(event OnComponentEndOverlap(XBox)
  (params (OverlappedComponent :type Primitive%20Component%20Object%20Reference) (OtherActor :type Actor%20Object%20Reference) (OtherComp :type Primitive%20Component%20Object%20Reference) (OtherBodyIndex :type Integer))
  (bind _asbp_big_character (Utilities|Casting|CastToBP_BigCharacter OtherActor))
  (Variables|/Game/Animations/Big/Big_AnimBP.Big_AnimBP_C|SetbIsPushing (Variables|/Game/Blueprints/Characters/BP_BigCharacter.BP_BigCharacter_C|GetBigAnimBP _asbp_big_character) false)
  (Physics|SetSimulatePhysics (Variables|Default|GetCube) false))

(fn ConstructionScript)