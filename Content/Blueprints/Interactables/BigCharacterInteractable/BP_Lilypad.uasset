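; BP_Lilypad is an interactable that the big character can push.
; When that character enters CollisionBox, it becomes the actor's owner, its anim Blueprint's pushing flag turns on and MeshCube starts simulating physics.
; Leaving clears the flag, physics and custom depth, and prints a debug "Hello".
; Overlaps branch on the other actor's first tag; small-character branches only cast, and the interact-prompt and highlight-enable nodes are unwired.
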(event OnComponentBeginOverlap(CollisionBox)
  (params (OverlappedComponent :type Primitive%20Component%20Object%20Reference) (OtherActor :type Actor%20Object%20Reference) (OtherComp :type Primitive%20Component%20Object%20Reference) (OtherBodyIndex :type Integer) (bFromSweep :type Boolean) (SweepResult :type Hit%20Result%20Structure%20%28by%20ref%29))
  ;[0.5778 1 0.571] BEGIN Overlap
  (switch string (Utilities|String|ToString(Name) (Utilities|Array|Get(acopy) (Variables|/Script/Engine.Actor|GetTags OtherActor)))
    (:BigCharacter
      (bind _asbp_big_character (Utilities|Casting|CastToBP_BigCharacter OtherActor))
      (bind _output_get (Variables|Default|SetBigCharRef _asbp_big_character))
      (Actor|SetOwner _output_get)
      (Variables|/Game/Animations/Big/Big_AnimBP.Big_AnimBP_C|SetbIsPushing (Variables|/Game/Blueprints/Characters/BP_BigCharacter.BP_BigCharacter_C|GetBigAnimBP (Variables|Default|GetBigCharRef)) true)
      (Physics|SetSimulatePhysics (Variables|Default|GetMeshCube) true))
    (:SmallCharacter
      (Utilities|Casting|CastToBP_SmallCharacter OtherActor))))

(event OnComponentEndOverlap(CollisionBox)
  (params (OverlappedComponent :type Primitive%20Component%20Object%20Reference) (OtherActor :type Actor%20Object%20Reference) (OtherComp :type Primitive%20Component%20Object%20Reference) (OtherBodyIndex :type Integer))
  ;[1 0.5411 0.5311] END Overlap
  (switch string (Utilities|String|ToString(Name) (Utilities|Array|Get(acopy) (Variables|/Script/Engine.Actor|GetTags OtherActor)))
    (:BigCharacter
      (Utilities|Casting|CastToBP_BigCharacter OtherActor)
      (Development|PrintString "Hello")
      (Variables|/Game/Animations/Big/Big_AnimBP.Big_AnimBP_C|SetbIsPushing (Variables|/Game/Blueprints/Characters/BP_BigCharacter.BP_BigCharacter_C|GetBigAnimBP (Variables|Default|GetBigCharRef)) false)
      (Rendering|SetRenderCustomDepth (Variables|Default|GetMeshCube) false)
      (Physics|SetSimulatePhysics (Variables|Default|GetMeshCube) false))
    (:SmallCharacter
      (Utilities|Casting|CastToBP_SmallCharacter OtherActor))))

(fn ConstructionScript)