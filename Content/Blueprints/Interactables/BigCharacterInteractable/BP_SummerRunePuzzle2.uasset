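; Timed rune pillar puzzle that the Big Character interacts with, highlighted while the character is inside its box.
; On the authority, Tick uses a Delay to cycle the rune number and pillar mesh about every second until completion.
; Interacting plays a camera-and-touch sequence, then compares the rune to its goal number.
; A single match completes it, turning all BP_ImagePuzzleRune texts green and triggering the linked vine during a camera view change.
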(event OnComponentBeginOverlap(Box)
  (params (OverlappedComponent :type Primitive%20Component%20Object%20Reference) (OtherActor :type Actor%20Object%20Reference) (OtherComp :type Primitive%20Component%20Object%20Reference) (OtherBodyIndex :type Integer) (bFromSweep :type Boolean) (SweepResult :type Hit%20Result%20Structure%20%28by%20ref%29))
  (bind _asbp_big_character (Utilities|Casting|CastToBP_BigCharacter OtherActor))
  (Variables|/Game/Blueprints/Characters/BP_BigCharacter.BP_BigCharacter_C|SetCanInteract _asbp_big_character true)
  (Default|UpdateInteract _asbp_big_character self true)
  (Variables|Default|SetBigCharRef _asbp_big_character)
  (Rendering|SetRenderCustomDepth (Variables|Default|GetStaticMesh) true))

(event OnComponentEndOverlap(Box)
  (params (OverlappedComponent :type Primitive%20Component%20Object%20Reference) (OtherActor :type Actor%20Object%20Reference) (OtherComp :type Primitive%20Component%20Object%20Reference) (OtherBodyIndex :type Integer))
  (bind _asbp_big_character (Utilities|Casting|CastToBP_BigCharacter OtherActor))
  (Variables|/Game/Blueprints/Characters/BP_BigCharacter.BP_BigCharacter_C|SetCanInteract _asbp_big_character false)
  (Default|UpdateInteract _asbp_big_character 0 false)
  (Rendering|SetRenderCustomDepth (Variables|Default|GetStaticMesh) false))

(event Custom|CheckRunes
  (if (Variables|Default|GetRuneActivated self)
    (bind _result (Math|Integer|IncrementInt (Variables|Default|GetCompleteCount))
      (:%20%20
        (Development|PrintString (Utilities|String|ToString(Integer) _result))
        (if (== _result 1)
          (Development|PrintString "Puzzle Completed")
          (for _array_element (Variables|Default|GetAllRunes)
            (Rendering|Components|TextRender|SetTextRenderColor (Variables|/Game/Blueprints/Interactables/BigCharacterInteractable/BP_ImagePuzzleRune.BP_ImagePuzzleRune_C|GetImage _array_element) (Variables|Default|GetColorGreen)))
          (Default|ChangeCameraView (Variables|Default|GetBigCharRef) 2)
          (Utilities|FlowControl|Delay 1.5)
          (Default|Activated (Variables|Default|GetVineReference) false)
          (Utilities|FlowControl|Delay 2.0)
          (Default|ChangeCameraView (Variables|Default|GetBigCharRef))
          (Variables|Default|SetPuzzleCompleted true))))
    (else
      (Development|PrintString "puzzle incomplete")
      (Variables|Default|SetCompleteCount 0))))

(event EventTick
  (params (DeltaSeconds :type Float%20%28single-precision%29))
  (Networking|SwitchHasAuthority
    (:Authority
      (if (not (Variables|Default|GetPuzzleCompleted))
        (Utilities|FlowControl|Delay 1.0)
        (CallFunction|IterateNumber)
        (CallFunction|ConfigureMesh)))))

(event EventBeginPlay
  (Rendering|Components|TextRender|SetText (Variables|Default|GetImage) (Utilities|Text|ToText(Integer) (Variables|Default|GetRuneNumber)))
  (bind _outactors (Actor|GetAllActorsOfClass "/Game/Blueprints/Interactables/BigCharacterInteractable/BP_ImagePuzzleRune.BP_ImagePuzzleRune_C"))
  (Variables|Default|SetAllRunes _outactors)
  (CallFunction|ConfigureMesh))

(event EventDoInteract
  (bind _bigcharref (Variables|Default|GetBigCharRef))
  (Default|ChangeCameraActor (Variables|Default|GetBigCharRef) self 0.5)
  (Default|DisablePlayerInput (Variables|Default|GetBigCharRef))
  (Transformation|Teleport (Variables|Default|GetBigCharRef) (Transformation|GetWorldLocation (Variables|Default|GetAnimationLocation)) "0, 0, 0")
  (Utilities|FlowControl|Delay 0.5)
  (Default|DoTouchAnimation (Variables|Default|GetBigCharRef))
  (Utilities|FlowControl|Delay 0.5)
  (Components|Activation|Activate (Variables|Default|GetParticleSystem) false)
  (Utilities|FlowControl|Delay 0.7)
  (Input|EnableInput _bigcharref 0)
  (Default|ChangeCameraActor _bigcharref _bigcharref 0.5)
  (if (== (Variables|Default|GetRuneNumber) (Variables|Default|GetGoalNumber))
    (Variables|Default|SetRuneActivated true)
    (Development|PrintString "rune activated")
    (CallFunction|CheckRunes)
    (else
      (Variables|Default|SetRuneActivated false))))

(fn ConstructionScript)

(fn ConfigureMesh
  (switch int (Variables|Default|GetRuneNumber)
    (:0
      (Components|StaticMesh|SetStaticMesh (Variables|Default|GetStaticMesh) "/Game/Assets/RunePillars/RunePillar2_Low.RunePillar2_Low"))
    (:1
      (Components|StaticMesh|SetStaticMesh (Variables|Default|GetStaticMesh) "/Game/Assets/RunePillars/RunePillarButton_Low.RunePillarButton_Low"))
    (:2
      (Components|StaticMesh|SetStaticMesh (Variables|Default|GetStaticMesh) "/Game/Assets/RunePillars/RunePillar3_Low.RunePillar3_Low"))
    (:3
      (Components|StaticMesh|SetStaticMesh (Variables|Default|GetStaticMesh) "/Game/Assets/RunePillars/RunePillar4_Low.RunePillar4_Low"))))

(fn IterateNumber
  (if (>= (Variables|Default|GetRuneNumber) 3)
    (bind _output_get (Variables|Default|SetRuneNumber 0))
    (else
      (bind _result (Math|Integer|IncrementInt (Variables|Default|GetRuneNumber))
        (:%20%20
          _))))
  (Rendering|Components|TextRender|SetText (Variables|Default|GetImage) (Utilities|Text|ToText(Integer) _output_get))
  (return))

(fn OnRepCompleteCount)

(fn OnRepPuzzleCompleted)