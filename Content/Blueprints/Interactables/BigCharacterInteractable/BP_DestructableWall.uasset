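; Destructible wall interactable that only BP_BigCharacter can punch down.
; PunchingBox overlap registers the wall as that character's interact target and toggles custom depth on DoorInLowDM as a highlight.
; DoInteract, on authority only, calls ServerPunch to teleport the character to AnimationLocation and play the punch montage.
; After timed delays it plays a blast sound at world origin, enables physics on the mesh, then destroys the actor.
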(event OnComponentBeginOverlap(Box)
  (params (OverlappedComponent :type Primitive%20Component%20Object%20Reference) (OtherActor :type Actor%20Object%20Reference) (OtherComp :type Primitive%20Component%20Object%20Reference) (OtherBodyIndex :type Integer) (bFromSweep :type Boolean) (SweepResult :type Hit%20Result%20Structure%20%28by%20ref%29)))

(event OnComponentEndOverlap(Box)
  (params (OverlappedComponent :type Primitive%20Component%20Object%20Reference) (OtherActor :type Actor%20Object%20Reference) (OtherComp :type Primitive%20Component%20Object%20Reference) (OtherBodyIndex :type Integer)))

(event OnComponentBeginOverlap(PunchingBox)
  (params (OverlappedComponent :type Primitive%20Component%20Object%20Reference) (OtherActor :type Actor%20Object%20Reference) (OtherComp :type Primitive%20Component%20Object%20Reference) (OtherBodyIndex :type Integer) (bFromSweep :type Boolean) (SweepResult :type Hit%20Result%20Structure%20%28by%20ref%29))
  (bind _asbp_big_character (Utilities|Casting|CastToBP_BigCharacter OtherActor))
  (Default|UpdateInteract _asbp_big_character self true)
  (Variables|Default|SetBigCharacterRef _asbp_big_character)
  (Rendering|SetRenderCustomDepth (Variables|Default|GetDoorIn_Low_DM) true))

(event OnComponentEndOverlap(PunchingBox)
  (params (OverlappedComponent :type Primitive%20Component%20Object%20Reference) (OtherActor :type Actor%20Object%20Reference) (OtherComp :type Primitive%20Component%20Object%20Reference) (OtherBodyIndex :type Integer))
  (bind _asbp_big_character (Utilities|Casting|CastToBP_BigCharacter OtherActor))
  (Default|UpdateInteract _asbp_big_character 0 false)
  (Rendering|SetRenderCustomDepth (Variables|Default|GetDoorIn_Low_DM) false))

(event Custom|ServerPunch
  (bind _bigcharacterref (Variables|Default|GetBigCharacterRef))
  (Transformation|Teleport _bigcharacterref (Transformation|GetWorldLocation (Variables|Default|GetAnimationLocation)) "0,-90.000000, 0")
  (Animation|PlayAnimMontage _bigcharacterref "/Game/Animations/Big/Big_PunchAnim_Montage.Big_PunchAnim_Montage" 1.0 "None")
  (Utilities|FlowControl|Delay 1.4)
  (Audio|PlaySoundatLocation "/Game/Audio/Blast.Blast" "0, 0, 0" "0, 0, 0" 1.0 1.0 0.0 0 0 0)
  (Physics|SetSimulatePhysics (Variables|Default|GetDoorIn_Low_DM) true)
  (Utilities|FlowControl|Delay 1.4)
  (Actor|DestroyActor))

(event EventDoInteract
  (Networking|SwitchHasAuthority
    (:Authority
      (CallFunction|ServerPunch))))

(fn ConstructionScript)