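; Timed rune interactable for a two-character puzzle, usable by either the big or small character according to its BigCharacter flag.
; Box overlap registers it with that character and toggles outline and hover particles.
; Interacting snaps the character into an animation with effects, then activates linked vines if OtherRune is active, otherwise resets after a delay.
; Tick displays the activation state as text.
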(event OnComponentBeginOverlap(Box)
  (params (OverlappedComponent :type Primitive%20Component%20Object%20Reference) (OtherActor :type Actor%20Object%20Reference) (OtherComp :type Primitive%20Component%20Object%20Reference) (OtherBodyIndex :type Integer) (bFromSweep :type Boolean) (SweepResult :type Hit%20Result%20Structure%20%28by%20ref%29))
  (if (Variables|Default|GetBigCharacter?)
    (bind _asbp_big_character (Utilities|Casting|CastToBP_BigCharacter OtherActor))
    (Variables|/Game/Blueprints/Characters/BP_BigCharacter.BP_BigCharacter_C|SetbCanInteract _asbp_big_character true)
    (Default|UpdateInteract _asbp_big_character self true)
    (Variables|Default|SetBigCharRef _asbp_big_character)
    (Rendering|SetRenderCustomDepth (Variables|Default|GetStaticMesh) true)
    (Components|Activation|SetActive (Variables|Default|GetHoverParticleSystem) true false)
    (else
      (bind _asbp_small_character (Utilities|Casting|CastToBP_SmallCharacter OtherActor))
      (Variables|/Game/Blueprints/Characters/BP_SmallCharacter.BP_SmallCharacter_C|SetCanInteract _asbp_small_character true)
      (Default|UpdateInteract _asbp_small_character self true)
      (Variables|Default|SetSmallCharRef _asbp_small_character)
      (Rendering|SetRenderCustomDepth (Variables|Default|GetStaticMesh) true)
      (Components|Activation|SetActive (Variables|Default|GetHoverParticleSystem) true false))))

(event OnComponentEndOverlap(Box)
  (params (OverlappedComponent :type Primitive%20Component%20Object%20Reference) (OtherActor :type Actor%20Object%20Reference) (OtherComp :type Primitive%20Component%20Object%20Reference) (OtherBodyIndex :type Integer))
  (if (Variables|Default|GetBigCharacter?)
    (bind _asbp_big_character (Utilities|Casting|CastToBP_BigCharacter OtherActor))
    (Variables|/Game/Blueprints/Characters/BP_BigCharacter.BP_BigCharacter_C|SetbCanInteract _asbp_big_character false)
    (Default|UpdateInteract _asbp_big_character 0 false)
    (Rendering|SetRenderCustomDepth (Variables|Default|GetStaticMesh) false)
    (Components|Activation|Deactivate (Variables|Default|GetHoverParticleSystem))
    (else
      (bind _asbp_small_character (Utilities|Casting|CastToBP_SmallCharacter OtherActor))
      (Variables|/Game/Blueprints/Characters/BP_SmallCharacter.BP_SmallCharacter_C|SetCanInteract _asbp_small_character false)
      (Default|UpdateInteract _asbp_small_character self false)
      (Rendering|SetRenderCustomDepth (Variables|Default|GetStaticMesh) false)
      (Components|Activation|Deactivate (Variables|Default|GetHoverParticleSystem)))))

(event Custom|RunBigAnimation
  (Transformation|Teleport (Variables|Default|GetBigCharRef) (Transformation|GetWorldLocation (Variables|Default|GetAnimationLocation)) (Variables|Default|GetAnimationRotation))
  (Default|DoTouchAnimation (Variables|Default|GetBigCharRef))
  (Components|Activation|Activate (Variables|Default|GetParticleSystem) false)
  (Audio|PlaySound2D "/Game/Audio/220171__gameaudio__flourish-spacey-1.220171__gameaudio__flourish-spacey-1" 1.0 1.0 0.0 0 0))

(event Custom|RunSmallAnimation
  (bind _smallcharref (Variables|Default|GetSmallCharRef))
  (Animation|PlayAnimMontage _smallcharref "/Game/Animations/Little/Little_ButtonAnim_Montage.Little_ButtonAnim_Montage" 1.0 "None")
  (Transformation|Teleport _smallcharref (Transformation|GetWorldLocation (Variables|Default|GetAnimationLocation)) (Variables|Default|GetAnimationRotation))
  (Components|Activation|Activate (Variables|Default|GetParticleSystem) false)
  (Audio|PlaySound2D "/Game/Audio/220171__gameaudio__flourish-spacey-1.220171__gameaudio__flourish-spacey-1" 1.0 1.0 0.0 0 0))

(event EventTick
  (params (DeltaSeconds :type Float%20%28single-precision%29))
  (if (Variables|Default|GetHasBeenActivated)
    (bind _output_get (Variables|Default|SetActivatedStatus "TRUE"))
    (Rendering|Components|TextRender|SetText (Variables|Default|GetImage) _output_get)
    (else
      (bind _output_get_2 (Variables|Default|SetActivatedStatus "FALSE"))
      (Rendering|Components|TextRender|SetText (Variables|Default|GetImage) _output_get_2))))

(event EventBeginPlay)

(event EventDoInteract
  (if (Variables|Default|GetBigCharacter?)
    (CallFunction|RunBigAnimation)
    (Variables|Default|SetHasBeenActivated true)
    (if (Variables|BP_TimerRuneBig_C|GetHasBeenActivated (Variables|Default|GetOtherRune))
      (Development|PrintString "big character says yes")
      (Default|Activated (Variables|Default|GetVinesReference) false)
      (else
        (Utilities|FlowControl|Delay (Variables|Default|GetActivationLengthTimer))
        (Variables|Default|SetHasBeenActivated false)))
    (else
      (CallFunction|RunSmallAnimation)
      (Variables|Default|SetHasBeenActivated true)
      (if (Variables|BP_TimerRuneBig_C|GetHasBeenActivated (Variables|Default|GetOtherRune))
        (Development|PrintString "small character says yes")
        (Default|Activated (Variables|Default|GetVinesReference) false)
        (else
          (Utilities|FlowControl|Delay (Variables|Default|GetActivationLengthTimer))
          (Variables|Default|SetHasBeenActivated false))))))

(fn ConstructionScript)

(fn ConfigureMesh
  (switch int 0
    (:0
      (Components|StaticMesh|SetStaticMesh (Variables|Default|GetStaticMesh) "/Game/Assets/RunePillars/RunePillar2_Low.RunePillar2_Low"))
    (:1
      (Components|StaticMesh|SetStaticMesh (Variables|Default|GetStaticMesh) "/Game/Assets/RunePillars/RunePillarButton_Low.RunePillarButton_Low"))
    (:2
      (Components|StaticMesh|SetStaticMesh (Variables|Default|GetStaticMesh) "/Game/Assets/RunePillars/RunePillar3_Low.RunePillar3_Low"))
    (:3
      (Components|StaticMesh|SetStaticMesh (Variables|Default|GetStaticMesh) "/Game/Assets/RunePillars/RunePillar4_Low.RunePillar4_Low"))))