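; Pushable lily pad puzzle piece that the big character can move once through interaction.
; Overlapping CollisionBox registers it as that character's interact target and highlights Cube with custom depth, until overlap ends.
; DoInteract, gated by DoOnce, slides Cube over one second to BoxToMoveTo's world transform, passed as a relative target.
; It then sets BeenMoved, which blocks further prompts on overlap.
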(event OnComponentBeginOverlap(CollisionBox)
  (params (OverlappedComponent :type Primitive%20Component%20Object%20Reference) (OtherActor :type Actor%20Object%20Reference) (OtherComp :type Primitive%20Component%20Object%20Reference) (OtherBodyIndex :type Integer) (bFromSweep :type Boolean) (SweepResult :type Hit%20Result%20Structure%20%28by%20ref%29))
  (if (not (Variables|Default|GetBeenMoved))
    (bind _asbp_big_character (Utilities|Casting|CastToBP_BigCharacter OtherActor))
    (Variables|/Game/Blueprints/Characters/BP_BigCharacter.BP_BigCharacter_C|SetInteractActorReference _asbp_big_character self)
    (Variables|/Game/Blueprints/Characters/BP_BigCharacter.BP_BigCharacter_C|SetbCanInteract _asbp_big_character true)
    (Default|UpdateInteract _asbp_big_character self true)
    (Variables|Default|SetBigCharRef _asbp_big_character)
    (Rendering|SetRenderCustomDepth (Variables|Default|GetCube) true)))

(event OnComponentEndOverlap(CollisionBox)
  (params (OverlappedComponent :type Primitive%20Component%20Object%20Reference) (OtherActor :type Actor%20Object%20Reference) (OtherComp :type Primitive%20Component%20Object%20Reference) (OtherBodyIndex :type Integer))
  (bind _asbp_big_character (Utilities|Casting|CastToBP_BigCharacter OtherActor))
  (Variables|/Game/Blueprints/Characters/BP_BigCharacter.BP_BigCharacter_C|SetInteractActorReference _asbp_big_character 0)
  (Variables|/Game/Blueprints/Characters/BP_BigCharacter.BP_BigCharacter_C|SetbCanInteract _asbp_big_character false)
  (Default|UpdateInteract _asbp_big_character 0 false)
  (Rendering|SetRenderCustomDepth (Variables|Default|GetCube) false))

(event EventDoInteract
  (bind _boxtomoveto (Variables|Default|GetBoxToMoveTo))
  (Utilities|FlowControl|DoOnce false
    (:Completed
      (Components|MoveComponentTo (Variables|Default|GetCube) (Transformation|GetWorldLocation _boxtomoveto) (Transformation|GetWorldRotation _boxtomoveto) false false 1.0 false)
      (Variables|Default|SetBeenMoved true))))

(fn ConstructionScript)