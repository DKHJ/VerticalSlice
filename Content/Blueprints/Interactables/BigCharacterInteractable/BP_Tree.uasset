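; BP_Tree is an interactable tree that the big character can kick over.
; A box overlap with BP_BigCharacter registers or clears the tree as its interaction target, caches the character and toggles an activation flag.
; When active, DoInteract plays the character's kick montage and the tree's fall animation, then rotates the whole actor to face the character's mesh so the fall is oriented relative to the kicker.
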(event OnComponentBeginOverlap(Box)
  (params (OverlappedComponent :type Primitive%20Component%20Object%20Reference) (OtherActor :type Actor%20Object%20Reference) (OtherComp :type Primitive%20Component%20Object%20Reference) (OtherBodyIndex :type Integer) (bFromSweep :type Boolean) (SweepResult :type Hit%20Result%20Structure%20%28by%20ref%29))
  (bind _asbp_big_character (Utilities|Casting|CastToBP_BigCharacter OtherActor))
  (Default|UpdateInteract _asbp_big_character self true)
  (Variables|Default|SetBigCharRef _asbp_big_character)
  (Variables|Default|SetIsActivated? true))

(event OnComponentEndOverlap(Box)
  (params (OverlappedComponent :type Primitive%20Component%20Object%20Reference) (OtherActor :type Actor%20Object%20Reference) (OtherComp :type Primitive%20Component%20Object%20Reference) (OtherBodyIndex :type Integer))
  (bind _asbp_big_character (Utilities|Casting|CastToBP_BigCharacter OtherActor))
  (Default|UpdateInteract _asbp_big_character self false)
  (Variables|Default|SetIsActivated? false))

(event EventDoInteract
  (bind _self self)
  (if (Variables|Default|GetIsActivated?)
    (Animation|PlayAnimMontage (Variables|Default|GetBigCharRef) "/Game/Animations/Big/Big_KickAnim_Montage.Big_KickAnim_Montage" 1.0 "None")
    (Components|Animation|PlayAnimation (Variables|Default|GetSkeletalMesh) "/Game/Animations/TreeFallAnim_Anim.TreeFallAnim_Anim" false)
    (Transformation|SetActorRotation _self (Math|Rotator|FindLookatRotation (Transformation|GetWorldLocation (Variables|Default|GetSkeletalMesh _self)) (Transformation|GetWorldLocation (Variables|/Script/Engine.Character|GetMesh (Variables|Default|GetBigCharRef)))))))

(fn ConstructionScript)