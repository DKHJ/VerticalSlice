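; An interactable puzzle rune that shows a number and counts as activated when that number matches its goal.
; A box overlap registers it with BP_BigCharacter, and each interaction cycles the number, wrapping back to zero.
; On a match, it loops over all runes gathered at BeginPlay, counting active ones and resetting on an inactive one.
; When the count hits four, every rune's text turns green.
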(event OnComponentBeginOverlap(Box)
  (params (OverlappedComponent :type Primitive%20Component%20Object%20Reference) (OtherActor :type Actor%20Object%20Reference) (OtherComp :type Primitive%20Component%20Object%20Reference) (OtherBodyIndex :type Integer) (bFromSweep :type Boolean) (SweepResult :type Hit%20Result%20Structure%20%28by%20ref%29))
  (bind _asbp_big_character (Utilities|Casting|CastToBP_BigCharacter OtherActor))
  (Variables|/Game/Blueprints/Characters/BP_BigCharacter.BP_BigCharacter_C|SetCanInteract _asbp_big_character true)
  (Default|UpdateInteract _asbp_big_character self true))

(event OnComponentEndOverlap(Box)
  (params (OverlappedComponent :type Primitive%20Component%20Object%20Reference) (OtherActor :type Actor%20Object%20Reference) (OtherComp :type Primitive%20Component%20Object%20Reference) (OtherBodyIndex :type Integer))
  (bind _asbp_big_character (Utilities|Casting|CastToBP_BigCharacter OtherActor))
  (Variables|/Game/Blueprints/Characters/BP_BigCharacter.BP_BigCharacter_C|SetCanInteract _asbp_big_character false)
  (Default|UpdateInteract _asbp_big_character 0 false))

(event Custom|CheckRunes
  (for _array_element (Variables|Default|GetAllRunes)
    (if (Variables|BP_ImagePuzzleRune_C|GetRuneActivated _array_element)
      (bind _result (Math|Integer|IncrementInt (Variables|Default|GetCompleteCount))
        (:%20%20
          (Development|PrintString (Utilities|String|ToString(Integer) _result))
          (if (== _result 4)
            (Development|PrintString "Puzzle Completed")
            (for _array_element_2 (Variables|Default|GetAllRunes)
              (Rendering|Components|TextRender|SetTextRenderColor (Variables|BP_ImagePuzzleRune_C|GetImage _array_element_2) (Variables|Default|GetColorGreen))))))
      (else
        (Development|PrintString "puzzle incomplete")
        (Variables|Default|SetCompleteCount 0)))))

(event EventBeginPlay
  (Rendering|Components|TextRender|SetText (Variables|Default|GetImage) (Utilities|Text|ToText(Integer) (Variables|Default|GetRuneNumber)))
  (bind _outactors (Actor|GetAllActorsOfClass "BP_ImagePuzzleRune_C"))
  (Variables|Default|SetAllRunes _outactors))

(event EventDoInteract
  (if (>= (Variables|Default|GetRuneNumber) 4)
    (bind _output_get (Variables|Default|SetRuneNumber 0))
    (else
      (bind _result (Math|Integer|IncrementInt (Variables|Default|GetRuneNumber))
        (:%20%20
          _))))
  (Rendering|Components|TextRender|SetText (Variables|Default|GetImage) (Utilities|Text|ToText(Integer) _output_get))
  (if (== (Variables|Default|GetRuneNumber) (Variables|Default|GetGoalNumber))
    (Variables|Default|SetRuneActivated true)
    (Development|PrintString "rune activated")
    (CallFunction|CheckRunes)
    (else
      (Variables|Default|SetRuneActivated false))))

(fn ConstructionScript)