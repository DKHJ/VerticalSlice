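; BP_WinterPuzzle1Rune is a winter puzzle rune that the big character touches to toggle its linked magic platform.
; Box overlap registers it as the character's interact target and enables custom-depth rendering on the mesh.
; DoInteract blends the camera, locks input, teleports the character into place, plays a touch montage and activates particles.
; Runes cached on BeginPlay are mutually exclusive: toggling one deactivates any other active rune and re-triggers its platform.
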(event OnComponentBeginOverlap(Box)
  (params (OverlappedComponent :type Primitive%20Component%20Object%20Reference) (OtherActor :type Actor%20Object%20Reference) (OtherComp :type Primitive%20Component%20Object%20Reference) (OtherBodyIndex :type Integer) (bFromSweep :type Boolean) (SweepResult :type Hit%20Result%20Structure%20%28by%20ref%29))
  (bind _asbp_big_character (Utilities|Casting|CastToBP_BigCharacter OtherActor))
  (Variables|/Game/Blueprints/Characters/BP_BigCharacter.BP_BigCharacter_C|SetInteractActorReference _asbp_big_character self)
  (Variables|/Game/Blueprints/Characters/BP_BigCharacter.BP_BigCharacter_C|SetCanInteract _asbp_big_character true)
  (Variables|Default|SetBigCharRef _asbp_big_character)
  (Rendering|SetRenderCustomDepth (Variables|Default|GetStaticMesh) true))

(event OnComponentEndOverlap(Box)
  (params (OverlappedComponent :type Primitive%20Component%20Object%20Reference) (OtherActor :type Actor%20Object%20Reference) (OtherComp :type Primitive%20Component%20Object%20Reference) (OtherBodyIndex :type Integer))
  (bind _asbp_big_character (Utilities|Casting|CastToBP_BigCharacter OtherActor))
  (Variables|/Game/Blueprints/Characters/BP_BigCharacter.BP_BigCharacter_C|SetInteractActorReference _asbp_big_character 0)
  (Variables|/Game/Blueprints/Characters/BP_BigCharacter.BP_BigCharacter_C|SetCanInteract _asbp_big_character false)
  (Rendering|SetRenderCustomDepth (Variables|Default|GetStaticMesh) false))

(event EventBeginPlay
  (bind _outactors (Actor|GetAllActorsOfClass "BP_WinterPuzzle1Rune_C"))
  (Variables|Default|SetAllRuneActors _outactors))

(event EventDoInteract
  (bind _bigcharref (Variables|Default|GetBigCharRef))
  (bind _bigcharref_2 (Variables|Default|GetBigCharRef))
  (Default|ChangeCameraActor (Variables|Default|GetBigCharRef) self 0.5)
  (Utilities|FlowControl|Delay 0.5)
  (Default|DisablePlayerInput _bigcharref_2)
  (Transformation|Teleport _bigcharref_2 (Transformation|GetWorldLocation (Variables|Default|GetAnimationLocation)) "0, 0, 0")
  (if (Variables|Default|GetActivated)
    (Variables|Default|SetActivated false)
    (else
      (Variables|Default|SetActivated true)))
  (Default|DoInteract (Variables|Default|GetMagicPlatformReference))
  (CallFunction|ResetAllOtherRunes self)
  (Animation|PlayAnimMontage (Variables|Default|GetBigCharRef) "/Game/Animations/Big/Big_TouchAnim_Montage.Big_TouchAnim_Montage" 1.0 "None")
  (Utilities|FlowControl|Delay 0.5)
  (Components|Activation|Activate (Variables|Default|GetTouchParticle_PAR) false)
  (Default|EnablePlayerInput (Variables|Default|GetBigCharRef))
  (Utilities|FlowControl|Delay 0.5)
  (Default|ChangeCameraActor _bigcharref _bigcharref 0.5))

(fn ConstructionScript)

(fn ResetAllOtherRunes
  (params (CurrentRune :type BP%20Winter%20Puzzle%201%20Rune%20Object%20Reference))
  (for _array_element (Variables|Default|GetAllRuneActors)
    (if (not (== _array_element CurrentRune))
      (if (Variables|BP_WinterPuzzle1Rune_C|GetActivated _array_element)
        (Variables|BP_WinterPuzzle1Rune_C|SetActivated _array_element false)
        (Default|DoInteract (Variables|BP_WinterPuzzle1Rune_C|GetMagicPlatformReference _array_element))))))