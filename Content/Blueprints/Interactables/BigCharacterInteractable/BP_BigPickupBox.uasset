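; BP_BigPickupBox is an interactable box that BP_BigCharacter can pick up, carry at reduced walk speed and put down.
; Its collision box registers or clears interaction on the character, and DoInteract passes the PickedUp state to SERVERInteract to toggle carrying.
; Pickup locks input and uses timed delays around snapping to the ApeBoxSocket, suspending collision and disabling physics.
; Putdown detaches the mesh, re-enables physics and restores normal speed.
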(event OnComponentBeginOverlap(CollisionBox)
  (params (OverlappedComponent :type Primitive%20Component%20Object%20Reference) (OtherActor :type Actor%20Object%20Reference) (OtherComp :type Primitive%20Component%20Object%20Reference) (OtherBodyIndex :type Integer) (bFromSweep :type Boolean) (SweepResult :type Hit%20Result%20Structure%20%28by%20ref%29))
  (bind _asbp_big_character (Utilities|Casting|CastToBP_BigCharacter OtherActor))
  (Default|UpdateInteract _asbp_big_character self true)
  (Variables|Default|SetBigCharRef _asbp_big_character))

(event OnComponentEndOverlap(CollisionBox)
  (params (OverlappedComponent :type Primitive%20Component%20Object%20Reference) (OtherActor :type Actor%20Object%20Reference) (OtherComp :type Primitive%20Component%20Object%20Reference) (OtherBodyIndex :type Integer))
  (bind _asbp_big_character (Utilities|Casting|CastToBP_BigCharacter OtherActor))
  (Default|UpdateInteract _asbp_big_character 0 false))

(event Custom|SERVER%20Interact
  (params (IsPickedUP :type Boolean))
  (bind _bigcharref (Variables|Default|GetBigCharRef))
  (bind _bigcharref_2 (Variables|Default|GetBigCharRef))
  (bind _bigcharref_3 (Variables|Default|GetBigCharRef))
  (bind _bigcharref_4 (Variables|Default|GetBigCharRef))
  (if IsPickedUP
    (Default|PutdownBigBox (Variables|Default|GetBigCharRef))
    (Physics|SetSimulatePhysics (Variables|Default|GetStaticMesh) true)
    (Transformation|DetachFromComponent (Variables|Default|GetStaticMesh) "KeepRelative" "KeepRelative" "KeepRelative" true)
    (Variables|Default|SetbPickedUp? false)
    (Default|EnablePlayerInput _bigcharref_3)
    (Variables|/Game/Blueprints/Characters/BP_BigCharacter.BP_BigCharacter_C|SetBigPickup _bigcharref_3 0)
    (Variables|/Game/Blueprints/Characters/BP_BigCharacter.BP_BigCharacter_C|SetbBigBoxPickedUp _bigcharref_3 false)
    (Variables|/Script/Engine.CharacterMovementComponent|SetMaxWalkSpeed (Variables|/Script/Engine.Character|GetCharacterMovement _bigcharref_3) 6e+02)
    (else
      (Default|DisablePlayerInput _bigcharref_2)
      (Default|PickupBigBox _bigcharref_2 (Transformation|GetActorLocation))
      (Collision|SetActorEnableCollision false)
      (Physics|SetSimulatePhysics (Variables|Default|GetStaticMesh) false)
      (Utilities|FlowControl|Delay 1.2)
      (Transformation|AttachComponentToComponent (Variables|/Script/Engine.Character|GetMesh _bigcharref) "ApeBoxSocket" "SnapToTarget" "SnapToTarget" "KeepWorld" true)
      (Variables|Default|SetbPickedUp? true)
      (Utilities|FlowControl|Delay 1.0)
      (Collision|SetActorEnableCollision true)
      (Default|EnablePlayerInput _bigcharref_4)
      (Variables|/Game/Blueprints/Characters/BP_BigCharacter.BP_BigCharacter_C|SetBigPickup _bigcharref_4 self)
      (Variables|/Game/Blueprints/Characters/BP_BigCharacter.BP_BigCharacter_C|SetbBigBoxPickedUp _bigcharref_4 true)
      (Variables|/Script/Engine.CharacterMovementComponent|SetMaxWalkSpeed (Variables|/Script/Engine.Character|GetCharacterMovement _bigcharref) 2e+02))))

(event EventDoInteract
  (CallFunction|SERVERInteract (Variables|Default|GetbPickedUp?)))

(fn ConstructionScript)