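; BP_WinterMechanism is a one-shot interactable that lets the small character activate vines on a referenced bridge.
; Its collision overlap toggles a custom-depth highlight on the mesh and registers or disables itself as that character's interact target.
; DoInteract calls SERVERActivate, which snaps the character to an animation point with a button montage.
; After a short delay it fires particles, the bridge vines and a 2D sound.
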(event OnComponentBeginOverlap(Collision)
  (params (OverlappedComponent :type Primitive%20Component%20Object%20Reference) (OtherActor :type Actor%20Object%20Reference) (OtherComp :type Primitive%20Component%20Object%20Reference) (OtherBodyIndex :type Integer) (bFromSweep :type Boolean) (SweepResult :type Hit%20Result%20Structure%20%28by%20ref%29))
  (bind _asbp_small_character (Utilities|Casting|CastToBP_SmallCharacter OtherActor))
  (Rendering|SetRenderCustomDepth (Variables|Character|GetMesh) true)
  (Variables|Default|SetSmallCharacterReference _asbp_small_character)
  (Default|UpdateInteract _asbp_small_character self true))

(event OnComponentEndOverlap(Collision)
  (params (OverlappedComponent :type Primitive%20Component%20Object%20Reference) (OtherActor :type Actor%20Object%20Reference) (OtherComp :type Primitive%20Component%20Object%20Reference) (OtherBodyIndex :type Integer))
  (bind _asbp_small_character (Utilities|Casting|CastToBP_SmallCharacter OtherActor))
  (Rendering|SetRenderCustomDepth (Variables|Character|GetMesh) false)
  (Default|UpdateInteract _asbp_small_character 0 false))

(event Custom|SERVER%20Activate
  (bind _smallcharacterreference (Variables|Default|GetSmallCharacterReference))
  (Utilities|FlowControl|DoOnce false
    (:Completed
      (Animation|PlayAnimMontage _smallcharacterreference "/Game/Animations/Little/Little_ButtonAnim_Montage.Little_ButtonAnim_Montage" 1.0 "None")
      (Transformation|Teleport _smallcharacterreference (Transformation|GetWorldLocation (Variables|Default|GetAnimationLocation)) "0,90.000000, 0")
      (Utilities|FlowControl|Delay 0.6)
      (Components|Activation|Activate (Variables|Default|GetParticleSystem) false)
      (Default|ActivateVines (Variables|Default|GetBridgeRef) true)
      (Audio|PlaySound2D "/Game/Audio/RuneInteractSound.RuneInteractSound" 1.0 1.0 0.0 0 0))))

(event EventDoInteract
  (Networking|SwitchHasAuthority
    (:Authority
      _)
    (:Remote
      _))
  (CallFunction|SERVERActivate))

(fn ConstructionScript)

(fn DoInteraction
  (return false))