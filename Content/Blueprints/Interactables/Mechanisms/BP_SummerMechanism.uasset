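; Interactable "summer" mechanism that switches a BP_SmallCharacter between its normal view and a fixed-in-place EagleCamera view.
; Collision overlap caches the character and registers or clears this actor as its interact target.
; DoInteract forwards to ServerDoInteract, which plays a sound and toggles Activated, changing camera and disabling or restoring walking movement on the cached character.
; The DoInteraction function is a stub returning false.
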(event OnComponentBeginOverlap(Collision)
  (params (OverlappedComponent :type Primitive%20Component%20Object%20Reference) (OtherActor :type Actor%20Object%20Reference) (OtherComp :type Primitive%20Component%20Object%20Reference) (OtherBodyIndex :type Integer) (bFromSweep :type Boolean) (SweepResult :type Hit%20Result%20Structure%20%28by%20ref%29))
  (bind _asbp_small_character (Utilities|Casting|CastToBP_SmallCharacter OtherActor))
  (bind _output_get (Variables|Default|SetSmallCharRef _asbp_small_character))
  (Default|UpdateInteract _output_get self true))

(event OnComponentEndOverlap(Collision)
  (params (OverlappedComponent :type Primitive%20Component%20Object%20Reference) (OtherActor :type Actor%20Object%20Reference) (OtherComp :type Primitive%20Component%20Object%20Reference) (OtherBodyIndex :type Integer))
  (bind _asbp_small_character (Utilities|Casting|CastToBP_SmallCharacter OtherActor))
  (Default|UpdateInteract _asbp_small_character 0 false))

(event Custom|Server%20Do%20Interact
  (bind _smallcharref (Variables|Default|GetSmallCharRef))
  (bind _smallcharref_2 (Variables|Default|GetSmallCharRef))
  (Audio|PlaySound2D "/Game/Audio/220171__gameaudio__flourish-spacey-1.220171__gameaudio__flourish-spacey-1" 1.0 1.0 0.0 0 0)
  (if (Variables|Default|GetActivated?)
    (Variables|Default|SetActivated? false)
    (Default|ChangeCamera _smallcharref_2)
    (Pawn|Components|CharacterMovement|SetMovementMode (Variables|/Script/Engine.Character|GetCharacterMovement _smallcharref_2) "MOVE_Walking" 0)
    (else
      (Variables|Default|SetActivated? true)
      (Default|ChangeCamera _smallcharref 3 (Variables|Default|GetEagleCamera))
      (Pawn|Components|CharacterMovement|DisableMovement (Variables|/Script/Engine.Character|GetCharacterMovement _smallcharref)))))

(event EventDoInteract
  (CallFunction|ServerDoInteract))

(fn ConstructionScript
  (|CallParentFunction))

(fn DoInteraction
  (return false))