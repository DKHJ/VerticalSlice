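; A magic jumping platform that fades in or out and reveals the next platform in a chain when a BP_SmallCharacter enters its box.
; The overlap clears the next platform's Activated flag, then calls its toggle, so that platform always turns on.
; Timelines drive opacity on a dynamic material, then set collision to match the flag when finished.
; BeginPlay runs the same toggle through DoInteract to set the starting state.
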(event OnComponentBeginOverlap(Box)
  (params (OverlappedComponent :type Primitive%20Component%20Object%20Reference) (OtherActor :type Actor%20Object%20Reference) (OtherComp :type Primitive%20Component%20Object%20Reference) (OtherBodyIndex :type Integer) (bFromSweep :type Boolean) (SweepResult :type Hit%20Result%20Structure%20%28by%20ref%29))
  (bind _nextjumpingplatformref (Variables|Default|GetNextJumpingPlatformRef))
  (Utilities|Casting|CastToBP_SmallCharacter OtherActor)
  (Variables|BP_JumpingMagicPlatform_C|SetActivated _nextjumpingplatformref false)
  (CallFunction|ActivateNextPlatform _nextjumpingplatformref))

(event Custom|ActivateNextPlatform
  (if (Variables|Default|GetActivated)
    (Variables|Default|SetActivated false)
    (bind _time (Timeline|Timeline_1 PlayFromStart)
      (:Update
        (Rendering|Material|SetScalarParameterValue (Variables|Default|GetLines) "Opacity_Control" _time :!class /Script/Engine.MaterialInstanceDynamic))
      (:Finished
        (if (Variables|Default|GetActivated)
          (Collision|SetCollisionEnabled (Variables|Default|GetStaticMesh) "QueryAndPhysics")
          (else
            (Collision|SetCollisionEnabled (Variables|Default|GetStaticMesh) "NoCollision")))))
    (else
      (Variables|Default|SetActivated true)
      (Timeline|Timeline_1 ReverseFromEnd))))

(event EventBeginPlay
  (CallFunction|DoInteract))

(event EventDoInteract
  (if (Variables|Default|GetActivated)
    (Variables|Default|SetActivated false)
    (bind _time (Timeline|Timeline_0 PlayFromStart)
      (:Update
        (Rendering|Material|SetScalarParameterValue (Variables|Default|GetLines) "Opacity_Control" _time :!class /Script/Engine.MaterialInstanceDynamic))
      (:Finished
        (if (Variables|Default|GetActivated)
          (Collision|SetCollisionEnabled (Variables|Default|GetStaticMesh) "QueryAndPhysics")
          (else
            (Collision|SetCollisionEnabled (Variables|Default|GetStaticMesh) "NoCollision")))))
    (else
      (Variables|Default|SetActivated true)
      (Timeline|Timeline_0 ReverseFromEnd))))

(fn ConstructionScript
  (bind _returnvalue (Rendering|Material|CreateDynamicMaterialInstance (Variables|Default|GetStaticMesh) 0 "/Game/Assets/DissolveMaterial/MagicPlatform_INS.MagicPlatform_INS" "None" :!class /Script/Engine.PrimitiveComponent))
  (Variables|Default|SetLines _returnvalue))

(fn OnRepActivated)