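; BP_HubWorldMovingPlatform is a moving platform that, once activated through DoInteract, shuttles back and forth along a spline.
; The Movement timeline drives the static mesh's world location by scaling spline length by an alpha value.
; Each time the timeline finishes, it flips IsCompleted and calls Activated again, alternating Play and Reverse in an endless ping-pong.
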(event Custom|Activated
  (if (Variables|Default|GetIsActivated?)
    (if (Variables|Default|GetIsCompleted?)
      (bind _time (Timeline|Movement Reverse)
        (:Update
          (Transformation|SetWorldLocation (Variables|Default|GetStaticMesh) (Spline|GetLocationatDistanceAlongSpline (Variables|Default|GetSpline) (* _time (Spline|GetSplineLength (Variables|Default|GetSpline))) "World") false false))
        (:Finished
          (if (Variables|Default|GetIsCompleted?)
            (Variables|Default|SetIsCompleted? false)
            (else
              (Variables|Default|SetIsCompleted? true)))
          (CallFunction|Activated)))
      (else
        (Timeline|Movement Play)))))

(event EventDoInteract
  (Variables|Default|SetIsActivated? true)
  (CallFunction|Activated))

(fn ConstructionScript)