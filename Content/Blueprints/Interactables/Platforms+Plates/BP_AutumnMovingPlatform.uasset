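; BP_AutumnMovingPlatform is a platform that shuttles back and forth along a spline while a BP_SmallCharacter occupies its trigger box.
; The Movement timeline drives the mesh's world location by scaling its output to a distance along the spline.
; Each finished run flips IsCompleted and re-triggers Activated, alternating Play and Reverse.
; Leaving the box only clears IsActivated, so the current run finishes before the platform stops.
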(event OnComponentBeginOverlap(Box)
  (params (OverlappedComponent :type Primitive%20Component%20Object%20Reference) (OtherActor :type Actor%20Object%20Reference) (OtherComp :type Primitive%20Component%20Object%20Reference) (OtherBodyIndex :type Integer) (bFromSweep :type Boolean) (SweepResult :type Hit%20Result%20Structure%20%28by%20ref%29))
  (Utilities|Casting|CastToBP_SmallCharacter OtherActor)
  (Variables|Default|SetIsActivated? true)
  (CallFunction|Activated))

(event OnComponentEndOverlap(Box)
  (params (OverlappedComponent :type Primitive%20Component%20Object%20Reference) (OtherActor :type Actor%20Object%20Reference) (OtherComp :type Primitive%20Component%20Object%20Reference) (OtherBodyIndex :type Integer))
  (Utilities|Casting|CastToBP_SmallCharacter OtherActor)
  (Variables|Default|SetIsActivated? false))

(event Custom|Activated
  (if (Variables|Default|GetIsActivated?)
    (if (Variables|Default|GetIsCompleted?)
      (bind _time (Timeline|Movement Reverse)
        (:Update
          (Transformation|SetWorldLocation (Variables|Default|GetStaticMesh) (Spline|GetLocationatDistanceAlongSpline (Variables|Default|GetSpline) (* _time (Spline|GetSplineLength (Variables|Default|GetSpline))) "World") false false))
        (:Finished
          (if (Variables|Default|GetIsCompleted?)
            (Variables|Default|SetIsCompleted? false)
            (else
              (Variables|Default|SetIsCompleted? true)))
          (CallFunction|Activated)))
      (else
        (Timeline|Movement Play)))))

(fn ConstructionScript)