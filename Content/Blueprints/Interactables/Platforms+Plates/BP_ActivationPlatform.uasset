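; Pressure platform that clears a linked vine when a BP_BigPickupBox rests on it without being held.
; On authority, overlap plays a sound, then once sets Activated and switches both characters' cameras to a configured view.
; After a delay, a timeline drives the vine's opacity parameter, then restores the cameras and disables its mesh collision.
; End overlap clears Activated only for BP_PushableBox, a different class from the trigger.
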(event OnComponentBeginOverlap(Box)
  (params (OverlappedComponent :type Primitive%20Component%20Object%20Reference) (OtherActor :type Actor%20Object%20Reference) (OtherComp :type Primitive%20Component%20Object%20Reference) (OtherBodyIndex :type Integer) (bFromSweep :type Boolean) (SweepResult :type Hit%20Result%20Structure%20%28by%20ref%29))
  (bind _asbp_big_pickup_box (Utilities|Casting|CastToBP_BigPickupBox OtherActor))
  (Networking|SwitchHasAuthority
    (:Authority
      (CallFunction|ServerCollision))))

(event OnComponentEndOverlap(Box)
  (params (OverlappedComponent :type Primitive%20Component%20Object%20Reference) (OtherActor :type Actor%20Object%20Reference) (OtherComp :type Primitive%20Component%20Object%20Reference) (OtherBodyIndex :type Integer))
  (Utilities|Casting|CastToBP_PushableBox OtherActor)
  (Variables|Default|SetActivated? false))

(event Custom|ActivatedEvent
  (bind _smallcharacterreference (Variables|Default|GetSmallCharacterReference))
  (bind _time (Timeline|Timeline_1 Play)
    (:Update
      (Rendering|Material|SetScalarParameterValue (Variables|/Game/Blueprints/Interactables/Vines/BP_Vines.BP_Vines_C|GetLines (Variables|Default|GetVineReference)) "Opacity_Control" _time :!class /Script/Engine.MaterialInstanceDynamic)
      (Utilities|FlowControl|DoOnce false
        (:Completed
          (Audio|PlaySound2D "/Game/Assets/Sounds/SFX/NormalVineActivateSound.NormalVineActivateSound" 1.0 1.0 0.0 0 0))))
    (:Finished
      (Default|ChangeCameraView (Variables|Default|GetBigCharacterReference))
      (Default|ChangeCamera _smallcharacterreference 0 _smallcharacterreference)
      (Collision|SetCollisionEnabled (Variables|/Game/Blueprints/Interactables/Vines/BP_Vines.BP_Vines_C|GetStaticMesh (Variables|Default|GetVineReference)) "NoCollision")
      (Development|PrintString (Utilities|String|ToString(Boolean) (Utilities|IsValid _smallcharacterreference)) true true "(R=0.000000,G=0.660000,B=1.000000,A=1.000000)" 5.0))))

(event Custom|Server%20Collision
  (if (not (Variables|/Game/Blueprints/Interactables/BigCharacterInteractable/BP_BigPickupBox.BP_BigPickupBox_C|GetbPickedUp? (stale OnComponentBeginOverlap(Box) _asbp_big_pickup_box)))
    (Audio|PlaySound2D "/Game/Audio/Props/Cave_Finish_Open.Cave_Finish_Open" 1.0 1.0 0.0 0 0)
    (Utilities|FlowControl|DoOnce false
      (:Completed
        (Variables|Default|SetActivated? true)
        (Variables|Default|SetStartLocation (Transformation|GetActorLocation (Variables|Default|GetVineReference)))
        (CallFunction|GetSmallCharacterReference)
        (Default|ChangeCamera (Variables|Default|GetSmallCharacterReference) (Variables|Default|GetCameraNumber))
        (Default|ChangeCameraView (Variables|Default|GetBigCharacterReference) (Variables|Default|GetCameraNumber))
        (Utilities|FlowControl|Delay 2.0)
        (CallFunction|ActivatedEvent)))))

(event EventBeginPlay
  (Utilities|FlowControl|Delay 0.3)
  (bind _outactors (Actor|GetAllActorsOfClass "/Game/Blueprints/Characters/BP_BigCharacter.BP_BigCharacter_C"))
  (Variables|Default|SetBigCharacterReference (Utilities|Array|Get(acopy) _outactors)))

(event EventGetSmallCharacterReference
  ;[1 0 0.1577] Get a reference to the small character
  (bind _outactors (Actor|GetAllActorsOfClass "/Game/Blueprints/Characters/BP_SmallCharacter.BP_SmallCharacter_C"))
  (Variables|Default|SetSmallCharacterReference (Utilities|Array|Get(acopy) _outactors)))

(fn ConstructionScript)