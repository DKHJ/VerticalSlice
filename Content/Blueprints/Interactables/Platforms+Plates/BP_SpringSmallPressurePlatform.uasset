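; Pressure plate that sinks when a throwable box lands on it and activates a linked vine bridge.
; On the server, box overlap stores the box, plays a 2D sound and runs a timeline lerping the actor down by a sink distance.
; When the timeline finishes, it activates the bridge vines and passes false to a second vine reference.
; End overlap is unwired, so the plate never releases on exit.
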(event OnComponentBeginOverlap(Box)
  (params (OverlappedComponent :type Primitive%20Component%20Object%20Reference) (OtherActor :type Actor%20Object%20Reference) (OtherComp :type Primitive%20Component%20Object%20Reference) (OtherBodyIndex :type Integer) (bFromSweep :type Boolean) (SweepResult :type Hit%20Result%20Structure%20%28by%20ref%29))
  ;[0.5748 1 0.5817] BEGIN overlap
  (Networking|SwitchHasAuthority
    (:Authority
      (bind _asbp_throwable_box (Utilities|Casting|CastToBP_ThrowableBox OtherActor))
      (Variables|Default|SetThrowBoxRef _asbp_throwable_box)
      (Variables|Default|SetIsActivated? true)
      (CallFunction|PlateMovement))))

(event OnComponentEndOverlap(Box)
  (params (OverlappedComponent :type Primitive%20Component%20Object%20Reference) (OtherActor :type Actor%20Object%20Reference) (OtherComp :type Primitive%20Component%20Object%20Reference) (OtherBodyIndex :type Integer))
  ;[1 0.5208 0.5208] END overlap
)

(event Custom|Activated
  (CallFunction|DoInteract))

(event Custom|PlateMovement
  (CallFunction|PlaySound)
  ;[1 1 1] Here we just need to check if we're going down or up
  (if (Variables|Default|GetIsActivated?)
    (bind _time (Timeline|Timeline_0 Play)
      (:Update
        (Transformation|SetActorLocation (Math|Vector|Lerp(Vector) (Variables|Default|GetStartLocation) (- (Variables|Default|GetStartLocation) (Math|Vector|MakeVector 0.0 0.0 (Variables|Default|GetPressurePlateSinkDistance))) _time) false false))
      (:Finished
        (if (Variables|Default|GetIsActivated?)
          (Default|ActivateVines (Variables|Default|GetVineBridgeRef) true)
          (Default|Activated (Variables|Default|GetVineRef) false)
          (else
            (Default|ActivateVines (Variables|Default|GetVineBridgeRef) false)))))
    (else
      (Timeline|Timeline_0 Reverse))))

(event Custom|PlaySound
  (Audio|PlaySound2D "/Game/Audio/Props/Cave_Finish_Open.Cave_Finish_Open" 1.0 1.0 0.0 0 0))

(event EventBeginPlay
  (Variables|Default|SetStartLocation (Transformation|GetWorldLocation (Variables|Default|GetStaticMesh))))

(fn ConstructionScript)