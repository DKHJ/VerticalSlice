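; BP_PressurePlatform is a pressure plate that drives a linked moving platform when a throwable box or the small character overlaps its box trigger.
; On overlap it sets its own and the platform's IsActivated flag, then fires Activated, which calls DoInteract on the platform.
; Only the small character leaving clears the flags and calls DoInteract again; a box leaving does not release the plate.
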(event OnComponentBeginOverlap(Box)
  (params (OverlappedComponent :type Primitive%20Component%20Object%20Reference) (OtherActor :type Actor%20Object%20Reference) (OtherComp :type Primitive%20Component%20Object%20Reference) (OtherBodyIndex :type Integer) (bFromSweep :type Boolean) (SweepResult :type Hit%20Result%20Structure%20%28by%20ref%29))
  (Utilities|FlowControl|Sequence
    (:then_0
      (bind _asbp_throwable_box (Utilities|Casting|CastToBP_ThrowableBox OtherActor))
      (Variables|Default|SetThrowBoxRef _asbp_throwable_box)
      (Variables|Default|SetIsActivated? true)
      (Variables|/Game/Blueprints/Interactables/Platforms+Plates/BP_MovingPlatform.BP_MovingPlatform_C|SetIsActivated? (Variables|Default|GetMovingPlatRef) true)
      (CallFunction|Activated))
    (:then_1
      (bind _asbp_small_character (Utilities|Casting|CastToBP_SmallCharacter OtherActor))
      (Variables|Default|SetSmallCharRef _asbp_small_character)
      (Variables|Default|SetIsActivated? true)
      (Variables|/Game/Blueprints/Interactables/Platforms+Plates/BP_MovingPlatform.BP_MovingPlatform_C|SetIsActivated? (Variables|Default|GetMovingPlatRef) true)
      (CallFunction|Activated))))

(event OnComponentEndOverlap(Box)
  (params (OverlappedComponent :type Primitive%20Component%20Object%20Reference) (OtherActor :type Actor%20Object%20Reference) (OtherComp :type Primitive%20Component%20Object%20Reference) (OtherBodyIndex :type Integer))
  (Utilities|Casting|CastToBP_SmallCharacter OtherActor)
  (Variables|Default|SetIsActivated? false)
  (CallFunction|Activated)
  (Variables|/Game/Blueprints/Interactables/Platforms+Plates/BP_MovingPlatform.BP_MovingPlatform_C|SetIsActivated? (Variables|Default|GetMovingPlatRef) false))

(event Custom|Activated
  (Default|DoInteract (Variables|Default|GetMovingPlatRef)))

(fn ConstructionScript)