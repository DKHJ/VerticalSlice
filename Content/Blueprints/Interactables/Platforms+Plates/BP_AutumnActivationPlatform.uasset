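; Autumn activation plate that clears a vine barrier when a BP_PushableBox is pushed onto it.
; The first overlap switches both the big and small characters to a configured camera, then fires the activation event after a short delay.
; On authority only, a timeline drives the vine's Opacity_Control material parameter, then restores both cameras and disables vine collision.
; Removing the box only clears the Activated flag, leaving the vine unchanged.
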(event OnComponentBeginOverlap(Box)
  (params (OverlappedComponent :type Primitive%20Component%20Object%20Reference) (OtherActor :type Actor%20Object%20Reference) (OtherComp :type Primitive%20Component%20Object%20Reference) (OtherBodyIndex :type Integer) (bFromSweep :type Boolean) (SweepResult :type Hit%20Result%20Structure%20%28by%20ref%29))
  (Utilities|Casting|CastToBP_PushableBox OtherActor)
  (Audio|PlaySound2D "/Game/Audio/Props/Cave_Finish_Open.Cave_Finish_Open" 1.0 1.0 0.0 0 0)
  (Utilities|FlowControl|DoOnce false
    (:Completed
      (Variables|Default|SetActivated? true)
      (Variables|Default|SetStartLocation (Transformation|GetActorLocation (Variables|Default|GetVineReference)))
      (Default|ChangeCameraView (Variables|Default|GetBigCharacterReference) (Variables|Default|GetCameraNumber))
      (Default|ChangeCamera (Variables|Default|GetSmallCharacterReference) (Variables|Default|GetCameraNumber))
      (Utilities|FlowControl|Delay 2.0)
      (CallFunction|CallActivatedEvent))))

(event OnComponentEndOverlap(Box)
  (params (OverlappedComponent :type Primitive%20Component%20Object%20Reference) (OtherActor :type Actor%20Object%20Reference) (OtherComp :type Primitive%20Component%20Object%20Reference) (OtherBodyIndex :type Integer))
  (Utilities|Casting|CastToBP_PushableBox OtherActor)
  (Variables|Default|SetActivated? false))

(event Custom|ActivatedEvent
  (Networking|SwitchHasAuthority
    (:Authority
      (bind _time (Timeline|Timeline_1 PlayFromStart)
        (:Update
          (Rendering|Material|SetScalarParameterValue (Variables|/Game/Blueprints/Interactables/Vines/BP_Vines.BP_Vines_C|GetLines (Variables|Default|GetVineReference)) "Opacity_Control" _time :!class /Script/Engine.MaterialInstanceDynamic)
          (Utilities|FlowControl|DoOnce false
            (:Completed
              (Audio|PlaySound2D "/Game/Audio/Fireball-Strong-Attack-Whoosh-www_fesliyanstudios_com.Fireball-Strong-Attack-Whoosh-www_fesliyanstudios_com" 1.0 1.0 0.0 0 0))))
        (:Finished
          (Default|ChangeCameraView (Variables|Default|GetBigCharacterReference))
          (Default|ChangeCamera (Variables|Default|GetSmallCharacterReference))
          (Collision|SetCollisionEnabled (Variables|/Game/Blueprints/Interactables/Vines/BP_Vines.BP_Vines_C|GetStaticMesh (Variables|Default|GetVineReference)) "NoCollision"))))))

(event Custom|CallActivatedEvent
  (CallFunction|ActivatedEvent))

(event EventBeginPlay
  (Utilities|FlowControl|Delay 0.5)
  (bind _outactors (Actor|GetAllActorsOfClass "/Game/Blueprints/Characters/BP_BigCharacter.BP_BigCharacter_C"))
  (Variables|Default|SetBigCharacterReference (Utilities|Array|Get(acopy) _outactors))
  (bind _outactors_2 (Actor|GetAllActorsOfClass "/Game/Blueprints/Characters/BP_SmallCharacter.BP_SmallCharacter_C"))
  (Variables|Default|SetSmallCharacterReference (Utilities|Array|Get(acopy) _outactors_2)))

(fn ConstructionScript)