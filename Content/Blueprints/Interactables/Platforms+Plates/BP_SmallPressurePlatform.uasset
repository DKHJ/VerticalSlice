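; Pressure plate for the small pushable box that, paired with a big platform, clears the winter ice vines.
; Box overlap sets its active flag only on the first entry, while leaving clears it.
; Tick polls both platforms' flags and fires the vine sequence once.
; A timeline drives the vines' opacity parameter alongside a sound, then switches the small character's camera and disables vine collision.
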(event OnComponentBeginOverlap(Box)
  (params (OverlappedComponent :type Primitive%20Component%20Object%20Reference) (OtherActor :type Actor%20Object%20Reference) (OtherComp :type Primitive%20Component%20Object%20Reference) (OtherBodyIndex :type Integer) (bFromSweep :type Boolean) (SweepResult :type Hit%20Result%20Structure%20%28by%20ref%29))
  (Utilities|Casting|CastToBP_SmallPushableBox OtherActor)
  (Utilities|FlowControl|DoOnce false
    (:Completed
      (Variables|Default|SetSmallPlatformActivated true))))

(event OnComponentEndOverlap(Box)
  (params (OverlappedComponent :type Primitive%20Component%20Object%20Reference) (OtherActor :type Actor%20Object%20Reference) (OtherComp :type Primitive%20Component%20Object%20Reference) (OtherBodyIndex :type Integer))
  (Utilities|Casting|CastToBP_SmallPushableBox OtherActor)
  (Variables|Default|SetSmallPlatformActivated false))

(event Custom|Activated
  (CallFunction|DoInteract))

(event Custom|ActivateTheVines
  (Audio|PlaySound2D "/Game/Assets/Sounds/SFX/IceVineSound.IceVineSound" 1.0 1.0 0.0 0 0)
  (bind _time (Timeline|Timeline_0 Play)
    (:Update
      (Rendering|Material|SetScalarParameterValue (Variables|/Game/Blueprints/Interactables/Vines/BP_WinterBoxVines.BP_WinterBoxVines_C|GetLines (Variables|Default|GetWinterBoxVines)) "Opacity_Control" _time :!class /Script/Engine.MaterialInstanceDynamic))
    (:Finished
      (Default|ChangeCamera (Variables|Default|GetSmallCharRef))
      (Collision|SetCollisionEnabled (Variables|/Game/Blueprints/Interactables/Vines/BP_WinterBoxVines.BP_WinterBoxVines_C|GetStaticMesh (Variables|Default|GetWinterBoxVines)) "NoCollision"))))

(event EventBeginPlay)

(event EventTick
  (params (DeltaSeconds :type Float%20%28single-precision%29))
  (if (and (Variables|Default|GetSmallPlatformActivated) (Variables|/Game/Blueprints/Interactables/Platforms+Plates/BP_WinterActivationPlatform.BP_WinterActivationPlatform_C|GetBigPlatformActivated (Variables|Default|GetBigPlatRef)))
    (Utilities|FlowControl|DoOnce false
      (:Completed
        (bind _outactors (Actor|GetAllActorsOfClass "/Game/Blueprints/Characters/BP_SmallCharacter.BP_SmallCharacter_C"))
        (Variables|Default|SetSmallCharRef (Utilities|Array|Get(acopy) _outactors))
        (CallFunction|ActivatetheVines)))))

(fn ConstructionScript)