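; Magic platform that toggles between solid and passable each time it is interacted with, also toggling once on BeginPlay.
; DoInteract flips Activated and plays a timeline forward or in reverse to fade the Opacity_Control parameter on a dynamic material created in the construction script.
; When the timeline finishes, mesh collision is enabled or disabled to match Activated, whose OnRep function is empty.
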(event EventBeginPlay
  (CallFunction|DoInteract))

(event EventDoInteract
  (if (Variables|Default|GetActivated)
    (Variables|Default|SetActivated false)
    (bind _time (Timeline|Timeline_0 PlayFromStart)
      (:Update
        (Rendering|Material|SetScalarParameterValue (Variables|Default|GetLines) "Opacity_Control" _time :!class /Script/Engine.MaterialInstanceDynamic))
      (:Finished
        (if (Variables|Default|GetActivated)
          (Collision|SetCollisionEnabled (Variables|Default|GetStaticMesh) "QueryAndPhysics")
          (else
            (Collision|SetCollisionEnabled (Variables|Default|GetStaticMesh) "NoCollision")))))
    (else
      (Variables|Default|SetActivated true)
      (Timeline|Timeline_0 ReverseFromEnd))))

(fn ConstructionScript
  (bind _returnvalue (Rendering|Material|CreateDynamicMaterialInstance (Variables|Default|GetStaticMesh) 0 "/Game/Assets/DissolveMaterial/MagicPlatform_INS.MagicPlatform_INS" "None" :!class /Script/Engine.PrimitiveComponent))
  (Variables|Default|SetLines _returnvalue))

(fn OnRepActivated)