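; BP_AutumnVines is an interactable vine that fades in or out and toggles its collision.
; The construction script creates a dynamic material, and BeginPlay sets its Opacity_Control and collision from StartVisible after a short delay.
; Activated drives that parameter through a timeline, reversed from the end when Deactivate is true.
; When that reverse finishes, collision is restored and the cached BP_BigCharacter's camera view is reset to 0.
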(event Custom|Activated
  (params (Deactivate? :type Boolean))
  (if Deactivate?
    (bind _time (Timeline|Time ReverseFromEnd)
      (:Update
        (Rendering|Material|SetScalarParameterValue (Variables|Default|GetLines) "Opacity_Control" _time :!class /Script/Engine.MaterialInstanceDynamic))
      (:Finished
        (if Deactivate?
          (Default|ChangeCameraView (Variables|Default|GetBigCharRef))
          (Collision|SetCollisionEnabled (Variables|Components|GetStaticMesh) "QueryAndPhysics")
          (else
            (Collision|SetCollisionEnabled (Variables|Components|GetStaticMesh) "NoCollision")))))
    (else
      (Timeline|Time Play))))

(event EventBeginPlay
  (Utilities|FlowControl|Delay 0.5)
  (bind _outactors (Actor|GetAllActorsOfClass "/Game/Blueprints/Characters/BP_BigCharacter.BP_BigCharacter_C"))
  (Variables|Default|SetBigCharRef (Utilities|Array|Get(acopy) _outactors))
  (if (Variables|Default|GetStartVisible?)
    (Rendering|Material|SetScalarParameterValue (Variables|Default|GetLines) "Opacity_Control" 0.0 :!class /Script/Engine.MaterialInstanceDynamic)
    (else
      (Rendering|Material|SetScalarParameterValue (Variables|Default|GetLines) "Opacity_Control" 1.0 :!class /Script/Engine.MaterialInstanceDynamic)
      (Collision|SetCollisionEnabled (Variables|Components|GetStaticMesh) "NoCollision"))))

(fn ConstructionScript
  (bind _returnvalue (Rendering|Material|CreateDynamicMaterialInstance (Variables|Components|GetStaticMesh) 0 "/Game/Assets/Vines/Vine_INS.Vine_INS" "None" :!class /Script/Engine.PrimitiveComponent))
  (Variables|Default|SetLines _returnvalue))