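; BP_Vines is an interactable vine actor that fades in or out and toggles its collision when activated.
; A timeline drives Opacity_Control on a dynamic material created in the construction script, with StartVisible setting the initial value.
; Activated wakes net dormancy, plays a sound, and runs the timeline in reverse when Deactivate is true.
; After a short delay, it switches BP_BigCharacter's camera view and sets collision, which is enabled when Deactivate is true.
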(event Custom|Activated
  (params (Deactivate? :type Boolean))
  (bind _outactors (Actor|GetAllActorsOfClass "/Game/Blueprints/Characters/BP_BigCharacter.BP_BigCharacter_C"))
  (Variables|Default|SetBigCharacterReference (Utilities|Array|Get(acopy) _outactors))
  (Networking|ForceNetUpdate)
  (Networking|SetNetDormancy "DORM_Awake")
  (if Deactivate?
    (Audio|PlaySound2D (Variables|Default|GetVineActivateSound) 1.0 1.0 0.0 0 0)
    (bind _time (Timeline|Time ReverseFromEnd)
      (:Update
        (Rendering|Material|SetScalarParameterValue (Variables|Default|GetLines) "Opacity_Control" _time :!class /Script/Engine.MaterialInstanceDynamic))
      (:Finished
        (Utilities|FlowControl|Delay 1.0)
        (Default|ChangeCameraView (Variables|Default|GetBigCharacterReference) (Variables|Default|GetCameraNumber))
        (if Deactivate?
          (Collision|SetCollisionEnabled (Variables|Components|GetStaticMesh) "QueryAndPhysics")
          (else
            (Collision|SetCollisionEnabled (Variables|Components|GetStaticMesh) "NoCollision")))))
    (else
      (Audio|PlaySound2D (Variables|Default|GetVineActivateSound) 1.0 1.0 0.0 0 0)
      (Timeline|Time Play))))

(event EventBeginPlay
  (if (Variables|Default|GetStartVisible?)
    (Rendering|Material|SetScalarParameterValue (Variables|Default|GetLines) "Opacity_Control" 0.0 :!class /Script/Engine.MaterialInstanceDynamic)
    (else
      (Rendering|Material|SetScalarParameterValue (Variables|Default|GetLines) "Opacity_Control" 1.0 :!class /Script/Engine.MaterialInstanceDynamic))))

(fn ConstructionScript
  (bind _returnvalue (Rendering|Material|CreateDynamicMaterialInstance (Variables|Components|GetStaticMesh) 0 (Variables|Default|GetVineMaterialInstance) "None" :!class /Script/Engine.PrimitiveComponent))
  (Variables|Default|SetLines _returnvalue))