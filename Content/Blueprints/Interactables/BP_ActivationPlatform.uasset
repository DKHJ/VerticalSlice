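; BP_ActivationPlatform is a platform that triggers when a BP_PushableBox enters its box, fading and unblocking a referenced vine.
; The first overlap sets Activated and switches both big and small characters' camera views, then waits briefly.
; A timeline drives the vine's Opacity_Control material parameter, then restores both cameras and disables the vine mesh's collision.
; Removing the box clears Activated, but the DoOnce-gated sequence is neither reversed nor replayed.
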(event OnComponentBeginOverlap(Box)
  (params (OverlappedComponent :type Primitive%20Component%20Object%20Reference) (OtherActor :type Actor%20Object%20Reference) (OtherComp :type Primitive%20Component%20Object%20Reference) (OtherBodyIndex :type Integer) (bFromSweep :type Boolean) (SweepResult :type Hit%20Result%20Structure%20%28by%20ref%29))
  (Utilities|Casting|CastToBP_PushableBox OtherActor)
  (Utilities|FlowControl|DoOnce false
    (:Completed
      (Variables|Default|SetActivated? true)
      (Variables|Default|SetStartLocation (Transformation|GetActorLocation (Variables|Default|GetVineReference)))
      (Default|ChangeCamera (Variables|Default|GetSmallCharacterReference) 1)
      (Default|ChangeCameraView (Variables|Default|GetBigCharacterReference) 1)
      (Utilities|FlowControl|Delay 2.0)
      (CallFunction|ActivatedEvent))))

(event OnComponentEndOverlap(Box)
  (params (OverlappedComponent :type Primitive%20Component%20Object%20Reference) (OtherActor :type Actor%20Object%20Reference) (OtherComp :type Primitive%20Component%20Object%20Reference) (OtherBodyIndex :type Integer))
  (Utilities|Casting|CastToBP_PushableBox OtherActor)
  (Variables|Default|SetActivated? false))

(event Custom|ActivatedEvent
  (bind _time (Timeline|Timeline_1 Play)
    (:Update
      (Rendering|Material|SetScalarParameterValue (Variables|/Game/Blueprints/Interactables/BP_Vines.BP_Vines_C|GetLines (Variables|Default|GetVineReference)) "Opacity_Control" _time :!class /Script/Engine.MaterialInstanceDynamic))
    (:Finished
      (Default|ChangeCameraView (Variables|Default|GetBigCharacterReference))
      (Default|ChangeCamera (Variables|Default|GetSmallCharacterReference))
      (Collision|SetCollisionEnabled (Variables|/Game/Blueprints/Interactables/BP_Vines.BP_Vines_C|GetStaticMesh (Variables|Default|GetVineReference)) "NoCollision"))))

(event EventBeginPlay
  (Utilities|FlowControl|Delay 0.2)
  (bind _outactors (Actor|GetAllActorsOfClass "/Game/Blueprints/Characters/BP_BigCharacter.BP_BigCharacter_C"))
  (Variables|Default|SetBigCharacterReference (Utilities|Array|Get(acopy) _outactors))
  (bind _outactors_2 (Actor|GetAllActorsOfClass "/Game/Blueprints/Characters/BP_SmallCharacter.BP_SmallCharacter_C"))
  (Variables|Default|SetSmallCharacterReference (Utilities|Array|Get(acopy) _outactors_2)))

(fn ConstructionScript)