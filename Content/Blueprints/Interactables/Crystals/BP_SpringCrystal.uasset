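; Spring crystal pickup that marks the Spring level complete when the big or small character overlaps its box.
; Collection sets the completion flag and increments the completed-level count in the network game instance, activates the character's pickup particle, plays a 2D sparkle sound and destroys the crystal.
; The big character's path runs this inline, while the small character's path calls ServerCollect, which duplicates the same steps.
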(event OnComponentBeginOverlap(Box)
  (params (OverlappedComponent :type Primitive%20Component%20Object%20Reference) (OtherActor :type Actor%20Object%20Reference) (OtherComp :type Primitive%20Component%20Object%20Reference) (OtherBodyIndex :type Integer) (bFromSweep :type Boolean) (SweepResult :type Hit%20Result%20Structure%20%28by%20ref%29))
  (bind _asbp_big_character (Utilities|Casting|CastToBP_BigCharacter OtherActor)
    (:then
      (bind _asnetwork_game_instance_bp (Utilities|Casting|CastToNetworkGameInstance_BP (Game|GetGameInstance)))
      (Variables|/Game/Blueprints/GameLogic/NetworkGameInstance_BP.NetworkGameInstance_BP_C|SetSpringCompleted _asnetwork_game_instance_bp true)
      (Math|Integer|IncrementInt (Variables|/Game/Blueprints/GameLogic/NetworkGameInstance_BP.NetworkGameInstance_BP_C|GetLevelsCompleted _asnetwork_game_instance_bp)
        (:%20%20
          (Components|Activation|Activate (Variables|/Game/Blueprints/Characters/BP_BigCharacter.BP_BigCharacter_C|GetPickupParticle _asbp_big_character) false)
          (Audio|PlaySound2D "/Game/Audio/fairy-sparkle-02-sound-effect-33959961.fairy-sparkle-02-sound-effect-33959961" 1.0 1.0 0.0 0 0)
          (Actor|DestroyActor))))
    (:CastFailed
      (bind _asbp_small_character (Utilities|Casting|CastToBP_SmallCharacter OtherActor))
      (Networking|SwitchHasAuthority
        (:Authority
          _)
        (:Remote
          _))
      (CallFunction|ServerCollect))))

(event Custom|Server%20Collect
  (bind _asnetwork_game_instance_bp (Utilities|Casting|CastToNetworkGameInstance_BP (Game|GetGameInstance)))
  (Variables|/Game/Blueprints/GameLogic/NetworkGameInstance_BP.NetworkGameInstance_BP_C|SetSpringCompleted _asnetwork_game_instance_bp true)
  (Math|Integer|IncrementInt (Variables|/Game/Blueprints/GameLogic/NetworkGameInstance_BP.NetworkGameInstance_BP_C|GetLevelsCompleted _asnetwork_game_instance_bp)
    (:%20%20
      (Components|Activation|Activate (Variables|/Game/Blueprints/Characters/BP_SmallCharacter.BP_SmallCharacter_C|GetPickupParticle (stale OnComponentBeginOverlap(Box) _asbp_small_character)) false)
      (Audio|PlaySound2D "/Game/Audio/fairy-sparkle-02-sound-effect-33959961.fairy-sparkle-02-sound-effect-33959961" 1.0 1.0 0.0 0 0)
      (Actor|DestroyActor))))

(fn ConstructionScript)