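; Winter puzzle rune that the small character interacts with to trigger a linked pillar and switch on its grid pieces.
; Overlapping its collision registers it as the interactable and enables custom-depth highlighting.
; Interacting toggles its state, plays a teleport-aligned montage, particles and sound, and always activates its grids.
; It also resets other active BP_WinterRune actors cached after BeginPlay, re-triggering their pillars and clearing their grids.
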(event OnComponentBeginOverlap(Collision)
  (params (OverlappedComponent :type Primitive%20Component%20Object%20Reference) (OtherActor :type Actor%20Object%20Reference) (OtherComp :type Primitive%20Component%20Object%20Reference) (OtherBodyIndex :type Integer) (bFromSweep :type Boolean) (SweepResult :type Hit%20Result%20Structure%20%28by%20ref%29))
  (bind _asbp_small_character (Utilities|Casting|CastToBP_SmallCharacter OtherActor))
  (Default|UpdateInteract _asbp_small_character self true)
  (Variables|Default|SetSmallCharacterReference _asbp_small_character)
  (Rendering|SetRenderCustomDepth (Variables|Character|GetMesh) true)
  (Components|Activation|Deactivate (Variables|Default|GetFireflyParticleSystem)))

(event OnComponentEndOverlap(Collision)
  (params (OverlappedComponent :type Primitive%20Component%20Object%20Reference) (OtherActor :type Actor%20Object%20Reference) (OtherComp :type Primitive%20Component%20Object%20Reference) (OtherBodyIndex :type Integer))
  (bind _asbp_small_character (Utilities|Casting|CastToBP_SmallCharacter OtherActor))
  (Default|UpdateInteract _asbp_small_character 0 false)
  (Rendering|SetRenderCustomDepth (Variables|Character|GetMesh) false))

(event Custom|PlaySound
  (Audio|PlaySound2D "/Game/Audio/RuneInteractSound.RuneInteractSound" 1.0 1.0 0.0 0 0))

(event Custom|RunAnimation
  (bind _smallcharacterreference (Variables|Default|GetSmallCharacterReference))
  (Animation|PlayAnimMontage _smallcharacterreference "/Game/Animations/Little/Little_ButtonAnim_Montage.Little_ButtonAnim_Montage" 1.0 "None")
  (Transformation|Teleport _smallcharacterreference (Transformation|GetWorldLocation (Variables|Default|GetAnimationLocation)) "0,90.000000, 0")
  (Utilities|FlowControl|Delay 0.6)
  (Components|Activation|Activate (Variables|Default|GetParticleSystem) false))

(event EventBeginPlay
  (Utilities|FlowControl|Delay 0.3)
  (bind _outactors (Actor|GetAllActorsOfClass "/Game/Blueprints/Interactables/Winter/BP_WinterRune.BP_WinterRune_C"))
  (Variables|Default|SetAllRuneReferences _outactors))

(event EventDoInteract
  (Development|PrintString "Small Rune Activated" true true "(R=0.503929,G=1.000000,B=0.350397,A=1.000000)")
  (if (Variables|Default|GetActivated?)
    (Variables|Default|SetActivated? false)
    (else
      (Variables|Default|SetActivated? true)))
  (CallFunction|RunAnimation)
  (Default|DoInteract (Variables|Default|GetPillarReference))
  (CallFunction|SetGridActivated)
  (CallFunction|ResetAllOtherRunes self)
  (CallFunction|PlaySound))

(fn ConstructionScript
  (|CallParentFunction))

(fn ResetAllOtherRunes
  (params (CurrentRune :type BP%20Winter%20Rune%20Object%20Reference))
  (for _array_element (Variables|Default|GetAllRuneReferences)
    (if (not (== CurrentRune _array_element))
      (if (Variables|/Game/Blueprints/Interactables/Winter/BP_WinterRune.BP_WinterRune_C|GetActivated? _array_element)
        (Variables|/Game/Blueprints/Interactables/Winter/BP_WinterRune.BP_WinterRune_C|SetActivated? _array_element false)
        (Default|DoInteract (Variables|/Game/Blueprints/Interactables/Winter/BP_WinterRune.BP_WinterRune_C|GetPillarReference _array_element))
        (CallFunction|SetGridOff _array_element)))))

(fn SetGridActivated
  (for _array_element (Variables|Default|GetGridReferences)
    (Variables|/Game/Blueprints/Interactables/Winter/BP_GridNode.BP_GridNode_C|SetActivated? _array_element true)))

(fn SetGridOff
  (for _array_element (Variables|Default|GetGridReferences)
    (Variables|/Game/Blueprints/Interactables/Winter/BP_GridNode.BP_GridNode_C|SetActivated? _array_element false)))