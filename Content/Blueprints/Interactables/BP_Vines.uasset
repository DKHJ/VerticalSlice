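; BP_Vines is an interactable vine mesh that fades through a material opacity parameter when activated.
; Construction creates a dynamic instance of Vine_INS, and BeginPlay sets its Opacity_Control from StartVisible.
; Activated plays the Time timeline forward or, when Reversed, backward from the end to drive that parameter.
; When the timeline finishes, LastSpringPuzzleCompleted decides whether the mesh has query and physics collision or none.
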(event Custom|Activated
  (params (Reversed :type Boolean))
  (if Reversed
    (bind _time (Timeline|Time ReverseFromEnd)
      (:Update
        (Rendering|Material|SetScalarParameterValue (Variables|Default|GetLines) "Opacity_Control" _time :!class /Script/Engine.MaterialInstanceDynamic))
      (:Finished
        (if (Variables|Default|GetLastSpringPuzzleCompleted)
          (Collision|SetCollisionEnabled (Variables|Components|GetStaticMesh) "QueryAndPhysics")
          (else
            (Collision|SetCollisionEnabled (Variables|Components|GetStaticMesh) "NoCollision")))))
    (else
      (Timeline|Time Play))))

(event EventBeginPlay
  (if (Variables|Default|GetStartVisible?)
    (Rendering|Material|SetScalarParameterValue (Variables|Default|GetLines) "Opacity_Control" 0.0 :!class /Script/Engine.MaterialInstanceDynamic)
    (else
      (Rendering|Material|SetScalarParameterValue (Variables|Default|GetLines) "Opacity_Control" 1.0 :!class /Script/Engine.MaterialInstanceDynamic))))

(fn ConstructionScript
  (bind _returnvalue (Rendering|Material|CreateDynamicMaterialInstance (Variables|Components|GetStaticMesh) 0 "/Game/Assets/Vines/Vine_INS.Vine_INS" "None" :!class /Script/Engine.PrimitiveComponent))
  (Variables|Default|SetLines _returnvalue))