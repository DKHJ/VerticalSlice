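; Small-character interactable rune that activates a referenced bridge vine object, once only.
; Box overlap registers the rune as the small character's interact target and toggles custom depth on its mesh; leaving clears both.
; DoInteract sets an Activated flag, triggers the vines, plays the character's button montage, teleports it to AnimationLocation, then activates a particle system after a short delay.
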(event OnComponentBeginOverlap(Box)
  (params (OverlappedComponent :type Primitive%20Component%20Object%20Reference) (OtherActor :type Actor%20Object%20Reference) (OtherComp :type Primitive%20Component%20Object%20Reference) (OtherBodyIndex :type Integer) (bFromSweep :type Boolean) (SweepResult :type Hit%20Result%20Structure%20%28by%20ref%29))
  (bind _asbp_small_character (Utilities|Casting|CastToBP_SmallCharacter OtherActor))
  (Default|UpdateInteract _asbp_small_character self true)
  (Variables|Default|SetSmallCharacterReference _asbp_small_character)
  (Rendering|SetRenderCustomDepth (Variables|Default|GetStaticMesh) true))

(event OnComponentEndOverlap(Box)
  (params (OverlappedComponent :type Primitive%20Component%20Object%20Reference) (OtherActor :type Actor%20Object%20Reference) (OtherComp :type Primitive%20Component%20Object%20Reference) (OtherBodyIndex :type Integer))
  (bind _asbp_small_character (Utilities|Casting|CastToBP_SmallCharacter OtherActor))
  (Default|UpdateInteract _asbp_small_character 0 false)
  (Rendering|SetRenderCustomDepth (Variables|Default|GetStaticMesh) false))

(event Custom|CustomEvent_0)

(event EventDoInteract
  (bind _smallcharacterreference (Variables|Default|GetSmallCharacterReference))
  (if (not (Variables|Default|GetActivated?))
    (Variables|Default|SetActivated? true)
    (Default|ActivateVines (Variables|Default|GetBridgeVineRef) true)
    (Animation|PlayAnimMontage _smallcharacterreference "/Game/Animations/Little/Little_ButtonAnim_Montage.Little_ButtonAnim_Montage" 1.0 "None")
    (Transformation|Teleport _smallcharacterreference (Transformation|GetWorldLocation (Variables|Default|GetAnimationLocation)) "0, 0, 0")
    (Utilities|FlowControl|Delay 0.6)
    (Components|Activation|Activate (Variables|Default|GetParticleSystem) false)))

(fn ConstructionScript)