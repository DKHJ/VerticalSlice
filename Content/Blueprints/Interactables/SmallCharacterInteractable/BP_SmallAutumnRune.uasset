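; A one-shot rune interactable that only the small character can use to trigger a linked vine.
; A box overlap registers the rune as that character's interact target and toggles custom depth on its mesh.
; On first interaction it calls the vine, optionally switches the big character's camera view and plays a sound.
; It also teleports the small character to an animation point for a button-press montage, activating particles after a short delay.
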(event OnComponentBeginOverlap(Box)
  (params (OverlappedComponent :type Primitive%20Component%20Object%20Reference) (OtherActor :type Actor%20Object%20Reference) (OtherComp :type Primitive%20Component%20Object%20Reference) (OtherBodyIndex :type Integer) (bFromSweep :type Boolean) (SweepResult :type Hit%20Result%20Structure%20%28by%20ref%29))
  (bind _asbp_small_character (Utilities|Casting|CastToBP_SmallCharacter OtherActor))
  (Default|UpdateInteract _asbp_small_character self true)
  (Variables|Default|SetSmallCharacterReference _asbp_small_character)
  (Rendering|SetRenderCustomDepth (Variables|Default|GetStaticMesh) true))

(event OnComponentEndOverlap(Box)
  (params (OverlappedComponent :type Primitive%20Component%20Object%20Reference) (OtherActor :type Actor%20Object%20Reference) (OtherComp :type Primitive%20Component%20Object%20Reference) (OtherBodyIndex :type Integer))
  (bind _asbp_small_character (Utilities|Casting|CastToBP_SmallCharacter OtherActor))
  (Default|UpdateInteract _asbp_small_character 0 false)
  (Rendering|SetRenderCustomDepth (Variables|Default|GetStaticMesh) false))

(event Custom|RunAnimation
  (bind _smallcharacterreference (Variables|Default|GetSmallCharacterReference))
  (Animation|PlayAnimMontage _smallcharacterreference "/Game/Animations/Little/Little_ButtonAnim_Montage.Little_ButtonAnim_Montage" 1.0 "None")
  (Transformation|Teleport _smallcharacterreference (Transformation|GetWorldLocation (Variables|Default|GetAnimationLocation)) (Variables|Default|GetAnimationRotation))
  (Utilities|FlowControl|Delay 0.6)
  (Components|Activation|Activate (Variables|Default|GetParticleSystem) false))

(event EventBeginPlay
  (bind _outactors (Actor|GetAllActorsOfClass "/Game/Blueprints/Characters/BP_BigCharacter.BP_BigCharacter_C"))
  (Variables|Default|SetBigCharacterReference (Utilities|Array|Get(acopy) _outactors)))

(event EventDoInteract
  (if (not (Variables|Default|GetActivated?))
    (Variables|Default|SetActivated? true)
    (if (Variables|Default|GetCameraEvent)
      (Default|ChangeCameraView (Variables|Default|GetBigCharacterReference) (Variables|Default|GetCameraNumber)))
    (Default|Activated (Variables|Default|GetVineRef) false)
    (CallFunction|RunAnimation)
    (Audio|PlaySound2D "/Game/Audio/220171__gameaudio__flourish-spacey-1.220171__gameaudio__flourish-spacey-1" 1.0 1.0 0.0 0 0)))

(fn ConstructionScript)