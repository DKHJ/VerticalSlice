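; Hub world crystal pillar that displays which of the four season levels are completed and triggers the end-game cinematic.
; On BeginPlay and when BP_BigCharacter overlaps its sphere, it reads completion flags from NetworkGameInstance_BP and sets each crystal slot to its season or opaque material.
; Each completed season calls CheckCompleted, which plays the HubEndGame_SEQ level sequence if all four are done.
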(event OnComponentBeginOverlap(CollisionSphere)
  (params (OverlappedComponent :type Primitive%20Component%20Object%20Reference) (OtherActor :type Actor%20Object%20Reference) (OtherComp :type Primitive%20Component%20Object%20Reference) (OtherBodyIndex :type Integer) (bFromSweep :type Boolean) (SweepResult :type Hit%20Result%20Structure%20%28by%20ref%29))
  (Utilities|Casting|CastToBP_BigCharacter OtherActor)
  (CallFunction|CheckCrystalsCollected))

(event EventBeginPlay
  (CallFunction|CheckCrystalsCollected))

(fn ConstructionScript)

(fn CheckCrystalsCollected
  (bind _asnetwork_game_instance_bp (Utilities|Casting|CastToNetworkGameInstance_BP (Game|GetGameInstance)))
  (bind (_summercompleted _wintercompleted _springcompleted _autumncompleted) (Default|GetLevelsCompleted _asnetwork_game_instance_bp))
  (bind (_array_element _array_index) (Utilities|Array|ForEachLoopwithBreak (Utilities|Array|MakeArray _springcompleted _summercompleted _autumncompleted _wintercompleted))
    (:LoopBody
      (if _array_element
        (switch int _array_index
          (:0
            (Rendering|Material|SetMaterial (Variables|Default|GetStaticMesh) 3 "/Game/Blueprints/Interactables/Crystals/Crystal_Spring_Inst.Crystal_Spring_Inst")
            (CallFunction|CheckCompleted))
          (:1
            (Rendering|Material|SetMaterial (Variables|Default|GetStaticMesh) 0 "/Game/Blueprints/Interactables/Crystals/Crytal_Summer_Inst.Crytal_Summer_Inst")
            (CallFunction|CheckCompleted))
          (:2
            (Rendering|Material|SetMaterial (Variables|Default|GetStaticMesh) 4 "/Game/Blueprints/Interactables/Crystals/Crystal_Autumn_Inst.Crystal_Autumn_Inst")
            (CallFunction|CheckCompleted))
          (:3
            (Rendering|Material|SetMaterial (Variables|Default|GetStaticMesh) 2 "/Game/Blueprints/Interactables/Crystals/Crystal_Winter_Inst.Crystal_Winter_Inst")
            (CallFunction|CheckCompleted)))
        (else
          (switch int _array_index
            (:0
              (Rendering|Material|SetMaterial (Variables|Default|GetStaticMesh) 3 "/Game/Animations/Big/BigGuyOpaque.BigGuyOpaque"))
            (:1
              (Rendering|Material|SetMaterial (Variables|Default|GetStaticMesh) 0 "/Game/Animations/Big/BigGuyOpaque.BigGuyOpaque"))
            (:2
              (Rendering|Material|SetMaterial (Variables|Default|GetStaticMesh) 4 "/Game/Animations/Big/BigGuyOpaque.BigGuyOpaque"))
            (:3
              (Rendering|Material|SetMaterial (Variables|Default|GetStaticMesh) 2 "/Game/Animations/Big/BigGuyOpaque.BigGuyOpaque"))))))))

(fn CheckCompleted
  (bind _asnetwork_game_instance_bp (Utilities|Casting|CastToNetworkGameInstance_BP (Game|GetGameInstance)))
  (bind (_summercompleted _wintercompleted _springcompleted _autumncompleted) (Default|GetLevelsCompleted _asnetwork_game_instance_bp))
  (if (Math|Boolean|ANDBoolean _summercompleted _wintercompleted _springcompleted _autumncompleted)
    (Networking|SwitchHasAuthority
      (:Authority
        _)
      (:Remote
        _))
    (bind _returnvalue (Sequencer|Player|CreateLevelSequencePlayer "/Game/LevelSequences/HubEndGame_SEQ.HubEndGame_SEQ"))
    (Sequencer|Player|Play _returnvalue :!class /Script/MovieScene.MovieSceneSequencePlayer)))