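; Cog wheel controller that reveals and activates cog wheels when a BP_BigCharacter enters its trigger box.
; The overlap runs CheckCogWheels only on the server.
; That event loops over the first three CogWheels references, making each hidden one visible and activated, with debug prints.
; It requires NetworkGameInstance_BP but reads no pickup count from it, despite a comment saying so.
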(event OnComponentBeginOverlap(Box)
  (params (OverlappedComponent :type Primitive%20Component%20Object%20Reference) (OtherActor :type Actor%20Object%20Reference) (OtherComp :type Primitive%20Component%20Object%20Reference) (OtherBodyIndex :type Integer) (bFromSweep :type Boolean) (SweepResult :type Hit%20Result%20Structure%20%28by%20ref%29))
  (Utilities|Casting|CastToBP_BigCharacter OtherActor)
  (Networking|SwitchHasAuthority
    (:Authority
      (Development|PrintString "[SERVER] Checking Cog Progress..." true true "(R=1.000000,G=0.675707,B=0.449984,A=1.000000)")
      (CallFunction|CheckCogWheels))))

(event Custom|CheckCogWheels
  ;[1 1 1] First we get the number of cogs picked up
  (Utilities|Casting|CastToNetworkGameInstance_BP (Game|GetGameInstance))
  (for _index (range 0 2)
    ;[1 1 1] Check through our references based on the cog number
    (if (not (Variables|/Game/Blueprints/BP_CogWheel.BP_CogWheel_C|GetVisible (Utilities|Array|Get(acopy) (Variables|Default|GetCogWheels) _index)))
      (Default|SetVisible (Utilities|Array|Get(acopy) (Variables|Default|GetCogWheels) _index) true)
      (Variables|/Game/Blueprints/BP_CogWheel.BP_CogWheel_C|SetActivated (Utilities|Array|Get(acopy) (Variables|Default|GetCogWheels) _index) true)
      (Development|PrintString "Cog Activated & Visible"))))

(fn ConstructionScript)