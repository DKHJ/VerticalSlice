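; ResetPuzzle_BP is a trigger volume that resets the kick-block puzzle when the big character steps into it.
; Shortly after BeginPlay it caches the first BP_KickBlock in the level.
; On overlap by BP_BigCharacter it clears that block's current node and teleports it back to a hardcoded start location.
; Unconnected test logic for resetting activated winter pillars is present but never runs.
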(event OnComponentBeginOverlap(Box)
  (params (OverlappedComponent :type Primitive%20Component%20Object%20Reference) (OtherActor :type Actor%20Object%20Reference) (OtherComp :type Primitive%20Component%20Object%20Reference) (OtherBodyIndex :type Integer) (bFromSweep :type Boolean) (SweepResult :type Hit%20Result%20Structure%20%28by%20ref%29))
  (bind _puzzlekickblock (Variables|Default|GetPuzzleKickBlock))
  (Utilities|Casting|CastToBP_BigCharacter OtherActor)
  (Variables|/Game/Blueprints/Interactables/BigCharacterInteractable/BP_KickBlock.BP_KickBlock_C|SetCurrent%20Node _puzzlekickblock 0)
  (Transformation|Teleport _puzzlekickblock "-1446.482544,135.000000,-15.000000" "0, 0, 0"))

(event EventBeginPlay
  (Utilities|FlowControl|Delay 0.2)
  (bind _outactors (Actor|GetAllActorsOfClass "/Game/Blueprints/Interactables/BigCharacterInteractable/BP_KickBlock.BP_KickBlock_C"))
  (Variables|Default|SetPuzzleKickBlock (Utilities|Array|Get(acopy) _outactors)))

(event EventTick
  (params (DeltaSeconds :type Float%20%28single-precision%29)))

(fn ConstructionScript)