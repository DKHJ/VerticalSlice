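; Replicated throwable box that the Big Character can pick up, while the Small Character only registers it.
; Box overlaps update each character's interact state, with outline highlighting for the Big Character.
; On BeginPlay the server sets the Big Character as owner; authority-gated interaction drives its pickup animation, disables physics and collision, and attaches the mesh to its palm socket.
; Hits while held, or from the Small Character, re-enable physics and movement replication.
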(event OnComponentBeginOverlap(Box)
  (params (OverlappedComponent :type Primitive%20Component%20Object%20Reference) (OtherActor :type Actor%20Object%20Reference) (OtherComp :type Primitive%20Component%20Object%20Reference) (OtherBodyIndex :type Integer) (bFromSweep :type Boolean) (SweepResult :type Hit%20Result%20Structure%20%28by%20ref%29))
  ;[0.5262 1 0.5526] BEGIN Overlap
  (if (not (Variables|Default|GetbPickedUp))
    (switch string (Utilities|String|ToString(Name) (Utilities|Array|Get(acopy) (Variables|/Script/Engine.Actor|GetTags OtherActor)))
      (:BigCharacter
        ;[0.5262 1 0.5526] BigCharacter
        (bind _asbp_big_character (Utilities|Casting|CastToBP_BigCharacter OtherActor))
        (bind _output_get (Variables|Default|SetBigCharRef _asbp_big_character))
        (Default|UpdateInteract _output_get self true)
        (Rendering|SetRenderCustomDepth (Variables|Default|GetMesh) true)
        (Components|Activation|SetActive (Variables|Default|GetParticleSystem) false false))
      (:SmallCharacter
        ;[0.4547 0.9402 1] SmallCharacter
        (bind _asbp_small_character (Utilities|Casting|CastToBP_SmallCharacter OtherActor))
        (bind _output_get_2 (Variables|Default|SetSmallCharRef _asbp_small_character))
        (Default|UpdateInteract _output_get_2 self false)
        (Components|Activation|SetActive (Variables|Default|GetParticleSystem) false false)
        (Variables|/Game/Blueprints/Characters/BP_SmallCharacter.BP_SmallCharacter_C|SetbLookingAtBox _output_get_2 true)))))

(event OnComponentEndOverlap(Box)
  (params (OverlappedComponent :type Primitive%20Component%20Object%20Reference) (OtherActor :type Actor%20Object%20Reference) (OtherComp :type Primitive%20Component%20Object%20Reference) (OtherBodyIndex :type Integer))
  (bind _asbp_big_character (Utilities|Casting|CastToBP_BigCharacter OtherActor)
    (:then
      (Default|UpdateInteract _asbp_big_character self false)
      (Rendering|SetRenderCustomDepth (Variables|Default|GetMesh) false)
      (Components|Activation|Deactivate (Variables|Default|GetParticleSystem)))
    (:CastFailed
      (bind _asbp_small_character (Utilities|Casting|CastToBP_SmallCharacter OtherActor))
      (Default|UpdateInteract _asbp_small_character 0 false)
      (Components|Activation|Deactivate (Variables|Default|GetParticleSystem))
      (Variables|/Game/Blueprints/Characters/BP_SmallCharacter.BP_SmallCharacter_C|SetbLookingAtBox _asbp_small_character true))))

(event Custom|Server%20Interact
  (bind _bigcharref (Variables|Default|GetBigCharRef))
  (bind _bigcharref_2 (Variables|Default|GetBigCharRef))
  (bind _biganimbp (Variables|/Game/Blueprints/Characters/BP_BigCharacter.BP_BigCharacter_C|GetBigAnimBP _bigcharref))
  (Networking|ForceNetUpdate)
  (Networking|SetNetDormancy "DORM_Awake")
  (if (Variables|/Game/Blueprints/Characters/BP_BigCharacter.BP_BigCharacter_C|GetbPickedUpBox _bigcharref_2)
    (Development|PrintString "Error: Character already has a box picked up" true true "(R=1.000000,G=0.000000,B=0.031819,A=1.000000)" 4.0)
    (else
      (Variables|/Game/Blueprints/Characters/BP_BigCharacter.BP_BigCharacter_C|SetThrowableBoxReference _bigcharref_2 self)
      (Rendering|SetRenderCustomDepth (Variables|Default|GetMesh) false)
      (Variables|/Game/Blueprints/Characters/BP_BigCharacter.BP_BigCharacter_C|SetbPickedUpBox _bigcharref true)
      (Variables|/Game/Animations/Big/Big_AnimBP.Big_AnimBP_C|SetbWaitForPickup _biganimbp true)
      (Variables|/Game/Animations/Big/Big_AnimBP.Big_AnimBP_C|SetbPickUpBox _biganimbp true)
      (Physics|SetSimulatePhysics (Variables|Default|GetMesh) false)
      (Collision|SetCollisionEnabled (Variables|Default|GetMesh) "NoCollision")
      (bind _returnvalue (Transformation|AttachComponentToComponent (Variables|Default|GetMesh) (Variables|/Script/Engine.Character|GetMesh _bigcharref) "ApeLPalmSocket" "SnapToTarget" "KeepWorld" "KeepRelative" true))
      (if _returnvalue
        (Transformation|SetActorLocation (Transformation|GetSocketLocation (Variables|/Script/Engine.Character|GetMesh (Variables|Default|GetBigCharRef)) "ApeLPalmSocket") false true)
        (else
          (Development|PrintString "Attachment Failed!"))))))

(event Custom|DestroySelf
  (params (Delay :type Float%20%28single-precision%29))
  (Utilities|FlowControl|Delay Delay)
  (Actor|DestroyActor))

(event Collision|EventHit
  (params (MyComp :type Primitive%20Component%20Object%20Reference) (Other :type Actor%20Object%20Reference) (OtherComp :type Primitive%20Component%20Object%20Reference) (bSelfMoved :type Boolean) (HitLocation :type Vector :default "0, 0, 0") (HitNormal :type Vector :default "0, 0, 0") (NormalImpulse :type Vector :default "0, 0, 0") (Hit :type Hit%20Result%20Structure%20%28by%20ref%29))
  (if (Variables|Default|GetbPickedUp)
    (Physics|SetSimulatePhysics (Variables|Default|GetMesh) true)
    (Variables|Default|SetbPickedUp false)
    (Class|Actor|SetReplicateMovement true)
    (else
      (Utilities|Casting|CastToBP_SmallCharacter Other)
      (Physics|SetSimulatePhysics (Variables|Default|GetMesh) true)
      (Class|Actor|SetReplicateMovement true))))

(event EventBeginPlay
  ;[1 1 1] Set the owner of these actors to the Big Character ( Server )
  (Networking|SwitchHasAuthority
    (:Authority
      (bind _returnvalue (Actor|GetActorOfClass "/Game/Blueprints/Characters/BP_BigCharacter.BP_BigCharacter_C"))
      (Actor|SetOwner _returnvalue)
      (Development|PrintString (Utilities|GetDisplayName _returnvalue)))))

(event EventDoInteract
  (Networking|SwitchHasAuthority
    (:Authority
      (if (not (Variables|Default|GetbPickedUp))
        (Variables|Default|SetbPickedUp true)
        (CallFunction|ServerInteract)))))

(fn ConstructionScript)