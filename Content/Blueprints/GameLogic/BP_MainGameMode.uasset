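; Game mode that starts a local two-player session with one big character and one small character.
; On BeginPlay it collects all PlayerStart actors and keeps the first two by array index, not by tag.
; It spawns BP_BigCharacter at the first for player controller 0, then creates a second local player and has it possess BP_SmallCharacter spawned at the second.
; Spawns use only each start's location.
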(event EventBeginPlay
  (CallFunction|GetAllPlayerStarts)
  (CallFunction|SpawnAllPlayers))

(fn ConstructionScript)

(fn GetAllPlayerStarts
  (Development|PrintString "[GM] Get All Player Starts" true true "(R=1.000000,G=0.749869,B=0.366636,A=1.000000)")
  (bind _outactors (Actor|GetAllActorsOfClass "/Script/Engine.PlayerStart"))
  (bind _output_get (Variables|Default|SetPlayerStartArray _outactors))
  (Variables|Default|SetPlayerStart1 (Utilities|Array|Get(acopy) _output_get))
  (Variables|Default|SetPlayerStart2 (Utilities|Array|Get(acopy) _output_get 1)))

(fn SpawnAllPlayers
  (Development|PrintString "[GM] Spawn All Players" true true "(R=1.000000,G=0.749869,B=0.366636,A=1.000000)")
  (Utilities|FlowControl|Sequence
    (:then_0
      ;[0.3228 0.9901 1] Spawn a character, get the player controller to Possess it.
      (bind _returnvalue (Game|SpawnActorfromClass "/Game/Blueprints/Characters/BP_BigCharacter.BP_BigCharacter_C" (Math|Conversions|ToTransform(Vector) (Transformation|GetActorLocation (Variables|Default|GetPlayerStart1))) "Undefined" 0 0))
      (Pawn|Possess (Game|GetPlayerController 0) _returnvalue))
    (:then_1
      ;[0.3228 0.9901 1] Spawn a character, get the player controller to Possess it.
      (bind _returnvalue_2 (Class|GameplayStatics|CreatePlayer 1))
      (bind _returnvalue_3 (Game|SpawnActorfromClass "/Game/Blueprints/Characters/BP_SmallCharacter.BP_SmallCharacter_C" (Math|Conversions|ToTransform(Vector) (Transformation|GetActorLocation (Variables|Default|GetPlayerStart2))) "Undefined" 0 0))
      (Pawn|Possess _returnvalue_2 _returnvalue_3))))