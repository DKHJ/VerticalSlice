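; Vine bridge actor that fades in or out and toggles its collision when activated.
; Construction creates a dynamic material instance, whose Opacity_Control parameter is driven by timelines, with zero as the revealed state.
; The one-way activation event switches BP_BigCharacter's camera during the reveal, while ActivateVines handles both directions, each with a sound.
; Collision starts disabled, even when StartVisible shows the bridge.
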(event Custom|ActivateVines
  (params (Activated? :type Boolean))
  (Audio|PlaySound2D "/Game/Assets/Sounds/SFX/NormalVineActivateSound.NormalVineActivateSound" 1.0 1.0 0.0 0 0)
  (if Activated?
    (CallFunction|DoInteract)
    (bind _time (Timeline|Timeline_0 ReverseFromEnd)
      (:Update
        (Rendering|Material|SetScalarParameterValue (Variables|Default|GetLines) "Opacity_Control" _time :!class /Script/Engine.MaterialInstanceDynamic))
      (:Finished
        (Default|ChangeCameraView (Variables|Default|GetBigCharRef))
        (Rendering|Material|SetScalarParameterValue (Variables|Default|GetLines) "Opacity_Control" 0.0 :!class /Script/Engine.MaterialInstanceDynamic)
        (Collision|SetActorEnableCollision true)))
    (else
      (CallFunction|DoInteract)
      (bind _time_2 (Timeline|Timeline_1 PlayFromStart)
        (:Update
          (Rendering|Material|SetScalarParameterValue (Variables|Default|GetLines) "Opacity_Control" _time_2 :!class /Script/Engine.MaterialInstanceDynamic))
        (:Finished
          (Collision|SetActorEnableCollision false))))))

(event EventBeginPlay
  (bind _outactors (Actor|GetAllActorsOfClass "/Game/Blueprints/Characters/BP_BigCharacter.BP_BigCharacter_C"))
  (Variables|Default|SetBigCharRef (Utilities|Array|Get(acopy) _outactors))
  (Collision|SetActorEnableCollision false)
  (if (Variables|Default|GetStartVisible?)
    (Rendering|Material|SetScalarParameterValue (Variables|Default|GetLines) "Opacity_Control" 0.0 :!class /Script/Engine.MaterialInstanceDynamic)
    (else
      (Rendering|Material|SetScalarParameterValue (Variables|Default|GetLines) "Opacity_Control" 1.0 :!class /Script/Engine.MaterialInstanceDynamic))))

(event EventOnActivatedVineBridgeEvent
  (Default|ChangeCameraView (Variables|Default|GetBigCharRef) 2)
  (Audio|PlaySound2D "/Game/Assets/Sounds/SFX/NormalVineActivateSound.NormalVineActivateSound" 1.0 1.0 0.0 0 0)
  (Utilities|FlowControl|Delay 1.0)
  (bind _time (Timeline|Time ReverseFromEnd)
    (:Update
      (Rendering|Material|SetScalarParameterValue (Variables|Default|GetLines) "Opacity_Control" _time :!class /Script/Engine.MaterialInstanceDynamic)
      (Collision|SetActorEnableCollision true))
    (:Finished
      (Utilities|FlowControl|Delay 0.5)
      (Default|ChangeCameraView (Variables|Default|GetBigCharRef))
      (Rendering|Material|SetScalarParameterValue (Variables|Default|GetLines) "Opacity_Control" 0.0 :!class /Script/Engine.MaterialInstanceDynamic)
      (Collision|SetActorEnableCollision true))))

(fn ConstructionScript
  (bind _returnvalue (Rendering|Material|CreateDynamicMaterialInstance (Variables|Character|GetMesh) 0 (Variables|Default|GetVineBridgeMaterialInst) "None" :!class /Script/Engine.PrimitiveComponent))
  (Variables|Default|SetLines _returnvalue))

(fn DoInteraction
  (return false))