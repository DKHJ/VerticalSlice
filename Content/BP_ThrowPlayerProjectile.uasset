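; BP_ThrowPlayerProjectile is a projectile that stands in for a thrown player and turns back into a small character on impact.
; On BeginPlay it makes itself the view target of player controller 1 and caches its starting rotation.
; On hit it spawns BP_SmallCharacter at Sphere1's location using the cached roll and yaw, has that controller possess it, then destroys itself.
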(event EventBeginPlay
  (Game|Player|SetViewTargetwithBlend (Game|GetPlayerController 1) self 0.0 "VTBlend_Linear" 0.0 false)
  (Variables|Default|SetStartRotation (Transformation|GetActorRotation self)))

(event Collision|EventHit
  (params (MyComp :type Primitive%20Component%20Object%20Reference) (Other :type Actor%20Object%20Reference) (OtherComp :type Primitive%20Component%20Object%20Reference) (bSelfMoved :type Boolean) (HitLocation :type Vector :default "0, 0, 0") (HitNormal :type Vector :default "0, 0, 0") (NormalImpulse :type Vector :default "0, 0, 0") (Hit :type Hit%20Result%20Structure%20%28by%20ref%29))
  (bind _startrotation (Variables|Default|GetStartRotation))
  (bind _returnvalue (Game|SpawnActorfromClass "/Game/Blueprints/Characters/BP_SmallCharacter.BP_SmallCharacter_C" (Math|Transform|MakeTransform (Transformation|GetWorldLocation (Variables|Default|GetSphere1)) (Math|Rotator|MakeRotator (.roll _startrotation) 0.0 (.yaw _startrotation))) "AdjustIfPossibleButAlwaysSpawn" 0 0))
  (Pawn|Possess (Game|GetPlayerController 1) _returnvalue)
  (Actor|DestroyActor) ; Then destroy this projectile
)

(fn ConstructionScript)