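; Brambles is an interactable obstacle that blocks the small character and can be destroyed by the big character.
; A box overlap teleports actors tagged SmallCharacter to a TeleportLocation, while BP_BigCharacter gets this actor as its interact target and the mesh gains a custom depth highlight.
; DoInteract runs only with authority, calling ServerStomp to play a stomp montage on that character, then destroy the brambles after a short delay.
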(event OnComponentBeginOverlap(Box)
  (params (OverlappedComponent :type Primitive%20Component%20Object%20Reference) (OtherActor :type Actor%20Object%20Reference) (OtherComp :type Primitive%20Component%20Object%20Reference) (OtherBodyIndex :type Integer) (bFromSweep :type Boolean) (SweepResult :type Hit%20Result%20Structure%20%28by%20ref%29))
  (if (Actor|ActorHasTag OtherActor "SmallCharacter")
    (Transformation|Teleport OtherActor (Transformation|GetActorLocation (Variables|Default|GetTeleportLocation)) "0, 0, 0")
    (else
      (bind _asbp_big_character (Utilities|Casting|CastToBP_BigCharacter OtherActor))
      (Variables|/Game/Blueprints/Characters/BP_BigCharacter.BP_BigCharacter_C|SetInteractActorReference _asbp_big_character self)
      (Variables|/Game/Blueprints/Characters/BP_BigCharacter.BP_BigCharacter_C|SetCanInteract _asbp_big_character true)
      (Variables|Default|SetBigCharRef _asbp_big_character)
      (Rendering|SetRenderCustomDepth (Variables|Default|GetStaticMesh) true))))

(event OnComponentEndOverlap(Box)
  (params (OverlappedComponent :type Primitive%20Component%20Object%20Reference) (OtherActor :type Actor%20Object%20Reference) (OtherComp :type Primitive%20Component%20Object%20Reference) (OtherBodyIndex :type Integer))
  (bind _asbp_big_character (Utilities|Casting|CastToBP_BigCharacter OtherActor))
  (Variables|/Game/Blueprints/Characters/BP_BigCharacter.BP_BigCharacter_C|SetInteractActorReference _asbp_big_character 0)
  (Variables|/Game/Blueprints/Characters/BP_BigCharacter.BP_BigCharacter_C|SetCanInteract _asbp_big_character false)
  (Rendering|SetRenderCustomDepth (Variables|Default|GetStaticMesh) false))

(event Custom|ServerStomp
  (Animation|PlayAnimMontage (Variables|Default|GetBigCharRef) "/Game/Animations/Big/Big_Stomp_Montage.Big_Stomp_Montage" 1.0 "None")
  (Utilities|FlowControl|Delay 0.5)
  (Actor|DestroyActor))

(event EventBeginPlay)

(event Collision|EventActorBeginOverlap
  (params (OtherActor :type Actor%20Object%20Reference)))

(event EventTick
  (params (DeltaSeconds :type Float%20%28single-precision%29)))

(event EventDoInteract
  (Networking|SwitchHasAuthority
    (:Authority
      (CallFunction|ServerStomp))))

(fn ConstructionScript)

(fn DoInteraction
  (return false))