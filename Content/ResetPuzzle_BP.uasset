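; Puzzle reset trigger that puts a kickable puzzle block back on a grid node when BP_BigCharacter enters its box.
; The overlap teleports PuzzleKickBlock to the GridNode's world location with zeroed rotation.
; BeginPlay caches all BP_WinterPillar actors after a short delay, but the loop meant to reset activated pillars is an unconnected test that never runs.
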(event OnComponentBeginOverlap(Box)
  (params (OverlappedComponent :type Primitive%20Component%20Object%20Reference) (OtherActor :type Actor%20Object%20Reference) (OtherComp :type Primitive%20Component%20Object%20Reference) (OtherBodyIndex :type Integer) (bFromSweep :type Boolean) (SweepResult :type Hit%20Result%20Structure%20%28by%20ref%29))
  (Utilities|Casting|CastToBP_BigCharacter OtherActor)
  (Transformation|Teleport (Variables|Default|GetPuzzleKickBlock) (Transformation|GetWorldLocation (Variables|/Game/Blueprints/Interactables/Winter/BP_GridNode.BP_GridNode_C|GetDefaultSceneRoot (Variables|Default|GetGridNode))) "0, 0, 0"))

(event EventBeginPlay
  (Utilities|FlowControl|Delay 0.5)
  (bind _outactors (Actor|GetAllActorsOfClass "/Game/Blueprints/Interactables/Winter/BP_WinterPillar.BP_WinterPillar_C"))
  (Variables|Default|SetWinterPillarRef _outactors))

(event Collision|EventActorBeginOverlap
  (params (OtherActor :type Actor%20Object%20Reference)))

(event EventTick
  (params (DeltaSeconds :type Float%20%28single-precision%29)))

(fn ConstructionScript)