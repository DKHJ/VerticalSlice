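; Sliding-puzzle piece that moves one piece-length into a free neighboring space when BP_BigCharacter pushes it.
; Overlapping XBox or YBox sets the character's pushing animation flag and calls MovePuzzlePiece; leaving clears the flag.
; MovePuzzlePiece line-traces candidate directions in fixed order, then a timeline lerps the piece toward the first unblocked one with sweep.
; InitPuzzlePiece passes puzzle index and grid size to a dynamic material.
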(event OnComponentBeginOverlap(XBox)
  (params (OverlappedComponent :type Primitive%20Component%20Object%20Reference) (OtherActor :type Actor%20Object%20Reference) (OtherComp :type Primitive%20Component%20Object%20Reference) (OtherBodyIndex :type Integer) (bFromSweep :type Boolean) (SweepResult :type Hit%20Result%20Structure%20%28by%20ref%29))
  (bind _asbp_big_character (Utilities|Casting|CastToBP_BigCharacter OtherActor))
  (Variables|/Game/Animations/Big/Big_AnimBP.Big_AnimBP_C|SetbIsPushing (Variables|/Game/Blueprints/Characters/BP_BigCharacter.BP_BigCharacter_C|GetBigAnimBP _asbp_big_character) true)
  (CallFunction|MovePuzzlePiece))

(event OnComponentEndOverlap(XBox)
  (params (OverlappedComponent :type Primitive%20Component%20Object%20Reference) (OtherActor :type Actor%20Object%20Reference) (OtherComp :type Primitive%20Component%20Object%20Reference) (OtherBodyIndex :type Integer))
  (bind _asbp_big_character (Utilities|Casting|CastToBP_BigCharacter OtherActor))
  (Variables|/Game/Animations/Big/Big_AnimBP.Big_AnimBP_C|SetbIsPushing (Variables|/Game/Blueprints/Characters/BP_BigCharacter.BP_BigCharacter_C|GetBigAnimBP _asbp_big_character) false))

(event OnComponentBeginOverlap(YBox)
  (params (OverlappedComponent :type Primitive%20Component%20Object%20Reference) (OtherActor :type Actor%20Object%20Reference) (OtherComp :type Primitive%20Component%20Object%20Reference) (OtherBodyIndex :type Integer) (bFromSweep :type Boolean) (SweepResult :type Hit%20Result%20Structure%20%28by%20ref%29))
  (bind _asbp_big_character (Utilities|Casting|CastToBP_BigCharacter OtherActor))
  (Variables|/Game/Animations/Big/Big_AnimBP.Big_AnimBP_C|SetbIsPushing (Variables|/Game/Blueprints/Characters/BP_BigCharacter.BP_BigCharacter_C|GetBigAnimBP _asbp_big_character) true)
  (CallFunction|MovePuzzlePiece))

(event OnComponentEndOverlap(YBox)
  (params (OverlappedComponent :type Primitive%20Component%20Object%20Reference) (OtherActor :type Actor%20Object%20Reference) (OtherComp :type Primitive%20Component%20Object%20Reference) (OtherBodyIndex :type Integer))
  (bind _asbp_big_character (Utilities|Casting|CastToBP_BigCharacter OtherActor))
  (Variables|/Game/Animations/Big/Big_AnimBP.Big_AnimBP_C|SetbIsPushing (Variables|/Game/Blueprints/Characters/BP_BigCharacter.BP_BigCharacter_C|GetBigAnimBP _asbp_big_character) false))

(event Custom|Move%20Puzzle%20Piece
  ;[1 1 1] Time Movement Event
  (bind _index (Utilities|FlowControl|ForLoopwithBreak 0 100)
    (:LoopBody
      (bind _movedirection (Utilities|CheckMoveDirection (Utilities|Select :Index _index :Option%200 "NewEnumerator0" :Option%201 "NewEnumerator1" :Option%202 "NewEnumerator2" :Option%203 "NewEnumerator3"))
        (:Free
          (Variables|Default|SetMovementDirection _movedirection)
          (CallFunction|BreakforLoop)
          (Variables|Default|SetPuzzlePieceLastLocation (Transformation|GetActorLocation))
          (bind _lerptime (Timeline|MovementTimeline PlayFromStart)
            (:Update
              (Transformation|SetActorLocation (Math|Vector|Lerp(Vector) (Variables|Default|GetPuzzlePieceLastLocation) (+ (Variables|Default|GetPuzzlePieceLastLocation) (* (Variables|Default|GetMovementDirection) (Variables|Default|GetPuzzlePieceSize))) _lerptime) true false))))))))

(event Custom|Break%20For%20Loop
  ;[1 1 1] Time Movement Event
  (Utilities|FlowControl|ForLoopwithBreak 0 100) ; enters at Break
)

(fn ConstructionScript)

(fn InitPuzzlePiece
  (params (PuzzleIndex :type Integer) (GridSize :type Integer))
  (bind _staticmesh (Variables|Default|GetStaticMesh))
  (bind _returnvalue (Rendering|Material|CreateDynamicMaterialInstance _staticmesh 0 (Rendering|Material|GetMaterial _staticmesh 0) "None" :!class /Script/Engine.PrimitiveComponent))
  (Rendering|Material|SetScalarParameterValue _returnvalue "[Puzzle Index]" (Math|Conversions|ToFloat(Integer) PuzzleIndex) :!class /Script/Engine.MaterialInstanceDynamic)
  (Rendering|Material|SetScalarParameterValue _returnvalue "Grid Size" (Math|Conversions|ToFloat(Integer) GridSize) :!class /Script/Engine.MaterialInstanceDynamic)
  (Rendering|Material|SetMaterial _staticmesh 0 _returnvalue))