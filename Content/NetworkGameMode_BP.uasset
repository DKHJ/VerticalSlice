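; Game mode for a two-player networked game that pairs a big character with a small one.
; On server PostLogin it sorts PlayerStarts by tag, numbers the player and calls ClientPostLogin on their controller.
; RespawnPlayerEvent destroys the current pawn, then possesses a new big character for the first PlayerArray entry, small otherwise.
; GetAllPlayerStarts and SpawnAllPlayers form a separate local two-player spawn path, uncalled here.
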(event Custom|RespawnPlayer
  (params (NPC :type Player%20Controller%20Object%20Reference)))

(event Custom|RespawnPlayerEvent
  (params (PlayerController :type Player%20Controller%20Object%20Reference))
  (bind _returnvalue (Pawn|GetControlledPawn PlayerController))
  (Utilities|IsValid _returnvalue
    (:Is%20Valid
      (Actor|DestroyActor _returnvalue))
    (:Is%20Not%20Valid
      _))
  (if (== (Variables|/Script/Engine.PlayerState|GetPlayerId (Utilities|Array|Get(acopy) (Variables|/Script/Engine.GameState|GetPlayerArray (Game|GetGameState)))) (Variables|/Script/Engine.PlayerState|GetPlayerId (Variables|/Script/Engine.Controller|GetPlayerState PlayerController)))
    (bind _returnvalue_2 (Game|SpawnActorfromClass "/Game/Blueprints/Characters/BP_BigCharacter.BP_BigCharacter_C" (Transformation|GetActorTransform (Utilities|Array|Get(acopy) (Variables|Default|GetPlayer1))) "AdjustIfPossibleButDontSpawnIfColliding" 0 0))
    (Pawn|Possess PlayerController _returnvalue_2)
    (else
      (bind _returnvalue_3 (Game|SpawnActorfromClass "/Game/Blueprints/Characters/BP_SmallCharacter.BP_SmallCharacter_C" (Transformation|GetActorTransform (Utilities|Array|Get(acopy) (Variables|Default|GetPlayer2))) "AdjustIfPossibleButDontSpawnIfColliding" 0 0))
      (Pawn|Possess PlayerController _returnvalue_3))))

(event EventPostLogin
  (params (NewPlayer :type Player%20Controller%20Object%20Reference))
  (Networking|SwitchHasAuthority
    (:Authority
      (bind _outactors (Actor|GetAllActorsOfClass "/Script/Engine.PlayerStart"))
      (for _array_element _outactors
        (if (Utilities|Name|Equal(Name) (Variables|/Script/Engine.PlayerStart|GetPlayerStartTag _array_element) "Player1")
          (Utilities|Array|AddUnique (Variables|Default|GetPlayer1) _array_element)
          (else
            (Utilities|Array|AddUnique (Variables|Default|GetPlayer2) _array_element))))
      (bind _asnetwork_player_state_bp (Utilities|Casting|CastToNetworkPlayerState_BP (Variables|/Script/Engine.Controller|GetPlayerState NewPlayer)))
      (Variables|/Game/NetworkPlayerState_BP.NetworkPlayerState_BP_C|SetPlayerNumber _asnetwork_player_state_bp (Utilities|Array|Length (Variables|/Script/Engine.GameStateBase|GetPlayerArray (Game|GetGameState))))
      (bind _asnetwork_player_controller_bp (Utilities|Casting|CastToNetworkPlayerController_BP NewPlayer))
      (Default|ClientPostLogin _asnetwork_player_controller_bp))))

(fn ConstructionScript)

(fn GetAllPlayerStarts
  (Development|PrintString "[GM] Get All Player Starts" true true "(R=1.000000,G=0.749869,B=0.366636,A=1.000000)")
  (bind _outactors (Actor|GetAllActorsOfClass "/Script/Engine.PlayerStart"))
  (bind _output_get (Variables|Default|SetPlayerStartArray _outactors))
  (Variables|Default|SetPlayer%20Start%201 (Utilities|Array|Get(acopy) _output_get))
  (Variables|Default|SetPlayer%20Start%202 (Utilities|Array|Get(acopy) _output_get 1)))

(fn SpawnAllPlayers
  (Development|PrintString "[GM] Spawn All Players" true true "(R=1.000000,G=0.749869,B=0.366636,A=1.000000)")
  (Utilities|FlowControl|Sequence
    (:then_0
      ;[0.3228 0.9901 1] Spawn a character, get the player controller to Possess it.
      (bind _returnvalue (Game|SpawnActorfromClass "/Game/Blueprints/Characters/BP_BigCharacter.BP_BigCharacter_C" (Math|Conversions|ToTransform(Vector) (Transformation|GetActorLocation (Variables|Default|GetPlayer%20Start%201))) "Undefined" 0 0))
      (Pawn|Possess (Game|GetPlayerController 0) _returnvalue))
    (:then_1
      ;[0.3228 0.9901 1] Spawn a character, get the player controller to Possess it.
      (Class|GameplayStatics|CreatePlayer 1)
      (bind _returnvalue_2 (Game|SpawnActorfromClass "/Game/Blueprints/Characters/BP_SmallCharacter.BP_SmallCharacter_C" (Math|Conversions|ToTransform(Vector) (Transformation|GetActorLocation (Variables|Default|GetPlayer%20Start%202))) "Undefined" 0 0))
      (Pawn|Possess (Game|GetPlayerController 1) _returnvalue_2))))