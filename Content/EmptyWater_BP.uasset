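; EmptyWater_BP is a water volume that sends the small character back to a teleport location and lets the big character swim.
; Small-character overlaps, or any overlap while BP_BigCharacter has it picked up, play a splash sound and teleport the overlapping actor after a one-second delay.
; Otherwise, the big character switches movement and animation to swimming if the water is swimmable.
; Leaving the volume restores walking.
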(event OnComponentEndOverlap(WaterCollisionBox)
  (params (OverlappedComponent :type Primitive%20Component%20Object%20Reference) (OtherActor :type Actor%20Object%20Reference) (OtherComp :type Primitive%20Component%20Object%20Reference) (OtherBodyIndex :type Integer))
  ;[1 0.5507 0.5308] OVERLAP: End
  (Utilities|Casting|CastToBP_BigCharacter OtherActor)
  (Variables|Default|SetBigCharOverlap false)
  (CallFunction|ChangetoWalkMode))

(event OnComponentBeginOverlap(WaterCollisionBox)
  (params (OverlappedComponent :type Primitive%20Component%20Object%20Reference) (OtherActor :type Actor%20Object%20Reference) (OtherComp :type Primitive%20Component%20Object%20Reference) (OtherBodyIndex :type Integer) (bFromSweep :type Boolean) (SweepResult :type Hit%20Result%20Structure%20%28by%20ref%29))
  ;[0.633 1 0.6611] OVERLAP: Begin
  (if (Variables|/Game/Blueprints/Characters/BP_BigCharacter.BP_BigCharacter_C|GetbSmallCharacterPickedUp (Variables|Default|GetBigCharRef))
    (Audio|PlaySound2D "/Game/Audio/Stone-Dropping-in-Water-A1-www_fesliyanstudios_com.Stone-Dropping-in-Water-A1-www_fesliyanstudios_com" 1.0 1.0 0.0 0 0)
    (Utilities|FlowControl|Delay 1.0)
    (Transformation|Teleport OtherActor (Transformation|GetActorLocation (Variables|Default|GetTeleport%20Location)) "0, 0, 0")
    (elif (Actor|ActorHasTag OtherActor "SmallCharacter")
      (Audio|PlaySound2D "/Game/Audio/Stone-Dropping-in-Water-A1-www_fesliyanstudios_com.Stone-Dropping-in-Water-A1-www_fesliyanstudios_com" 1.0 1.0 0.0 0 0)
      (Utilities|FlowControl|Delay 1.0)
      (Transformation|Teleport OtherActor (Transformation|GetActorLocation (Variables|Default|GetTeleport%20Location)) "0, 0, 0")
      (else
        (Utilities|Casting|CastToBP_BigCharacter OtherActor)
        (Variables|Default|SetBigCharOverlap true)
        (if (Variables|Default|GetIsSwimableWater)
          (CallFunction|ChangetoSwimmingMode))))))

(event Custom|ChangeToSwimmingMode
  (bind _bigcharref (Variables|Default|GetBigCharRef))
  ;[0.4062 1 0.9901] Swimming
  (Variables|/Script/VerticalSlice.VerticalSliceCharacter|SetisSwimming (Variables|Default|GetBigCharRef) true)
  (Pawn|Components|CharacterMovement|SetMovementMode (Variables|/Script/Engine.Character|GetCharacterMovement _bigcharref) "MOVE_Swimming" 0)
  (Variables|/Game/Animations/Big/Big_AnimBP.Big_AnimBP_C|SetbisSwimming (Variables|/Game/Blueprints/Characters/BP_BigCharacter.BP_BigCharacter_C|GetBigAnimBP _bigcharref) true))

(event Custom|ChangeToWalkMode
  (bind _bigcharref (Variables|Default|GetBigCharRef))
  ;[1 0.9611 0.9301] Walking
  (Variables|/Script/VerticalSlice.VerticalSliceCharacter|SetisSwimming (Variables|Default|GetBigCharRef) false)
  (Pawn|Components|CharacterMovement|SetMovementMode (Variables|/Script/Engine.Character|GetCharacterMovement _bigcharref) "MOVE_Walking" 0)
  (Variables|/Game/Animations/Big/Big_AnimBP.Big_AnimBP_C|SetbisSwimming (Variables|/Game/Blueprints/Characters/BP_BigCharacter.BP_BigCharacter_C|GetBigAnimBP _bigcharref) false))

(event EventBeginPlay
  ;[1 0.7437 0.5481] BEGINPLAY: Get our Reference of the Big Character
  (bind _outactors (Actor|GetAllActorsOfClass "/Game/Blueprints/Characters/BP_BigCharacter.BP_BigCharacter_C"))
  (Variables|Default|SetBigCharRef (Utilities|Array|Get(acopy) _outactors)))

(fn ConstructionScript)