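; Spline-based generator Blueprint, named for water but using cliff naming, that builds a chain of deformed meshes along a spline in the construction script.
; It pads a per-point data array to the spline point count, then adds one spline mesh per segment with interpolated bank, width and thickness.
; Looping and collision are optional, and a debug toggle draws point index labels above the spline.
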(event EventBeginPlay)

(event Collision|EventActorBeginOverlap
  (params (OtherActor :type Actor%20Object%20Reference)))

(event EventTick
  (params (DeltaSeconds :type Float%20%28single-precision%29)))

(fn ConstructionScript
  (Utilities|FlowControl|Sequence
    (:then_0
      (|StoreNumberofSplinePoints))
    (:then_1
      (|BuildCliffDataArray))
    (:then_2
      (for _index (range 0 (- (Variables|Default|GetNumber%20of%20Spline%20Points) (Math|Integer|SelectInt 1 2 (Variables|TrackSetup|GetLoopingTrack))))
        (CallFunction|BuildCliffElement _index (Variables|CliffMesh|GetCliffMesh))))
    (:then_3
      (|DrawSplinePointNumbers))))

(fn BuildCliffElement
  (params (LoopIndex :type Integer) (CliffElementMesh :type Static%20Mesh%20Object%20Reference))
  (LocalVariables|SetLocal_CurrentLoopIndex LoopIndex)
  (LocalVariables|SetLocal_NextLoopIndex (Math|Integer|%(Integer) (+ LoopIndex 1) (Variables|Default|GetNumber%20of%20Spline%20Points)))
  (LocalVariables|SetLocal_CliffElementMesh CliffElementMesh)
  (Utilities|FlowControl|Sequence
    (:then_0
      (LocalVariables|SetLocal_StartLocation (.Location (Spline|GetLocationandTangentatSplinePoint (Variables|Default|GetSpline) (LocalVariables|GetLocal_CurrentLoopIndex) "Local")))
      (LocalVariables|SetLocal_StartTangent (.Tangent (Spline|GetLocationandTangentatSplinePoint (Variables|Default|GetSpline) (LocalVariables|GetLocal_CurrentLoopIndex) "Local")))
      (LocalVariables|SetLocal_EndLocation (.Location (Spline|GetLocationandTangentatSplinePoint (Variables|Default|GetSpline) (LocalVariables|GetLocal_NextLoopIndex) "Local")))
      (LocalVariables|SetEnd_EndTangent (.Tangent (Spline|GetLocationandTangentatSplinePoint (Variables|Default|GetSpline) (LocalVariables|GetLocal_NextLoopIndex) "Local")))
      (LocalVariables|SetLocal_StartRoll (.cliffbank (Utilities|Array|Get(acopy) (Variables|TrackSetup|GetCliffDataArray) (LocalVariables|GetLocal_CurrentLoopIndex))))
      (LocalVariables|SetLocal_StartScale (Math|Vector2D|MakeVector2D (.trackwidth (Utilities|Array|Get(acopy) (Variables|TrackSetup|GetCliffDataArray) (LocalVariables|GetLocal_CurrentLoopIndex))) (.cliffthickness (Utilities|Array|Get(acopy) (Variables|TrackSetup|GetCliffDataArray) (LocalVariables|GetLocal_CurrentLoopIndex)))))
      (LocalVariables|SetLocal_EndRoll (.cliffbank (Utilities|Array|Get(acopy) (Variables|TrackSetup|GetCliffDataArray) (LocalVariables|GetLocal_NextLoopIndex))))
      (LocalVariables|SetLocal_EndScale (Math|Vector2D|MakeVector2D (.trackwidth (Utilities|Array|Get(acopy) (Variables|TrackSetup|GetCliffDataArray) (LocalVariables|GetLocal_NextLoopIndex))) (.cliffthickness (Utilities|Array|Get(acopy) (Variables|TrackSetup|GetCliffDataArray) (LocalVariables|GetLocal_NextLoopIndex))))))
    (:then_1
      (bind _returnvalue (AddComponent|AddSplineMeshComponent false))
      (LocalVariables|SetLocal_CurrentSplineMesh _returnvalue)
      (Components|StaticMesh|SetStaticMesh (LocalVariables|GetLocal_CurrentSplineMesh) (LocalVariables|GetLocal_CliffElementMesh))
      (SplineMesh|SetStartandEnd (LocalVariables|GetLocal_CurrentSplineMesh) (LocalVariables|GetLocal_StartLocation) (LocalVariables|GetLocal_StartTangent) (LocalVariables|GetLocal_EndLocation) (LocalVariables|GetEnd_EndTangent) true :!class /Script/Engine.SplineMeshComponent)
      (Class|SplineMeshComponent|SetStartRoll (LocalVariables|GetLocal_CurrentSplineMesh) (LocalVariables|GetLocal_StartRoll) true)
      (Class|SplineMeshComponent|SetEndRoll (LocalVariables|GetLocal_CurrentSplineMesh) (LocalVariables|GetLocal_EndRoll) true)
      (SplineMesh|SetStartScale (LocalVariables|GetLocal_CurrentSplineMesh) (LocalVariables|GetLocal_StartScale) true :!class /Script/Engine.SplineMeshComponent)
      (SplineMesh|SetEndScale (LocalVariables|GetLocal_CurrentSplineMesh) (LocalVariables|GetLocal_EndScale) true :!class /Script/Engine.SplineMeshComponent)
      (Collision|SetCollisionEnabled (LocalVariables|GetLocal_CurrentSplineMesh) (select (Variables|CliffDebug|GetCollisions) "QueryAndPhysics" "NoCollision")))))