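; Trigger volume actor that randomly plays a sound at its own location when the player character walks into it.
; On overlap, a weighted random bool decides whether the configured sound plays.
; The construction script sizes a box and a sphere component, then uses a toggle to make only one shape visible and able to generate overlaps.
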(event Collision|EventActorBeginOverlap
  (params (OtherActor :type Actor%20Object%20Reference))
  (if (== OtherActor (Game|GetPlayerCharacter 0))
    (if (Math|Random|RandomBoolwithWeight (Variables|Default|GetWeight))
      (Audio|PlaySoundatLocation (Variables|Default|GetSound) (Transformation|GetActorLocation) "0, 0, 0" 1.0 1.0 0.0 0 0 0))))

(fn ConstructionScript
  (bind _box (Variables|Default|GetBox))
  (bind _sphere (Variables|Default|GetSphere))
  (bind _sphere_option (Variables|Default|GetSphere_Option))
  (bind _returnvalue (not _sphere_option))
  (Components|Box|SetBoxExtent _box (Variables|Default|GetExtents) true)
  (Components|Sphere|SetSphereRadius _sphere (Variables|Default|GetRadius) true)
  (Variables|/Script/Engine.PrimitiveComponent|SetbGenerateOverlapEvents _sphere _sphere_option)
  (Rendering|SetVisibility _sphere _sphere_option false)
  (Variables|/Script/Engine.PrimitiveComponent|SetbGenerateOverlapEvents _box _returnvalue)
  (Rendering|SetVisibility _box _returnvalue false))