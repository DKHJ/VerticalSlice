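; Ambient audio volume that plays a positional sound at random intervals and random offsets while the player is inside it.
; Construction script sizes and enables overlaps on the selected sphere, box or capsule.
; Player overlap starts a function-name timer and exit clears it; each spawn re-arms it with a new random delay.
; Offsets follow the forward, right and up axes of either the player or the actor, per PlayerOrigin.
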(event Custom|Sound_Trig
  (bind _returnvalue (Game|GetPlayerCharacter 0))
  (bind _self self)
  (bind _player_origin (Variables|Default|GetPlayer_Origin))
  (bind _min (Variables|Distance|GetMin))
  (bind _max (Variables|Distance|GetMax))
  (bind (_x _y _z) (Math|Vector|BreakVector _min))
  (bind (_x_2 _y_2 _z_2) (Math|Vector|BreakVector _max))
  (bind _returnvalue_2 (select _player_origin _returnvalue _self))
  ;[1 1 1] Spawn sound
  (Audio|SpawnSoundatLocation (Variables|Default|GetSound) (+ (Transformation|GetActorLocation _returnvalue_2) (+ (* (Transformation|GetActorForwardVector _returnvalue_2) (Math|Random|RandomFloatinRange _x _x_2)) (* (Transformation|GetActorRightVector _returnvalue_2) (Math|Random|RandomFloatinRange _y _y_2)) (* (Transformation|GetActorUpVector _returnvalue_2) (Math|Random|RandomFloatinRange _z _z_2)))) "0, 0, 0" (Variables|Default|GetVolume) 1.0 0.0 0 0)
  (CallFunction|Retrigger))

(event Custom|Retrigger
  ;[1 1 1] Check for player and start
  (Utilities|Time|SetTimerbyFunctionName 0 "Sound_Trig" (Math|Random|RandomFloatinRange (Variables|Time|GetTime_Min) (Variables|Default|GetTIme_Max))))

(event Collision|EventActorBeginOverlap
  (params (OtherActor :type Actor%20Object%20Reference))
  ;[1 1 1] Check for player and start
  (if (== (Game|GetPlayerCharacter 0) OtherActor)
    (Development|PrintString "Working")
    (Utilities|Time|SetTimerbyFunctionName 0 "Sound_Trig" (Math|Random|RandomFloatinRange (Variables|Time|GetTime_Min) (Variables|Default|GetTIme_Max)))))

(event Collision|EventActorEndOverlap
  (params (OtherActor :type Actor%20Object%20Reference))
  ;[1 1 1] Check for player and start
  (if (== (Game|GetPlayerCharacter 0) OtherActor)
    (Utilities|Time|ClearTimerbyFunctionName 0 "Sound_Trig")))

(event EventBeginPlay
  ;[1 1 1] Check for player and start
  (for _array_element (Utilities|Array|MakeArray (Game|GetPlayerController 0))
    (if (== (Game|GetPlayerCharacter 0) _array_element)
      (Utilities|Time|SetTimerbyFunctionName 0 "Sound_Trig" (Math|Random|RandomFloatinRange (Variables|Time|GetTime_Min) (Variables|Default|GetTIme_Max))))))

(fn ConstructionScript
  (bind _sphere (Variables|Default|GetSphere))
  (bind _box (Variables|Default|GetBox))
  (bind _capsule (Variables|Default|GetCapsule))
  (switch Utilities|FlowControl|Switch|SwitchonAudio_POS_Shapes (Variables|Shape|GetShape)
    (:NewEnumerator0
      (Components|Sphere|SetSphereRadius _sphere (Variables|Shape|GetSphere_Radius) true)
      (Variables|/Script/Engine.PrimitiveComponent|SetbGenerateOverlapEvents _sphere true))
    (:NewEnumerator1
      (Components|Box|SetBoxExtent _box (Variables|Shape|GetBox_Extents) true)
      (Variables|/Script/Engine.PrimitiveComponent|SetbGenerateOverlapEvents _box true))
    (:NewEnumerator2
      (Components|Capsule|SetCapsuleSize _capsule (Variables|Shape|GetCapsule_Radius) (Variables|Shape|GetCapsule_Half_Height) true)
      (Variables|/Script/Engine.PrimitiveComponent|SetbGenerateOverlapEvents _capsule true))))