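; BP_MovingAudio is a moving sound source that plays its configured sound while travelling along splines on the actor.
; Each trigger picks a random spline component, re-rolling any of 150 units or shorter, and a timeline scaled by MovementSpeed drives the audio along it.
; The timeline's Retrigger event starts another random path when looping, otherwise fades the sound out.
; Optional auto-start, spline debug drawing and a sphere visualiser support setup.
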(event Custom|Trigger_Movement
  (bind _audio (Variables|Default|GetAudio))
  ;[1 1 1] Choose Spline
  (Variables|Default|SetSelectedSpline (Utilities|Array|Get(acopy) (Variables|Default|GetSplineArray) (Math|Random|RandomInteger (Utilities|Array|Length (Variables|Default|GetSplineArray)))))
  (if (> (Spline|GetSplineLength (Variables|Default|GetSelectedSpline)) 1.5e+02)
    ;[1 1 1] Move Along Spline
    (Utilities|FlowControl|Sequence
      (:then_0
        (Utilities|FlowControl|DoOnce false :!label _label
          (:Completed
            (Audio|Components|Audio|Play _audio 0.0))))
      (:then_1
        (bind _spline_position (Timeline|Timeline_0 PlayFromStart)
          (:Update
            (Transformation|SetRelativeLocation (Variables|Default|GetAudio) (Spline|GetLocationatDistanceAlongSpline (Variables|Default|GetSelectedSpline) (* (Spline|GetSplineLength (Variables|Default|GetSelectedSpline)) _spline_position) "Local") false false)
            (if (Variables|Default|GetShowVisualiser)
              (Transformation|SetRelativeLocation (Variables|Default|GetSphere) (Spline|GetLocationatDistanceAlongSpline (Variables|Default|GetSelectedSpline) (* (Spline|GetSplineLength (Variables|Default|GetSelectedSpline)) _spline_position) "Local") false false)))
          (:Retrigger
            (if (Variables|Default|GetLooping)
              (CallFunction|TriggerMovement)
              (else
                (Audio|Components|Audio|FadeOut _audio 1.0 0.0 "Linear" :!class /Script/Engine.AudioComponent)
                (goto _label Reset)))))))
    (else
      (CallFunction|ChooseSpline))))

(event Custom|ChooseSpline
  (bind _audio (Variables|Default|GetAudio))
  ;[1 1 1] Choose Spline
  (Variables|Default|SetSelectedSpline (Utilities|Array|Get(acopy) (Variables|Default|GetSplineArray) (Math|Random|RandomInteger (Utilities|Array|Length (Variables|Default|GetSplineArray)))))
  (if (> (Spline|GetSplineLength (Variables|Default|GetSelectedSpline)) 1.5e+02)
    ;[1 1 1] Move Along Spline
    (Utilities|FlowControl|Sequence
      (:then_0
        (Utilities|FlowControl|DoOnce false :!label _label
          (:Completed
            (Audio|Components|Audio|Play _audio 0.0))))
      (:then_1
        (bind _spline_position (Timeline|Timeline_0 PlayFromStart)
          (:Update
            (Transformation|SetRelativeLocation (Variables|Default|GetAudio) (Spline|GetLocationatDistanceAlongSpline (Variables|Default|GetSelectedSpline) (* (Spline|GetSplineLength (Variables|Default|GetSelectedSpline)) _spline_position) "Local") false false)
            (if (Variables|Default|GetShowVisualiser)
              (Transformation|SetRelativeLocation (Variables|Default|GetSphere) (Spline|GetLocationatDistanceAlongSpline (Variables|Default|GetSelectedSpline) (* (Spline|GetSplineLength (Variables|Default|GetSelectedSpline)) _spline_position) "Local") false false)))
          (:Retrigger
            (if (Variables|Default|GetLooping)
              (CallFunction|TriggerMovement)
              (else
                (Audio|Components|Audio|FadeOut _audio 1.0 0.0 "Linear" :!class /Script/Engine.AudioComponent)
                (goto _label Reset)))))))
    (else
      (CallFunction|ChooseSpline))))

(event EventBeginPlay
  ;[1 1 1] set up
  (if (Variables|Default|GetShowVisualiser)
    (Rendering|SetVisibility (Variables|Default|GetSphere) true false))
  (Components|Timeline|SetPlayRate (Variables|Default|GetTimeline_0) (Variables|Default|GetMovementSpeed))
  (Audio|Components|Audio|SetSound (Variables|Default|GetAudio) (Variables|Default|GetSound))
  (Variables|/Script/Engine.AudioComponent|SetAttenuationSettings (Variables|Default|GetAudio) (Variables|Default|GetAttenuationSettings))
  (Variables|Default|SetSplineArray (Actor|GetComponentsByClass "/Script/Engine.SplineComponent"))
  (for _array_element (Variables|Default|GetSplineArray)
    (Class|SplineComponent|SetDrawDebug _array_element (Variables|Default|GetShowSplines)))
  (if (Variables|Default|GetAuto)
    (CallFunction|TriggerMovement)))

(fn ConstructionScript)