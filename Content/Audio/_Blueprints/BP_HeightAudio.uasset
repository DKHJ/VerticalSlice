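; BP_HeightAudio is an ambient audio zone that plays tree wind gusts, plus creaks near the top, based on the player's height.
; While the player is inside the sphere, sized by Extents, a self-retriggering randomized timer fires one-shot 2D sounds and is cleared on exit.
; Player Z, normalized between StartHeight and EndHeight, sets both the volume and the delay range between MaxDelayTime and MinDelayTime.
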(event OnComponentBeginOverlap(Sphere)
  (params (OverlappedComponent :type Primitive%20Component%20Object%20Reference) (OtherActor :type Actor%20Object%20Reference) (OtherComp :type Primitive%20Component%20Object%20Reference) (OtherBodyIndex :type Integer) (bFromSweep :type Boolean) (SweepResult :type Hit%20Result%20Structure%20%28by%20ref%29))
  (bind _returnvalue (Game|GetPlayerCharacter 0))
  (bind _max_delay_time (Variables|Default|GetMax_Delay_Time))
  (bind _start_height (Variables|Default|GetStart_Height))
  (bind _end_height (Variables|Default|GetEnd_Height))
  (bind _min_delay_time (Variables|Default|GetMin_Delay_Time))
  (bind _returnvalue_2 (Transformation|GetActorLocation _returnvalue))
  (bind _z (Math|Vector|BreakVector _returnvalue_2))
  (bind _returnvalue_3 (Math|Float|MapRangeClamped _z _start_height _end_height 0.0 1.0))
  (bind _returnvalue_4 (Math|Float|MapRangeClamped _returnvalue_3 0.0 1.0 _max_delay_time _min_delay_time))
  (bind _returnvalue_5 (* _returnvalue_4 0.5))
  (bind _returnvalue_6 (+ _returnvalue_5 _returnvalue_4))
  (bind _returnvalue_7 (Math|Random|RandomFloatinRange _returnvalue_4 _returnvalue_6))
  ;[1 1 1] switch on
  (if (== (Game|GetPlayerCharacter 0) OtherActor)
    (Utilities|Time|SetTimerbyFunctionName 0 "Trigger_Sound" _returnvalue_7)
    (Development|PrintString (Utilities|String|ToString(Float) _returnvalue_7) false)))

(event OnComponentEndOverlap(Sphere)
  (params (OverlappedComponent :type Primitive%20Component%20Object%20Reference) (OtherActor :type Actor%20Object%20Reference) (OtherComp :type Primitive%20Component%20Object%20Reference) (OtherBodyIndex :type Integer))
  ;[1 1 1] switch on
  (if (== (Game|GetPlayerCharacter 0) OtherActor)
    (Utilities|Time|ClearTimerbyFunctionName 0 "Trigger_Sound")))

(event Custom|Trigger_Sound
  (bind _returnvalue (Game|GetPlayerCharacter 0))
  (bind _start_height (Variables|Default|GetStart_Height))
  (bind _end_height (Variables|Default|GetEnd_Height))
  (bind _returnvalue_2 (Transformation|GetActorLocation _returnvalue))
  (bind _z (Math|Vector|BreakVector _returnvalue_2))
  (bind _returnvalue_3 (Math|Float|MapRangeClamped _z _start_height _end_height 0.0 1.0))
  ;[1 1 1] play sounds
  (Audio|PlaySound2D "/Game/Audio/Ambience/Weather/as_ab_ao_Trees_Wind_Trig.as_ab_ao_Trees_Wind_Trig" _returnvalue_3 1.0 0.0 0 0) ; Wind Gusts
  (if (> _returnvalue_3 0.8)
    (Audio|PlaySound2D "/Game/Audio/Ambience/Trees/as_ab_ao_Tree_Creaks.as_ab_ao_Tree_Creaks" _returnvalue_3 1.0 0.0 0 0) ; Tree Creaks
  )
  (CallFunction|Retrigger))

(event Custom|Retrigger
  (bind _returnvalue (Game|GetPlayerCharacter 0))
  (bind _max_delay_time (Variables|Default|GetMax_Delay_Time))
  (bind _start_height (Variables|Default|GetStart_Height))
  (bind _end_height (Variables|Default|GetEnd_Height))
  (bind _min_delay_time (Variables|Default|GetMin_Delay_Time))
  (bind _returnvalue_2 (Transformation|GetActorLocation _returnvalue))
  (bind _z (Math|Vector|BreakVector _returnvalue_2))
  (bind _returnvalue_3 (Math|Float|MapRangeClamped _z _start_height _end_height 0.0 1.0))
  (bind _returnvalue_4 (Math|Float|MapRangeClamped _returnvalue_3 0.0 1.0 _max_delay_time _min_delay_time))
  (bind _returnvalue_5 (* _returnvalue_4 0.5))
  (bind _returnvalue_6 (+ _returnvalue_5 _returnvalue_4))
  (bind _returnvalue_7 (Math|Random|RandomFloatinRange _returnvalue_4 _returnvalue_6))
  ;[1 1 1] switch on
  (Utilities|Time|SetTimerbyFunctionName 0 "Trigger_Sound" _returnvalue_7)
  (Development|PrintString (Utilities|String|ToString(Float) _returnvalue_7) false))

(event EventBeginPlay
  (bind _returnvalue (Game|GetPlayerCharacter 0))
  (bind _max_delay_time (Variables|Default|GetMax_Delay_Time))
  (bind _start_height (Variables|Default|GetStart_Height))
  (bind _end_height (Variables|Default|GetEnd_Height))
  (bind _min_delay_time (Variables|Default|GetMin_Delay_Time))
  (bind _returnvalue_2 (Transformation|GetActorLocation _returnvalue))
  (bind _z (Math|Vector|BreakVector _returnvalue_2))
  (bind _returnvalue_3 (Math|Float|MapRangeClamped _z _start_height _end_height 0.0 1.0))
  (bind _returnvalue_4 (Math|Float|MapRangeClamped _returnvalue_3 0.0 1.0 _max_delay_time _min_delay_time))
  (bind _returnvalue_5 (* _returnvalue_4 0.5))
  (bind _returnvalue_6 (+ _returnvalue_5 _returnvalue_4))
  (bind _returnvalue_7 (Math|Random|RandomFloatinRange _returnvalue_4 _returnvalue_6))
  ;[1 1 1] setup
  (for _array_element (Collision|GetOverlappingActors 0 :!class /Script/Engine.Actor)
    (if (== _array_element (Game|GetPlayerCharacter 0))
      ;[1 1 1] switch on
      (Utilities|Time|SetTimerbyFunctionName 0 "Trigger_Sound" _returnvalue_7)
      (Development|PrintString (Utilities|String|ToString(Float) _returnvalue_7) false))))

(event EventTick
  (params (DeltaSeconds :type Float%20%28single-precision%29))
  ;[1 1 1] Debug
  (Development|PrintString (Utilities|String|ToString(Text) (Utilities|Text|FormatText "Height {Height}" (Math|Float|MapRangeClamped (.Z (Math|Vector|BreakVector (Transformation|GetActorLocation (Game|GetPlayerCharacter 0)))) (Variables|Default|GetStart_Height) (Variables|Default|GetEnd_Height) 0.0 1.0))) false false "(R=0.000000,G=0.660000,B=1.000000,A=1.000000)" DeltaSeconds))

(fn ConstructionScript
  (Components|Sphere|SetSphereRadius (Variables|Default|GetSphere) (Variables|Default|GetExtents) true))