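; WaterBlockers_BP is a collision barrier, named for blocking water, that is active only while the big character has the small character picked up.
; On BeginPlay it caches the first BP_BigCharacter found in the level.
; Every Tick it polls that character's SmallCharacterPickedUp flag and switches WaterBlockerBox between query-and-physics collision and no collision.
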(event EventBeginPlay
  (bind _outactors (Actor|GetAllActorsOfClass "/Game/Blueprints/Characters/BP_BigCharacter.BP_BigCharacter_C"))
  (Variables|Default|SetBigCharRef (Utilities|Array|Get(acopy) _outactors)))

(event EventTick
  (params (DeltaSeconds :type Float%20%28single-precision%29))
  (if (Variables|/Game/Blueprints/Characters/BP_BigCharacter.BP_BigCharacter_C|GetbSmallCharacterPickedUp (Variables|Default|GetBigCharRef))
    (Collision|SetCollisionEnabled (Variables|Default|GetWaterBlockerBox) "QueryAndPhysics")
    (else
      (Collision|SetCollisionEnabled (Variables|Default|GetWaterBlockerBox) "NoCollision"))))

(fn ConstructionScript)