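; BP_ThrowableBoxProjectile is a box in the spring puzzles that BP_BigCharacter can pick up.
; On a hit it enables physics simulation on its cube.
; A Box overlap registers or clears it as the character's interact target.
; Interacting destroys the actor and sets the character's PickedUpBox flag, or prints an error if a box is already carried.
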(event OnComponentBeginOverlap(Box)
  (params (OverlappedComponent :type Primitive%20Component%20Object%20Reference) (OtherActor :type Actor%20Object%20Reference) (OtherComp :type Primitive%20Component%20Object%20Reference) (OtherBodyIndex :type Integer) (bFromSweep :type Boolean) (SweepResult :type Hit%20Result%20Structure%20%28by%20ref%29))
  (bind _asbp_big_character (Utilities|Casting|CastToBP_BigCharacter OtherActor))
  (Default|UpdateInteract _asbp_big_character self true)
  (Variables|Default|SetBigCharacterRef _asbp_big_character))

(event OnComponentEndOverlap(Box)
  (params (OverlappedComponent :type Primitive%20Component%20Object%20Reference) (OtherActor :type Actor%20Object%20Reference) (OtherComp :type Primitive%20Component%20Object%20Reference) (OtherBodyIndex :type Integer))
  (bind _asbp_big_character (Utilities|Casting|CastToBP_BigCharacter OtherActor))
  (Default|UpdateInteract _asbp_big_character self false))

(event EventBeginPlay)

(event Collision|EventHit
  (params (MyComp :type Primitive%20Component%20Object%20Reference) (Other :type Actor%20Object%20Reference) (OtherComp :type Primitive%20Component%20Object%20Reference) (bSelfMoved :type Boolean) (HitLocation :type Vector :default "0, 0, 0") (HitNormal :type Vector :default "0, 0, 0") (NormalImpulse :type Vector :default "0, 0, 0") (Hit :type Hit%20Result%20Structure%20%28by%20ref%29))
  (Physics|SetSimulatePhysics (Variables|Default|GetCube) true))

(event EventDoInteract
  (if (Variables|/Game/Characters/BP_BigCharacter.BP_BigCharacter_C|GetPickedUpBox (Variables|Default|GetBigCharacterRef))
    (Development|PrintString "Error: Character already has a box picked up" true true "(R=1.000000,G=0.000000,B=0.031819,A=1.000000)" 4.0)
    (else
      (Actor|DestroyActor)
      (Variables|/Game/Characters/BP_BigCharacter.BP_BigCharacter_C|SetPickedUpBox (Variables|Default|GetBigCharacterRef) true)
      (Development|PrintString "Box picked up!" true true "(R=0.000000,G=1.000000,B=0.043410,A=1.000000)" 4.0))))

(fn ConstructionScript)

(fn BDoInteract
  (return false))